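; Construction manager that queues building jobs as placeholder proxy actors and assigns them to construction offices.
; Each new proxy goes to the nearest staffed, jobless office by straight-line distance, or into a bid list if none qualifies.
; BidManager hands a given contractor the closest pending bid.
; A proxy's completion event swaps it for the real building from the parallel queue entry and registers it with the game state.
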(event Custom|BindConstructionComplete
  (params (Proxy :type Construction%20Proxy%20BP%20Object%20Reference))
  (Utilities|IsValid Proxy ; check if on click not null clicked
    (:Is%20Valid
      (EventDispatchers|BindEventtoConstructionCompleted Proxy (EventDispatchers|CreateEvent :!event Custom|ConstructionCompleted)))))

(event Custom|ConstructionCompleted
  (params (Proxy :type Construction%20Proxy%20BP%20Object%20Reference))
  (CallFunction|FinishConstruction Proxy))

(fn ConstructionScript)

(fn QueueConstruction
  (params (ConstructionStruct :type Construction%20Struct%20Structure))
  (bind (_buildingclass _proxyclass _transform _displaymesh _workhoursrequired) (Utilities|Struct|BreakConstruction_Struct ConstructionStruct))
  (bind _returnvalue (Game|SpawnActorfromClass _proxyclass _transform "AlwaysSpawn" 0 _displaymesh 0)) ; We spawn proxy class and not actuall mesh yet
  (CallFunction|BindConstructionComplete _returnvalue) ; Custom event - Binds event dispatcher and creates event finished construction
  (Utilities|Array|Add (Variables|Default|GetProxies) _returnvalue)
  (Utilities|Array|Add (Variables|Default|GetQueue) ConstructionStruct)
  (Utilities|IsValid _returnvalue ; check if clicked is not null
    (:Is%20Valid
      (Default|SetConstructionTime _returnvalue _workhoursrequired)
      (CallFunction|InitialContractorSearch _returnvalue))))

(fn FinishConstruction
  (params (Proxy :type Construction%20Proxy%20BP%20Object%20Reference))
  (bind _queue (Variables|Default|GetQueue))
  (bind _proxies (Variables|Default|GetProxies))
  (bind _output_get (LocalVariables|SetIndex (Utilities|Array|FindItem _proxies Proxy)))
  (LocalVariables|SetConfig (Utilities|Array|Get(acopy) _queue _output_get))
  (Utilities|Array|RemoveIndex _queue (LocalVariables|GetIndex))
  (Utilities|Array|RemoveIndex _proxies (LocalVariables|GetIndex))
  (bind _returnvalue (Game|SpawnActorfromClass (.BuildingClass (Utilities|Struct|BreakConstruction_Struct (LocalVariables|GetConfig))) (.Transform (Utilities|Struct|BreakConstruction_Struct (LocalVariables|GetConfig))) "AlwaysSpawn" 0 0 (.Resource (Utilities|Struct|BreakConstruction_Struct (LocalVariables|GetConfig))) 0))
  (Default|AddBuildingtoGame (Variables|References|GetGameStateRef) _returnvalue)
  (Default|CallFinishedConstruction Proxy) ; calls construction office bp to clear job site
  (Actor|DestroyActor Proxy) ; remove proxy
)

(fn InitialContractorSearch
  (params (Proxy :type Construction%20Proxy%20BP%20Object%20Reference))
  (LocalVariables|SetProxy_LOCAL Proxy)
  (bind _outactors (Actor|GetAllActorsOfClass "/Game/TD2020/Blueprints/Buildings/Commercial/ConstructionOffice_BP.ConstructionOffice_BP_C")) ; expensive!!!!!! - it gets all construction offices in level
  (bind _output_get (LocalVariables|SetAllConstructionOffices_LOCAL _outactors)) ; sets them to local variable so we can use them later
  (if (> (Utilities|Array|Length _output_get) 0)
    (for _array_element (LocalVariables|GetAllConstructionOffices_LOCAL) ; fills arrays with length and offices
      (bind _output_get_2 (LocalVariables|SetSelectedOffice_LOCAL _array_element)) ; construction office
      (if (and (.HasOccupants (Default|GetOccupants _output_get_2)) (not (Default|GetJobStatus _output_get_2))) ; has employees and doesnt have job
        (Utilities|Array|Add (LocalVariables|GetDistanceToSite_LOCAL) (Transformation|GetDistanceTo (LocalVariables|GetSelectedOffice_LOCAL) (LocalVariables|GetProxy_LOCAL))) ; add distances to array
        (Utilities|Array|AddUnique (LocalVariables|GetAvaliableConstructionOffices_LOCAL) (LocalVariables|GetSelectedOffice_LOCAL)) ; added because it has same index as distance - can llok by index
      ))
    (if (> (Utilities|Array|Length (LocalVariables|GetAvaliableConstructionOffices_LOCAL)) 0) ; if no offices set it to construction bid
      (bind _output_get_3 (Variables|/Game/TD2020/Blueprints/Construction/ConstructionProxy_BP.ConstructionProxy_BP_C|SetContractor (LocalVariables|GetProxy_LOCAL) (Utilities|Array|Get(acopy) (LocalVariables|GetAvaliableConstructionOffices_LOCAL) (.IndexOfMinValue (Math|Float|MinOfFloatArray (LocalVariables|GetDistanceToSite_LOCAL)))))) ; set to nearest construction office
      (Default|SetCurrentJob _output_get_3 (LocalVariables|GetProxy_LOCAL))
      (return)
      (else
        _)))
  (Utilities|Array|AddUnique (Variables|Default|GetConstructionBids) (LocalVariables|GetProxy_LOCAL)) ; we dont have any construction offices
  (return))

(fn BidManager
  (params (Contractor :type Construction%20Office%20BP%20Object%20Reference))
  (LocalVariables|SetContractor_LOCAL Contractor)
  (if (> (Utilities|Array|Length (Variables|Default|GetConstructionBids)) 0)
    (for _array_element (Variables|Default|GetConstructionBids) ; creates array of distances
      (Utilities|Array|Add (LocalVariables|GetDistanceToSites_LOCAL) (Transformation|GetDistanceTo (LocalVariables|GetContractor_LOCAL) _array_element)) ; index of construction bid matches index of distances
    )
    (bind _output_get (LocalVariables|SetJobSites_LOCAL (Utilities|Array|Get(acopy) (Variables|Default|GetConstructionBids) (.IndexOfMinValue (Math|Float|MinOfFloatArray (LocalVariables|GetDistanceToSites_LOCAL))))))
    (bind _returnvalue (Utilities|Array|RemoveItem (Variables|Default|GetConstructionBids) _output_get)) ; remove item
    (if _returnvalue ; didnt remove because of used index
      (Variables|/Game/TD2020/Blueprints/Construction/ConstructionProxy_BP.ConstructionProxy_BP_C|SetContractor (LocalVariables|GetJobSites_LOCAL) (LocalVariables|GetContractor_LOCAL))
      (return (LocalVariables|GetJobSites_LOCAL) false)
      (else
        _)))
  (return 0 false) ; empty job site if no bids and won bid false
)