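; Construction proxy actor that shows a ghosted building mesh while assigned workers build it over game time.
; Each tick it accrues work time scaled by workforce and the GameState's time unit, updated through a game-speed dispatcher.
; On completion it fires ConstructionCompleted, frees and unhides workers, then destroys itself.
; When selected through a HUD request, it glides the camera over via timeline lerp and opens its widget, locking navigation and main HUD.
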(event Custom|AdjustTime
  (params (TimeUnit :type Float%20%28single-precision%29))
  ;[1 1 1] Adjust time
  (Variables|Time|SetTimeUnit TimeUnit))

(event Custom|DisplayHUD
  (params (Actor :type Actor%20Object%20Reference))
  (bind _controllerref (Variables|References|GetControllerRef))
  ;[1 1 1] DisplayHUD
  (if (== Actor self) ; if we selected this thing, if not ignore it
    (Utilities|FlowControl|Sequence
      (:then_0
        (bind _newlocation (|LerpLocation) ; update is kinda like tick - lerps between old and new location
          (:Update
            (Transformation|SetActorLocation (Variables|/Game/TD2020/Blueprints/Camera/CameraPawnController.CameraPawnController_C|GetCameraPawnRef (Variables|References|GetControllerRef)) _newlocation false false))))
      (:then_1
        (UserInterface|Viewport|AddtoViewport (Variables|References|GetProxyHUD) 0)
        (Input|SetInputModeUIOnly _controllerref (Variables|References|GetProxyHUD) "LockAlways") ; disables our keyboard functions
        (Variables|/Game/TD2020/Blueprints/Camera/CameraPawnController.CameraPawnController_C|SetDisableCamNav _controllerref true)
        (Widget|SetIsEnabled (Variables|/Game/TD2020/Blueprints/Camera/CameraPawnController.CameraPawnController_C|GetMainHudRef _controllerref) false) ; disable creating buildings
      ))))

(event EventBeginPlay
  ;[1 1 1] Begin Play
  (bind _output_get (Variables|References|SetGameStateRef (.AsMy%20Game%20State (Utilities|Casting|CastToMyGameState (Game|GetGameState)))))
  (EventDispatchers|BindEventtoUpdateGameSpeed _output_get (EventDispatchers|CreateEvent :!event Custom|AdjustTime)) ; bind proxy to dispatcher
  (Variables|Time|SetTimeUnit (Default|GetCurrentTimeUnit (Variables|References|GetGameStateRef)))
  (bind _output_get_2 (Variables|References|SetControllerRef (.AsCamera%20Pawn%20Controller (Utilities|Casting|CastToCameraPawnController (Game|GetPlayerController 0)))))
  (EventDispatchers|BindEventtoHUDRequest _output_get_2 (EventDispatchers|CreateEvent :!event Custom|DisplayHUD))
  (bind _returnvalue (UserInterface|CreateWidget "/Game/TD2020/HUDs/Proxy_HUD.Proxy_HUD_C" 0 self (Variables|References|GetControllerRef)))
  (Variables|References|SetProxyHUD _returnvalue))

(event EventTick
  (params (DeltaSeconds :type Float%20%28single-precision%29))
  ;[1 1 1] Event Tick
  (Variables|Time|SetDelta DeltaSeconds)
  (if (not (Variables|Default|GetIsConstructionCompleted))
    (CallFunction|DoWork)
    (if (>= (Variables|Default|GetWorkTimeSpent) (Variables|Default|GetConstructionTime))
      (Variables|Default|SetIsConstructionCompleted true) ; is completed
      (Default|CallConstructionCompleted self) ; calls event that is bound to it (construction complete)...
      (CallFunction|ConstructionComplete)
      (if (UserInterface|Viewport|IsinViewport (Variables|References|GetProxyHUD))
        (Default|RemoveHUD (Variables|References|GetProxyHUD)))
      (Utilities|FlowControl|Delay 0.2)
      (Actor|DestroyActor))))

(fn ConstructionScript
  (bind _staticmesh (Variables|Components|GetStaticMesh))
  (Components|StaticMesh|SetStaticMesh _staticmesh (Variables|References|GetDisplayMesh))
  (Rendering|Material|SetMaterial _staticmesh 0 "/Game/TD2020/Geometry/Materials/Ghost_M_Inst.Ghost_M_Inst") ; ghost material instance
  (CallFunction|SetBuildingEntrance (Variables|Components|GetEntrance) (Variables|Components|GetStaticMesh))
  (CallFunction|SetBuildingCollisionBox (Variables|Components|GetCollision) (Variables|Components|GetStaticMesh)))

(fn SetConstructionTime
  (params (WorkHours :type Float%20%28single-precision%29))
  (Variables|Default|SetConstructionTime (* WorkHours 6e+01))
  (return))

(fn DoWork
  (bind _active_workers (CallFunction|GetWorkforce))
  (if (> _active_workers 0.0)
    (bind _output_get (Variables|Time|SetClockwork (.ClockworkOut (CallFunction|SetClockwork (Variables|Time|GetDelta) (/ (Variables|Time|GetTimeUnit) _active_workers) (Variables|Time|GetClockwork)))))
    (Variables|Default|SetWorkTimeSpent (* _output_get 6e+01))
    (return)
    (else
      (return))))

(fn GetWorkforce
  (return (Math|Conversions|ToFloat(Integer) (Utilities|Array|Length (Variables|References|GetActiveWorkers)))))

(fn ReporttoShift
  (params (Worker :type NPC%20BP%20Object%20Reference))
  (Utilities|Array|Add (Variables|References|GetActiveWorkers) Worker)
  (return))

(fn ConstructionComplete
  (if (> (CallFunction|GetWorkforce) 0.0)
    (for _array_element (Variables|References|GetActiveWorkers)
      (Default|SetIsBusy _array_element false) ; when construction is completed, free all workers - is busy = false
      (Rendering|SetActorHiddenInGame _array_element false) ; set actors visible
    )
    (Variables|References|SetActiveWorkers (Utilities|Array|MakeArray 0)) ; clear array
    (return)
    (else
      (return))))

(fn LeaveShift
  (params (Employee :type NPC%20BP%20Object%20Reference))
  (if (> (Utilities|Array|FindItem (Variables|References|GetActiveWorkers) Employee) -1)
    (bind _returnvalue (Utilities|Array|RemoveItem (Variables|References|GetActiveWorkers) Employee)) ; if is in workers array  - remove it
    (return _returnvalue)
    (else
      (return false))))