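; Player controller for a top-down building game that drives the CameraPawn and handles selection and building placement.
; Axis and screen-edge movement support a Shift boost, with axis speed scaling by zoom; holding Pan opens gates for rotation and suspends movement.
; BeginPlay spawns the construction manager, ghost building and HUD.
; In build mode the ghost follows the cursor and rotates; clicking queues valid construction, otherwise it sends clicked actors to the HUD.
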(event EventBeginPlay
  (bind _returnvalue (Math|Transform|MakeTransform "0, 0, 0" "0, 0, 0" "0.500000,0.500000,0.500000"))
  (bind _self self)
  ;[1 1 1] Begin Play
  (Utilities|FlowControl|Sequence
    (:then_0
      (Utilities|ReferenceCasts))
    (:then_1
      (bind _returnvalue_2 (Game|SpawnActorfromClass "/Game/TD2020/Blueprints/Construction/ConstructionManager_BP.ConstructionManager_BP_C" _returnvalue "AlwaysSpawn" 0 (Variables|References|GetGameStateRef) 0))
      (Variables|References|SetConstructionManagerRef _returnvalue_2))
    (:then_2
      (bind _returnvalue_3 (Game|SpawnActorfromClass "/Game/TD2020/Blueprints/Buildings/GhostBuilding_BP.GhostBuilding_BP_C" _returnvalue "AlwaysSpawn" 0 _self 0))
      (Variables|References|SetGhostBuildingRef _returnvalue_3))
    (:then_3
      (Input|SetInputModeGameandUI _self (Variables|References|GetMainHudRef) "LockAlways" false)
      (Utilities|CreateHUDs)
      (UserInterface|Viewport|AddtoViewport (Variables|References|GetMainHudRef) 0))))

(event EventTick
  (params (DeltaSeconds :type Float%20%28single-precision%29))
  ;[1 1 1] Construction
  ;;[1 1 1] Tick
  (if (Variables|Default|GetBuildModeActive)
    (|SetCursorWorldPosition)))

(event Input|ActionEvents|InputActionPan
  (params (Key :type Key%20Structure))
  (bind _camerapawnref (Variables|References|GetCameraPawnRef))
  (bind _returnvalue (Transformation|GetActorRotation _camerapawnref))
  (bind (_roll _pitch _yaw) (Math|Rotator|BreakRotator _returnvalue))
  ;[1 1 1] Camera
  ;;[1 1 1] Pan
  ;;;[1 1 1] Pan Y
  (:Pressed
    (Variables|Default|SetDisableCamNav true)
    (Utilities|FlowControl|Gate true) ; enters at Open
  )
  (:Released
    (Variables|Default|SetDisableCamNav false)
    (Utilities|FlowControl|Gate true) ; enters at Close
  ))

(event Input|ActionEvents|InputActionExit
  (params (Key :type Key%20Structure))
  ;[1 1 1] Camera
  ;;[1 1 1] Exit
  (:Pressed
    (Game|QuitGame 0 "Quit")))

(event Input|ActionEvents|InputActionZoomReset
  (params (Key :type Key%20Structure))
  ;[1 1 1] Camera
  ;;[1 1 1] Zoom
  ;;;[1 1 1] Reset Zoom
  (:Pressed
    (Variables|/Script/Engine.SpringArmComponent|SetTargetArmLength (Variables|/Game/TD2020/Blueprints/Camera/CameraPawn.CameraPawn_C|GetSpringArm (Variables|References|GetCameraPawnRef)) 2.5e+03) ; 1000
  ))

(event Input|ActionEvents|InputActionCameraX
  (params (Key :type Key%20Structure)))

(event Input|ActionEvents|InputActionCameraY
  (params (Key :type Key%20Structure)))

(event Input|ActionEvents|InputActionPanReset
  (params (Key :type Key%20Structure))
  (bind _camerapawnref (Variables|References|GetCameraPawnRef))
  (bind _returnvalue (Transformation|GetActorRotation _camerapawnref))
  (bind (_roll _pitch _yaw) (Math|Rotator|BreakRotator _returnvalue))
  ;[1 1 1] Camera
  ;;[1 1 1] Pan
  ;;;[1 1 1] Pan Reset
  (:Pressed
    (Transformation|SetActorRotation _camerapawnref (Math|Rotator|MakeRotator _roll 0.0 _yaw))))

(event Input|ActionEvents|InputActionRotateBuildingRight
  (params (Key :type Key%20Structure))
  (bind _ghostbuildingref (Variables|References|GetGhostBuildingRef))
  (bind _returnvalue (Transformation|GetActorRotation _ghostbuildingref))
  (bind (_roll _pitch _yaw) (Math|Rotator|BreakRotator _returnvalue))
  ;[1 1 1] Construction
  ;;[1 1 1] Rotate building right
  (:Pressed
    (if (and (Utilities|IsValid _ghostbuildingref) (Variables|Default|GetBuildModeActive))
      (Transformation|SetActorRotation _ghostbuildingref (Math|Rotator|MakeRotator _roll _pitch (- _yaw (Variables|Default|GetBuildingRotationRate)))))))

(event Input|ActionEvents|InputActionRotateBuildingLeft
  (params (Key :type Key%20Structure))
  (bind _ghostbuildingref (Variables|References|GetGhostBuildingRef))
  (bind _returnvalue (Transformation|GetActorRotation _ghostbuildingref))
  (bind (_roll _pitch _yaw) (Math|Rotator|BreakRotator _returnvalue))
  ;[1 1 1] Construction
  ;;[1 1 1] Rotate building left
  (:Pressed
    (if (and (Utilities|IsValid _ghostbuildingref) (Variables|Default|GetBuildModeActive))
      (Transformation|SetActorRotation _ghostbuildingref (Math|Rotator|MakeRotator _roll _pitch (+ _yaw (Variables|Default|GetBuildingRotationRate)))))))

(event Input|ActionEvents|InputActionZoomIn
  (params (Key :type Key%20Structure))
  (bind _camerapawnref (Variables|References|GetCameraPawnRef))
  (bind _springarm (Variables|/Game/TD2020/Blueprints/Camera/CameraPawn.CameraPawn_C|GetSpringArm _camerapawnref))
  ;[1 1 1] Camera
  ;;[1 1 1] Zoom
  ;;;[1 1 1] Zoom In
  (:Pressed
    (Variables|/Script/Engine.SpringArmComponent|SetTargetArmLength _springarm (Math|Float|Clamp(Float) (- (Variables|/Script/Engine.SpringArmComponent|GetTargetArmLength _springarm) (Variables|Default|GetZoomSensitivity)) 2.5e+02 (Variables|Default|GetMaxArmDistance)))))

(event Input|ActionEvents|InputActionZoomOut
  (params (Key :type Key%20Structure))
  (bind _camerapawnref (Variables|References|GetCameraPawnRef))
  (bind _springarm (Variables|/Game/TD2020/Blueprints/Camera/CameraPawn.CameraPawn_C|GetSpringArm _camerapawnref))
  ;[1 1 1] Camera
  ;;[1 1 1] Zoom
  ;;;[1 1 1] Zoom Out
  (:Pressed
    (Variables|/Script/Engine.SpringArmComponent|SetTargetArmLength _springarm (Math|Float|Clamp(Float) (+ (Variables|Default|GetZoomSensitivity) (Variables|/Script/Engine.SpringArmComponent|GetTargetArmLength _springarm)) 2.5e+02 (Variables|Default|GetMaxArmDistance)))))

(event Input|ActionEvents|InputActionPan
  (params (Key :type Key%20Structure))
  (bind _camerapawnref (Variables|References|GetCameraPawnRef))
  (bind _returnvalue (Transformation|GetActorRotation _camerapawnref))
  (bind (_roll _pitch _yaw) (Math|Rotator|BreakRotator _returnvalue))
  ;[1 1 1] Camera
  ;;[1 1 1] Pan
  ;;;[1 1 1] Pan X
  (:Pressed
    (Variables|Default|SetDisableCamNav true)
    (Utilities|FlowControl|Gate true) ; enters at Open
  )
  (:Released
    (Variables|Default|SetDisableCamNav false)
    (Utilities|FlowControl|Gate true) ; enters at Close
  ))

(event Input|ActionEvents|InputActionDeselect
  (params (Key :type Key%20Structure))
  ;[1 1 1] Construction
  ;;[1 1 1] Deselect
  (:Pressed
    (if (Variables|Default|GetBuildModeActive)
      (Default|KillGhost (Variables|References|GetGhostBuildingRef))
      (Variables|Default|SetBuildModeActive false))))

(event Input|AxisEvents|InputAxisMoveForward
  (params (AxisValue :type Float%20%28single-precision%29))
  (bind _camerapawnref (Variables|References|GetCameraPawnRef))
  ;[1 1 1] Camera
  ;;[1 1 1] Movement
  ;;;[1 1 1] Movement X
  (if (not (Variables|Default|GetDisableCamNav))
    (Transformation|SetActorTransform _camerapawnref (Utilities|MovementX (CallFunction|MovementSpeedCalculation) (Variables|Default|GetFastMoveMultiplier) AxisValue _camerapawnref))))

(event Input|AxisEvents|InputAxisMoveRight
  (params (AxisValue :type Float%20%28single-precision%29))
  (bind _movesensitivity (CallFunction|MovementSpeedCalculation))
  (bind _camerapawnref (Variables|References|GetCameraPawnRef))
  (bind _fastmovemultiplier (Variables|Default|GetFastMoveMultiplier))
  (bind _transform (Utilities|MovementY AxisValue _movesensitivity _fastmovemultiplier _camerapawnref))
  (bind (_location _rotation _scale) (Math|Transform|BreakTransform _transform))
  (bind (_x _y) (Math|Vector|BreakVector _location))
  ;[1 1 1] Camera
  ;;[1 1 1] Movement
  ;;;[1 1 1] Movement Y
  (if (not (Variables|Default|GetDisableCamNav))
    (Transformation|SetActorTransform (Variables|References|GetCameraPawnRef) (Math|Transform|MakeTransform (Math|Vector|MakeVector _x _y 5e+01) _rotation _scale))))

(event Input|MouseEvents|MouseX
  (params (AxisValue :type Float%20%28single-precision%29))
  (bind _camerapawnref (Variables|References|GetCameraPawnRef))
  (bind _returnvalue (Transformation|GetActorRotation _camerapawnref))
  (bind (_roll _pitch _yaw) (Math|Rotator|BreakRotator _returnvalue))
  ;[1 1 1] Camera
  ;;[1 1 1] Pan
  ;;;[1 1 1] Pan X
  (Utilities|FlowControl|Gate true
    (:Exit
      (Transformation|SetActorRotation (Variables|References|GetCameraPawnRef) (Math|Rotator|MakeRotator _roll _pitch (+ _yaw (* (Variables|Default|GetPanSensitivity) (+ AxisValue (stale Input|GamepadEvents|GamepadRightX AxisValue)))))))))

(event Input|GamepadEvents|GamepadRightY
  (params (AxisValue :type Float%20%28single-precision%29))
  (bind _camerapawnref (Variables|References|GetCameraPawnRef))
  (bind _returnvalue (Transformation|GetActorRotation _camerapawnref))
  (bind (_roll _pitch _yaw) (Math|Rotator|BreakRotator _returnvalue))
  ;[1 1 1] Camera
  ;;[1 1 1] Pan
  ;;;[1 1 1] Pan Y
  (Utilities|FlowControl|Gate true
    (:Exit
      (Transformation|SetActorRotation (Variables|References|GetCameraPawnRef) (Math|Rotator|MakeRotator _roll (Math|Float|Clamp(Float) (+ _pitch (* (Variables|Default|GetPanSensitivity) (+ (stale Input|MouseEvents|MouseY AxisValue) AxisValue))) -15.0 8e+01) _yaw)))))

(event Input|GamepadEvents|GamepadRightX
  (params (AxisValue :type Float%20%28single-precision%29))
  (bind _camerapawnref (Variables|References|GetCameraPawnRef))
  (bind _returnvalue (Transformation|GetActorRotation _camerapawnref))
  (bind (_roll _pitch _yaw) (Math|Rotator|BreakRotator _returnvalue))
  ;[1 1 1] Camera
  ;;[1 1 1] Pan
  ;;;[1 1 1] Pan X
  (Utilities|FlowControl|Gate true
    (:Exit
      (Transformation|SetActorRotation (Variables|References|GetCameraPawnRef) (Math|Rotator|MakeRotator _roll _pitch (+ _yaw (* (Variables|Default|GetPanSensitivity) (+ (stale Input|MouseEvents|MouseX AxisValue) AxisValue))))))))

(event Input|MouseEvents|MouseX
  (params (AxisValue :type Float%20%28single-precision%29))
  ;[1 1 1] Camera
  ;;[1 1 1] Movement
  ;;;[1 1 1] Edge Movement
  (if (not (Variables|Default|GetDisableCamNav))
    (bind (_deltaxspeed _deltayspeed) (Utilities|ScreenEdgeMovement))
    (Transformation|AddActorLocalOffset (Variables|References|GetCameraPawnRef) (Math|Vector|MakeVector _deltaxspeed _deltayspeed 0.0) true false)))

(event Input|MouseEvents|MouseY
  (params (AxisValue :type Float%20%28single-precision%29))
  ;[1 1 1] Camera
  ;;[1 1 1] Movement
  ;;;[1 1 1] Edge Movement
  (if (not (Variables|Default|GetDisableCamNav))
    (Utilities|ScreenEdgeMovement) ; enters at MouseY
  ))

(event Input|MouseEvents|MouseY
  (params (AxisValue :type Float%20%28single-precision%29))
  (bind _camerapawnref (Variables|References|GetCameraPawnRef))
  (bind _returnvalue (Transformation|GetActorRotation _camerapawnref))
  (bind (_roll _pitch _yaw) (Math|Rotator|BreakRotator _returnvalue))
  ;[1 1 1] Camera
  ;;[1 1 1] Pan
  ;;;[1 1 1] Pan Y
  (Utilities|FlowControl|Gate true
    (:Exit
      (Transformation|SetActorRotation (Variables|References|GetCameraPawnRef) (Math|Rotator|MakeRotator _roll (Math|Float|Clamp(Float) (+ _pitch (* (Variables|Default|GetPanSensitivity) (+ AxisValue (stale Input|GamepadEvents|GamepadRightY AxisValue)))) -15.0 8e+01) _yaw)))))

(event Input|KeyboardEvents|LeftShift
  (params (Key :type Key%20Structure))
  ;[1 1 1] Camera
  ;;[1 1 1] Movement
  ;;;[1 1 1] Move Multiplier
  (:Pressed
    (Variables|Default|SetFastMoveMultiplier 2.0))
  (:Released
    (Variables|Default|SetFastMoveMultiplier 1.0)))

(event Input|MouseEvents|LeftMouseButton
  (params (Key :type Key%20Structure))
  (bind _selectableobjectsenum (Variables|Default|GetSelectableObjectsEnum))
  (bind _hitresult (Class|PlayerController|GetHitResultUnderCursorforObjects _selectableobjectsenum true))
  (bind _hitactor (Collision|BreakHitResult _hitresult))
  ;[1 1 1] Construction
  ;;[1 1 1] Select construction option
  (:Pressed
    (if (Variables|Default|GetBuildModeActive)
      (if (|VertifyAsPlaceable)
        (bind _constructionstruct (Default|GetConstructionStruct (Variables|References|GetGhostBuildingRef)))
        (Default|QueueConstruction (Variables|References|GetConstructionManagerRef) _constructionstruct)
        (Default|KillGhost (Variables|References|GetGhostBuildingRef)))
      (elif (!= _hitactor 0)
        (Default|CallHUDRequest _hitactor) ; call when we click something that we want
      ))))

(event Input|KeyboardEvents|V
  (params (Key :type Key%20Structure))
  (bind _self self)
  (bind _location (CallFunction|SetCursorWorldPosition _self 1e+04))
  ;[1 1 1] Construction
  ;;[1 1 1] Spawn Builder
  (:Pressed
    (Game|SpawnActorfromClass "/Game/TD2020/Blueprints/AI/NPC_BP.NPC_BP_C" (Math|Transform|MakeTransform (Math|Vector|MakeVector (.x _location) (.y _location) 1e+02) "0, 0, 0" "0.500000,0.500000,0.500000") "Undefined" 0 (Variables|References|GetGameStateRef) 0)))

(event Input|TouchEvents|InputTouch
  (params (Location :type Vector) (FingerIndex :type ETouchIndex%20Enum))
  (bind _selectableobjectsenum (Variables|Default|GetSelectableObjectsEnum))
  (bind _hitresult (Class|PlayerController|GetHitResultUnderCursorforObjects _selectableobjectsenum true))
  (bind _hitactor (Collision|BreakHitResult _hitresult))
  ;[1 1 1] Construction
  ;;[1 1 1] Select construction option
  ;;;[1 1 1] Touch
  (:Pressed
    (if (Utilities|Enum|Equal(Enum) FingerIndex "Touch1")
      (if (Variables|Default|GetBuildModeActive)
        (if (|VertifyAsPlaceable)
          (bind _constructionstruct (Default|GetConstructionStruct (Variables|References|GetGhostBuildingRef)))
          (Default|QueueConstruction (Variables|References|GetConstructionManagerRef) _constructionstruct)
          (Default|KillGhost (Variables|References|GetGhostBuildingRef)))
        (elif (!= _hitactor 0)
          (Default|CallHUDRequest _hitactor) ; call when we click something that we want
        ))
      (elif (Utilities|Enum|Equal(Enum) FingerIndex "Touch2") ; Tukaj lahko dodam za move controlls s prsti
        _))))

(fn ConstructionScript)

(fn MovementSpeedCalculation
  (return (Math|Float|Clamp(Float) (/ (Variables|/Script/Engine.SpringArmComponent|GetTargetArmLength (Variables|/Game/TD2020/Blueprints/Camera/CameraPawn.CameraPawn_C|GetSpringArm (Variables|References|GetCameraPawnRef))) 1e+02) 5.0 2e+01)))

(fn SetSightDistance
  (return (+ (Variables|Default|GetSightDistance) (Variables|/Script/Engine.SpringArmComponent|GetTargetArmLength (Variables|/Game/TD2020/Blueprints/Camera/CameraPawn.CameraPawn_C|GetSpringArm (Variables|References|GetCameraPawnRef))))))

(fn SetCalendar
  (params (Date :type Array%20of%20Integers))
  (return false))

(fn SetClock
  (params (Time :type Array%20of%20Integers))
  (return false))