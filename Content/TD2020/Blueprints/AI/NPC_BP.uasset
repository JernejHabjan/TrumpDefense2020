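; NPC pawn Blueprint for TD2020 that generates a random profile and shows its own HUD when selected.
; The construction script randomly picks a sex, tints a dynamic body material to match, and draws a name from that sex's name enum.
; BeginPlay caches the AI and camera controllers, creates the HUD widget and binds to the camera controller's HUD request.
; SetIsBusy writes a busy flag to the AI blackboard.
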(event Custom|DisplayHUD
  (params (Actor :type Actor%20Object%20Reference))
  ;[1 1 1] DisplayHUD
  (if (== Actor self) ; Gets called on selected, if not selected this class, ignore it
    (UserInterface|Viewport|AddtoViewport (Variables|References|GetNPC_HUD) 0)))

(event EventBeginPlay
  ;[1 1 1] BeginPlay
  (Variables|References|SetAIControllerRef (.AsNPC%20AI%20Controller (Utilities|Casting|CastToNPC_AI_Controller (AI|GetAIController self))))
  (bind _output_get (Variables|References|SetCameraControllerRef (.AsCamera%20Pawn%20Controller (Utilities|Casting|CastToCameraPawnController (Game|GetPlayerController 0)))))
  (EventDispatchers|BindEventtoHUDRequest _output_get (EventDispatchers|CreateEvent :!event Custom|DisplayHUD))
  (bind _returnvalue (UserInterface|CreateWidget "/Game/TD2020/HUDs/NPC_HUD.NPC_HUD_C"))
  (Variables|References|SetNPC_HUD _returnvalue))

(fn ConstructionScript
  (CallFunction|RandomNPCFeatures))

(fn RandomNPCFeatures
  (bind _returnvalue (Rendering|Material|CreateDynamicMaterialInstance (Variables|Character|GetMesh) 0 0 :!class /Script/Engine.PrimitiveComponent))
  (LocalVariables|SetMaterialInstance _returnvalue)
  (if (Utilities|Enum|Equal(Enum) (Utilities|Enum|LiteralenumNPCSex_ENUM (Utilities|Enum|ByteToEnumNPCSex_ENUM (Math|Conversions|ToByte(Integer) (Math|Random|RandomIntegerinRange 0 1)))) "NewEnumerator0")
    (Rendering|Material|SetVectorParameterValue (LocalVariables|GetMaterialInstance) "BodyColor" (LocalVariables|GetMaleColor) :!class /Script/Engine.MaterialInstanceDynamic) ; male
    (bind _name (CallFunction|GetRandomName "NewEnumerator0"))
    (Variables|Default|SetMyProfile (Utilities|Struct|MakeNPCProfile_Struct _name "NewEnumerator0"))
    (else
      (Rendering|Material|SetVectorParameterValue (LocalVariables|GetMaterialInstance) "BodyColor" (LocalVariables|GetFemaleColor) :!class /Script/Engine.MaterialInstanceDynamic) ; female
      (bind _name_2 (CallFunction|GetRandomName "NewEnumerator1"))
      (Variables|Default|SetMyProfile (Utilities|Struct|MakeNPCProfile_Struct _name_2 "NewEnumerator1")))))

(fn GetRandomName
  (params (Sex :type NPCSex_ENUM%20Enum :default "NewEnumerator0"))
  (if (Utilities|Enum|Equal(Enum) Sex "NewEnumerator0")
    (return (Utilities|String|EnumtoString (Utilities|Enum|LiteralenumNPCNameMale_ENUM (Utilities|Enum|ByteToEnumNPCNameMale_ENUM (Math|Conversions|ToByte(Integer) (Math|Random|RandomIntegerinRange 0 (- (|GetNumEnumEntries) 1)))))))
    (else
      (return (Utilities|String|EnumtoString (Utilities|Enum|LiteralenumNPCNameFemale_ENUM (Utilities|Enum|ByteToEnumNPCNameFemale_ENUM (Math|Conversions|ToByte(Integer) (Math|Random|RandomIntegerinRange 0 (- (|GetNumEnumEntries) 1))))))))))

(fn SetIsBusy
  (params (IsBusy :type Boolean))
  (AI|Components|Blackboard|SetValueasBool (AI|GetBlackboard (Variables|References|GetAIControllerRef)) (Variables|Default|GetIsBusy) IsBusy)
  (return))