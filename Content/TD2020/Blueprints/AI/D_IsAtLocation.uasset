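; Behavior Tree decorator that checks whether an NPC is at a location chosen by its LocationCheck setting.
; It caches the controlled pawn as an NPC_BP, then switches on LocationCheck.
; Only the Office case is shown, comparing the CurrentLocation blackboard object to the NPC profile's PlaceOfEmployment.
; CurrentLocation is noted as set only while the NPC is at a building, not wandering.
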(fn PerformConditionCheckAI
  (params (OwnerController :type AI%20Controller%20Object%20Reference) (ControlledPawn :type Pawn%20Object%20Reference))
  (|ReferenceCast ControlledPawn)
  (switch Utilities|FlowControl|Switch|SwitchonLocationType_ENUM (Variables|Default|GetLocationCheck)
    (:NewEnumerator2
      ;[1 1 1] Office
      (return (== (Class|BTFunctionLibrary|GetBlackboardValueasObject (Variables|Default|GetCurrentLocation)) (.placeofemployment (Variables|/Game/TD2020/Blueprints/AI/NPC_BP.NPC_BP_C|GetMyProfile (Variables|Default|GetPawn))))))))