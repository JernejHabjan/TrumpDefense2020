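; Base resource node actor that scatters a resource field in the level and registers itself with MyGameState on BeginPlay.
; Construction script reads Resources_DT, sizes the spawn, production and placement boxes and decal, then adds seeded random mesh instances snapped to the ground by line trace.
; Ghost buildings overlapping the meshes are forced to a bad location.
; Those entering PlaceableArea receive this resource, cleared on exit.
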(event OnComponentBeginOverlap(InstancedResourceMesh)
  (params (OverlappedComponent :type Primitive%20Component%20Object%20Reference) (OtherActor :type Actor%20Object%20Reference) (OtherComp :type Primitive%20Component%20Object%20Reference) (OtherBodyIndex :type Integer) (bFromSweep :type Boolean) (SweepResult :type Hit%20Result%20Structure%20%28by%20ref%29))
  ;[1 1 1] On component begin overlap
  (bind _asghost_building_bp (Utilities|Casting|CastToGhostBuilding_BP OtherActor)) ; is it ghost building?
  (Variables|/Game/TD2020/Blueprints/Buildings/GhostBuilding_BP.GhostBuilding_BP_C|SetForceBadLocation _asghost_building_bp true) ; forces unplacable if placed on rocks etc
)

(event OnComponentEndOverlap(InstancedResourceMesh)
  (params (OverlappedComponent :type Primitive%20Component%20Object%20Reference) (OtherActor :type Actor%20Object%20Reference) (OtherComp :type Primitive%20Component%20Object%20Reference) (OtherBodyIndex :type Integer))
  ;[1 1 1] On component end overlap
  (bind _asghost_building_bp (Utilities|Casting|CastToGhostBuilding_BP OtherActor)) ; is it ghost building?
  (Variables|/Game/TD2020/Blueprints/Buildings/GhostBuilding_BP.GhostBuilding_BP_C|SetForceBadLocation _asghost_building_bp false))

(event OnComponentBeginOverlap(PlaceableArea)
  (params (OverlappedComponent :type Primitive%20Component%20Object%20Reference) (OtherActor :type Actor%20Object%20Reference) (OtherComp :type Primitive%20Component%20Object%20Reference) (OtherBodyIndex :type Integer) (bFromSweep :type Boolean) (SweepResult :type Hit%20Result%20Structure%20%28by%20ref%29))
  ;[1 1 1] On component begin overlap
  (bind _asghost_building_bp (Utilities|Casting|CastToGhostBuilding_BP OtherActor))
  (Default|SetResource _asghost_building_bp self))

(event OnComponentEndOverlap(PlaceableArea)
  (params (OverlappedComponent :type Primitive%20Component%20Object%20Reference) (OtherActor :type Actor%20Object%20Reference) (OtherComp :type Primitive%20Component%20Object%20Reference) (OtherBodyIndex :type Integer))
  ;[1 1 1] On component end overlap
  (bind _asghost_building_bp (Utilities|Casting|CastToGhostBuilding_BP OtherActor))
  (Default|ClearResource _asghost_building_bp))

(event EventBeginPlay
  ;[1 1 1] BeginPlay
  (Utilities|IsValid (Variables|References|GetGameStateRef)
    (:Is%20Not%20Valid
      (bind _output_get (Variables|References|SetGameStateRef (.AsMy%20Game%20State (Utilities|Casting|CastToMyGameState (Game|GetGameState)))))
      (Default|AddResource _output_get self))))

(fn ConstructionScript
  (bind _spawnareavolume (Variables|Default|GetSpawnAreaVolume))
  (bind _instancedresourcemesh (Variables|Default|GetInstancedResourceMesh))
  (bind _placeablearea (Variables|Default|GetPlaceableArea))
  (bind _spawnareavolume_2 (Variables|Default|GetSpawnAreaVolume))
  (bind _randomlocationseed (Variables|ResourcesPrimary|GetRandomLocationSeed))
  (bind _randomrotationseed (Variables|ResourcesPrimary|GetRandomRotationSeed))
  (bind _returnvalue (Class|KismetMathLibrary|RandomRotatorfromStream true _randomrotationseed))
  (bind _returnvalue_2 (Transformation|GetWorldLocation _spawnareavolume))
  (bind _boxextent (Variables|/Script/Engine.BoxComponent|GetBoxExtent _spawnareavolume))
  (bind _boxextent_2 (Variables|/Script/Engine.BoxComponent|GetBoxExtent _placeablearea))
  (bind _boxextent_3 (Variables|/Script/Engine.BoxComponent|GetBoxExtent _spawnareavolume_2))
  (bind _returnvalue_3 (Utilities|GetDataTableRow "/Game/TD2020/DataTables/Resources_DT.Resources_DT" (Utilities|String|StringToName (Utilities|String|EnumtoString (Variables|Default|GetResource))))
    (:then
      (bind _output_get (Variables|Default|SetResourceStruct _returnvalue_3))
      (Components|StaticMesh|SetStaticMesh (Variables|Default|GetInstancedResourceMesh) (.ResourceMesh (Utilities|Struct|BreakResources_Struct _output_get)))
      (Components|Box|SetBoxExtent (Variables|Default|GetSpawnAreaVolume) (Variables|ResourcesPrimary|GetSpawnAreaSize) true) ; extent is half height from pivot point
      (Components|Box|SetBoxExtent (Variables|Default|GetProductionVolume) (+ (Variables|ResourcesPrimary|GetSpawnAreaSize) (Variables|Default|GetProductionVolumeSize)) true)
      (Components|Box|SetBoxExtent (Variables|Default|GetPlaceableArea) (+ (Variables|ResourcesPrimary|GetBuildingPlacementBounds) (Variables|ResourcesPrimary|GetSpawnAreaSize)) true)
      (Transformation|SetRelativeScale3D (Variables|Default|GetGoodPlacementDecal) (Math|Vector|MakeVector (.z _boxextent_2) (.y _boxextent_2) (.x _boxextent_2)))
      (for _index (range 1 (Variables|ResourcesPrimary|GetLevels))
        (bind _returnvalue_4 (Components|InstancedStaticMesh|AddInstance _instancedresourcemesh (Math|Transform|MakeTransform (Math|Vector|MakeVector (Math|Random|RandomFloatinRangefromStream (* (.x _boxextent_3) -1.0) (.x _boxextent_3) _randomlocationseed) (Math|Random|RandomFloatinRangefromStream (* (.y _boxextent_3) -1.0) (.y _boxextent_3) _randomlocationseed) (.z _boxextent_3)) (Math|Rotator|MakeRotator (Math|Float|Clamp(Float) (.roll _returnvalue) 0.0 (Variables|ResourcesPrimary|GetRollRotationTreshold)) (Math|Float|Clamp(Float) (.pitch _returnvalue) 0.0 (Variables|ResourcesPrimary|GetPitchRotationTreshold)) (Math|Float|Clamp(Float) (.yaw _returnvalue) 0.0 (Variables|ResourcesPrimary|GetYawRotationTreshold))) (/ (Transformation|GetWorldScale (Variables|Default|GetInstancedResourceMesh)) 2.0))))
        (bind _output_get_2 (LocalVariables|SetInstanceIndex_LOCAL _returnvalue_4))
        (bind _outhit (Collision|LineTraceByChannel (.location (.OutInstanceTransform (Components|InstancedStaticMesh|GetInstanceTransform _instancedresourcemesh _output_get_2 true))) (Math|Vector|MakeVector (.X (Math|Vector|BreakVector (.location (.OutInstanceTransform (Components|InstancedStaticMesh|GetInstanceTransform _instancedresourcemesh _output_get_2 true))))) (.Y (Math|Vector|BreakVector (.location (.OutInstanceTransform (Components|InstancedStaticMesh|GetInstanceTransform _instancedresourcemesh _output_get_2 true))))) (Variables|ResourcesPrimary|GetTraceZDistance)) "TraceTypeQuery3" false 0 "None"))
        (Components|InstancedStaticMesh|UpdateInstanceTransform (Variables|Default|GetInstancedResourceMesh) (LocalVariables|GetInstanceIndex_LOCAL) (Math|Transform|MakeTransform (Math|Vector|MakeVector (.x (.TraceStart (Collision|BreakHitResult _outhit))) (.y (.TraceStart (Collision|BreakHitResult _outhit))) (Math|Float|Clamp(Float) (.z (.ImpactPoint (Collision|BreakHitResult _outhit))) (- (.z _returnvalue_2) (.z _boxextent)) (+ (.z _returnvalue_2) (.z _boxextent)))) (.rotation (.OutInstanceTransform (Components|InstancedStaticMesh|GetInstanceTransform (Variables|Default|GetInstancedResourceMesh) (LocalVariables|GetInstanceIndex_LOCAL) false))) (.scale (.OutInstanceTransform (Components|InstancedStaticMesh|GetInstanceTransform (Variables|Default|GetInstancedResourceMesh) (LocalVariables|GetInstanceIndex_LOCAL) false)))) true false false)))))