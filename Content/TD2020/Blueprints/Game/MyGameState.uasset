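; Game state that runs the in-game clock and calendar and shows both on the main HUD.
; Each tick advances a Clockwork time value scaled by TimeUnit, splits it into seconds, minutes and hours, and adds DayTick to roll days, months and years.
; UpdateGameStateSpeed rescales TimeUnit from the default speed and passes it to CallUpdateGameSpeed.
; SetClock and SetCalendar are stubs returning false.
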(event EventBeginPlay
  ;[1 1 1] Begin Play
  (Variables|References|SetControllerRef (.AsCamera%20Pawn%20Controller (Utilities|Casting|CastToCameraPawnController (Game|GetPlayerController 0))))
  (Variables|Default|SetClockwork (+ (Math|Conversions|ToFloat(Integer) (Variables|Default|GetHours)) (Math|Conversions|ToFloat(Integer) (Variables|Default|GetMinutes)) (Math|Conversions|ToFloat(Integer) (Variables|Default|GetSeconds))))
  (Variables|Default|SetGameDate (Utilities|Array|MakeArray (Variables|Default|GetDay) (Variables|Default|GetMonth) (Variables|Default|GetYear)))
  (Variables|Components|SetMainUIRef (Variables|/Game/TD2020/Blueprints/Camera/CameraPawnController.CameraPawnController_C|GetMainHudRef (Variables|References|GetControllerRef)))
  (Variables|Default|SetTimeUnit (Variables|Default|GetDefaultGameSpeed)))

(event EventTick
  (params (DeltaSeconds :type Float%20%28single-precision%29))
  ;[1 1 1] Tick
  (Variables|Default|SetClockwork (.ClockworkOut (CallFunction|SetClockwork DeltaSeconds (Variables|Default|GetTimeUnit) (Variables|Default|GetClockwork)))) ; remainder of 24
  (Variables|Default|SetDayTick (.DayTick (CallFunction|SetClockwork DeltaSeconds (Variables|Default|GetTimeUnit) (Variables|Default|GetClockwork))))
  (CallFunction|Clock)
  (CallFunction|Calendar))

(event EventUpdateGameStateSpeed
  (params (Multiplier :type Float%20%28single-precision%29))
  ;[1 1 1] Update Game Speed
  (bind _output_get (Variables|Default|SetTimeUnit (* Multiplier (Variables|Default|GetDefaultGameSpeed))))
  (Default|CallUpdateGameSpeed _output_get))

(fn ConstructionScript)

(fn Clock
  (bind _clockwork (Variables|Default|GetClockwork))
  (bind _returnvalue (* _clockwork 3.6e+03))
  (bind (_remainder _returnvalue_2) (Math|Float|Division(WholeandRemainder) _returnvalue 6e+01))
  (bind _returnvalue_3 (Math|Conversions|ToFloat(Integer) _returnvalue_2))
  (bind (_remainder_2 _returnvalue_4) (Math|Float|Division(WholeandRemainder) _returnvalue_3 6e+01))
  (Variables|Default|SetSeconds (Math|Float|Floor _remainder))
  (Variables|Default|SetMinutes (Math|Float|Floor _remainder_2))
  (Variables|Default|SetHours (Math|Float|Floor (.Remainder (Math|Float|Division(WholeandRemainder) (Math|Conversions|ToFloat(Integer) _returnvalue_4) 24.0))))
  (bind _output_get (Variables|Default|SetGameTime (Utilities|Array|MakeArray (Variables|Default|GetSeconds) (Variables|Default|GetMinutes) (Variables|Default|GetHours))))
  (Class|IHUD|SetClock(Message) (Variables|/Game/TD2020/Blueprints/Camera/CameraPawnController.CameraPawnController_C|GetMainHudRef (Variables|References|GetControllerRef)) _output_get))

(fn Calendar
  (bind _output_get (Variables|Default|SetDay (+ (Variables|Default|GetDayTick) (Variables|Default|GetDay))))
  (if (> _output_get (Class|KismetMathLibrary|DaysinMonth (Variables|Default|GetYear) (Variables|Default|GetMonth)))
    (Variables|Default|SetDay 1) ; we reached the end of the month
    (Math|Integer|IncrementInt (Variables|Default|GetMonth) ; increment month
      (:%20%20
        _)))
  (if (> (Variables|Default|GetMonth) 12)
    (Variables|Default|SetMonth 1)
    (Math|Integer|IncrementInt (Variables|Default|GetYear)
      (:%20%20
        _)))
  (bind _output_get_2 (Variables|Default|SetGameDate (Utilities|Array|MakeArray (Variables|Default|GetDay) (Variables|Default|GetMonth) (Variables|Default|GetYear))))
  (Class|IHUD|SetCalendar(Message) (Variables|/Game/TD2020/Blueprints/Camera/CameraPawnController.CameraPawnController_C|GetMainHudRef (Variables|References|GetControllerRef)) _output_get_2) ; set HUD calendar
)

(fn GetCurrentTimeUnit
  (return (Variables|Default|GetTimeUnit)))

(fn SetCalendar
  (params (Date :type Array%20of%20Integers))
  (return false))

(fn SetClock
  (params (Time :type Array%20of%20Integers))
  (return false))