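; BuildingMaster_BP is a master building actor that sets up its mesh, entrance and collision box on construction and tracks its employees.
; On BeginPlay it creates its own HUD widget and binds to the camera controller's HUD request event.
; When selected, it lerps the camera pawn to itself via a timeline macro, shows the HUD in UI-only input, and disables camera navigation and the main HUD.
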(event Custom|DisplayHUD
  (params (Actor :type Actor%20Object%20Reference))
  (bind _controllerref (Variables|References|GetControllerRef))
  ;[1 1 1] DisplayHUD
  (if (== Actor self) ; ignore if youre not
    (Utilities|FlowControl|Sequence
      (:then_0
        (bind _newlocation (|LerpLocation) ; update is kinda like tick - lerps between old and new location
          (:Update
            (Transformation|SetActorLocation (Variables|/Game/TD2020/Blueprints/Camera/CameraPawnController.CameraPawnController_C|GetCameraPawnRef (Variables|References|GetControllerRef)) _newlocation false false))))
      (:then_1
        (UserInterface|Viewport|AddtoViewport (Variables|References|GetBuildingHUD) 0)
        (Input|SetInputModeUIOnly _controllerref (Variables|References|GetBuildingHUD) "LockAlways") ; disables our keyboard functions
        (Variables|/Game/TD2020/Blueprints/Camera/CameraPawnController.CameraPawnController_C|SetDisableCamNav _controllerref true)
        (Widget|SetIsEnabled (Variables|/Game/TD2020/Blueprints/Camera/CameraPawnController.CameraPawnController_C|GetMainHudRef _controllerref) false) ; disable creating buildings
      ))))

(event EventBeginPlay
  ;[1 1 1] BeginPlay
  (bind _output_get (Variables|References|SetControllerRef (.AsCamera%20Pawn%20Controller (Utilities|Casting|CastToCameraPawnController (Game|GetPlayerController 0)))))
  (EventDispatchers|BindEventtoHUDRequest _output_get (EventDispatchers|CreateEvent :!event Custom|DisplayHUD)) ; when we click something usefull in camera pawn controller this gets called
  (bind _returnvalue (UserInterface|CreateWidget "/Game/TD2020/HUDs/Building_HUD.Building_HUD_C" 0 self (Variables|References|GetControllerRef))) ; building hud
  (Variables|References|SetBuildingHUD _returnvalue))

(fn ConstructionScript
  (Components|StaticMesh|SetStaticMesh (Variables|Components|GetStaticMesh) (Variables|References|GetDisplayMesh))
  (CallFunction|SetBuildingEntrance (Variables|Components|GetEntrance) (Variables|Components|GetStaticMesh))
  (CallFunction|SetBuildingCollisionBox (Variables|Components|GetCollision) (Variables|Components|GetStaticMesh))
  (Development|PrintString "Building master created"))

(fn GetEmployees
  (bind _employees (Variables|Default|GetEmployees))
  (bind _returnvalue (Utilities|Array|Length _employees))
  (return (> _returnvalue 0) _returnvalue _employees))