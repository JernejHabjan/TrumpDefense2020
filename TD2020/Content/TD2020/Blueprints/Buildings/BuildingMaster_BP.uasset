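; Base building actor for the TD2020 RTS, handling setup, staffing, residents, unit spawning and death.
; BeginPlay registers the building, updates requirements and sets health from actor data on authority; construction places the entrance and default rally point.
; Hiring, jobs and tenancy route to optional construction and vacancy components, while entering characters are hidden with stamina drain paused.
; Units spawn through the Commander above the entrance; the first-of-kind unlock is unfinished.
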(event EventBeginPlay
  ;[1 1 1] BeginPlay
  (|CallParentFunction)
  (CallFunction|CheckFirstOfItsKind (Utilities|GetClass self))
  ;;[1 1 1] TODO WHERE TO PLACE THIS
  (Networking|SwitchHasAuthority
    (:Authority
      (Default|AddBuildingtoGame (Variables|Default|GetGameStateRef) self)
      (CallFunction|UpdateRequirements (Variables|Default|GetCommander))
      (CallFunction|SetHealth))))

(event EventTick
  (params (DeltaSeconds :type Float%20%28single-precision%29))
  ;[1 1 1] Tick
  (Utilities|FlowControl|Delay 0.1)
  (Default|UpdateRallytoActor (Variables|Default|GetTD2020RallyComponent)))

(fn ConstructionScript
  (|CallParentFunction)
  (Components|StaticMesh|SetStaticMesh (Variables|Default|GetActorStaticMesh) (Variables|References|GetDisplayMesh))
  (CallFunction|SetBuildingCollisionBox (Variables|Components|GetEntranceCollision) (Variables|Default|GetActorStaticMesh))
  (Transformation|SetWorldLocation (Variables|Components|GetEntrance) (Transformation|GetWorldLocation (Variables|Components|GetEntranceSphere)) false false)
  (Default|SetRally (Variables|Default|GetTD2020RallyComponent) (Transformation|GetWorldLocation (Variables|Components|GetEntrance)))
  (Variables|Default|SetListName "InfantryList"))

(fn AssignEmployeeJob
  (params (Employee :type NPC%20Object%20Reference))
  (bind _returnvalue (Actor|GetComponentbyClass "/Game/TD2020/Blueprints/Components/TD2020ConstructionComponent.TD2020ConstructionComponent_C"))
  (Utilities|IsValid _returnvalue
    (:Is%20Valid
      (bind (_jobassigned _jobinstance _joblocation) (Default|AssignEmployeeJob _returnvalue Employee))
      (return _jobassigned _jobinstance _joblocation) ; actor because it may work on a tree or mine rocks
    )
    (:Is%20Not%20Valid
      (Development|PrintString (Utilities|String|Append "Building of type >" (Utilities|GetClassDisplayName (Utilities|GetClass self)) "< doesn't have construction component - cannot assign employee job") true true "(R=1.000000,G=0.000000,B=0.014766,A=1.000000)" 1e+01)
      (return false 0 "0, 0, 0"))))

(fn EnterBuilding
  (params (Character :type Base%20Character%20Object%20Reference))
  (bind _aicontroller (Variables|/Game/TD2020/Blueprints/AI/Characters/BaseCharacter.BaseCharacter_C|GetAIController Character))
  (Rendering|SetActorHiddenInGame Character true) ; dissapear
  (Utilities|Time|PauseTimerbyHandle (Variables|/Game/TD2020/Blueprints/AI/CharacterAIController.CharacterAIController_C|GetDepleteStaminaHandle _aicontroller)) ; we no longer deplete stamina
  (Default|SwitchSleep _aicontroller)
  (return true))

(fn ExitBuilding
  (params (Character :type Base%20Character%20Object%20Reference))
  (bind _aicontroller (Variables|/Game/TD2020/Blueprints/AI/Characters/BaseCharacter.BaseCharacter_C|GetAIController Character))
  (Rendering|SetActorHiddenInGame Character false)
  (Utilities|Time|UnpauseTimerbyHandle (Variables|/Game/TD2020/Blueprints/AI/CharacterAIController.CharacterAIController_C|GetDepleteStaminaHandle _aicontroller)) ; starts depleting stamina again
  (Utilities|Time|ClearandInvalidateTimerbyHandle (Variables|/Game/TD2020/Blueprints/AI/CharacterAIController.CharacterAIController_C|GetRegainStaminaHandle _aicontroller))
  (Default|SwitchSleep _aicontroller)
  (return true))

(fn GetOccupants
  (LocalVariables|SetHasOccupants_LOCAL false)
  (LocalVariables|SetNumberOfOccupants_LOCAL 0)
  (LocalVariables|SetListOfOccupants_LOCAL (Utilities|Array|MakeArray 0))
  (bind (_rtsselectable _rtsowner _td2020attackable _td2020health _rtsproductioncost _rtsproduction _td2020constructionsite _rtsname _rtsportrait _td2020construction _td2020vacancy) (CallFunction|GetComponents))
  (Utilities|IsValid _td2020construction
    (:Is%20Valid
      (LocalVariables|SetHasOccupants_LOCAL (.HasEmployees (Default|GetEmployees _td2020construction)))
      (LocalVariables|SetNumberOfOccupants_LOCAL (+ (LocalVariables|GetNumberOfOccupants_LOCAL) (.NumberOfEmployees (Default|GetEmployees _td2020construction))))
      (Utilities|Array|AppendArray (LocalVariables|GetListOfOccupants_LOCAL) (.ListOfEmployees (Default|GetEmployees _td2020construction)))
      (Utilities|IsValid _td2020vacancy
        (:Is%20Valid
          (LocalVariables|SetHasOccupants_LOCAL (or (.HasOccupants (Default|GetOccupants _td2020vacancy)) (LocalVariables|GetHasOccupants_LOCAL)))
          (LocalVariables|SetNumberOfOccupants_LOCAL (+ (LocalVariables|GetNumberOfOccupants_LOCAL) (.NumberOfOccupants (Default|GetOccupants _td2020vacancy))))
          (Utilities|Array|AppendArray (LocalVariables|GetListOfOccupants_LOCAL) (.ListOfOccupants (Default|GetOccupants _td2020vacancy))))
        (:Is%20Not%20Valid
          _)))
    (:Is%20Not%20Valid
      _))
  (return (LocalVariables|GetHasOccupants_LOCAL) (LocalVariables|GetNumberOfOccupants_LOCAL) (LocalVariables|GetListOfOccupants_LOCAL)))

(fn ToCommanderSpawnUnit
  (params (InUnit :type Base%20Character%20Class%20Reference))
  (bind _commander (Variables|Default|GetCommander))
  (bind _entrance (Variables|Components|GetEntrance))
  (bind _returnvalue (Transformation|GetWorldTransform _entrance))
  (Default|ROSSpawnUnit _commander InUnit (Math|Transform|MakeTransform (Math|Vector|MakeVector (.x (.location _returnvalue)) (.y (.location _returnvalue)) (+ (.z (.location _returnvalue)) 1e+02)) (.rotation _returnvalue) (.scale _returnvalue)) _commander (Default|GetRallyPoint (Variables|Default|GetTD2020RallyComponent)))
  (CallFunction|SetFloatingText (Utilities|GetClassDisplayName InUnit) (Math|Color|MakeColor 0.0 1.0 1.0) 2.0))

(fn HireEmployee
  (params (Applicant :type NPC%20Object%20Reference))
  (LocalVariables|SetApplicant_LOCAL Applicant)
  (bind (_rtsselectable _rtsowner _td2020attackable _td2020health _rtsproductioncost _rtsproduction _td2020constructionsite _rtsname _rtsportrait _td2020construction _td2020vacancy _rtsresourcedrain) (CallFunction|GetComponents))
  (Utilities|IsValid _rtsresourcedrain ; first check for resource mining
    (:Is%20Valid
      _)
    (:Is%20Not%20Valid
      (Utilities|IsValid _td2020construction
        (:Is%20Valid
          (bind _washired (Default|HireEmployee _td2020construction (LocalVariables|GetApplicant_LOCAL)))
          (return _washired self))
        (:Is%20Not%20Valid
          _))))
  ;[1 1 1] For mining etc - NOT DEFINED COMPONENT - if it doesnt need extra functions like construction does - i can change this later - not essential
  (if (< (.NumberOfOccupants (CallFunction|GetOccupants)) (.MaxEmployees (Utilities|Struct|BreakBuilding_STRUCT_02 (Variables|BuildingInfo|GetBuildingStruct))))
    (Utilities|Array|AddUnique (Variables|Default|GetEmployees_BP) (LocalVariables|GetApplicant_LOCAL))
    (return true self)
    (else
      (return false 0))))

(fn SetCurrentJob
  (params (CurrentJobSite :type Construction%20Proxy%20Object%20Reference))
  (bind _td2020construction (CallFunction|GetComponents))
  (Utilities|IsValid _td2020construction
    (:Is%20Valid
      (Default|SetCurrentJob _td2020construction CurrentJobSite)
      (return 0))))

(fn SetNewTenant
  (params (NPC :type NPC%20Object%20Reference%20%28by%20ref%29))
  (bind _td2020vacancy (CallFunction|GetComponents))
  (Utilities|IsValid _td2020vacancy
    (:Is%20Valid
      (Default|SetNewTenant _td2020vacancy NPC))
    (:Is%20Not%20Valid
      (Development|PrintString (Utilities|String|Append "New Tenant cannot be set in >" (Utilities|GetClassDisplayName (Utilities|GetClass self)) "<") true true "(R=1.000000,G=0.093044,B=0.000000,A=1.000000)" 1e+01))))

(fn ApplyforResidency
  (bind _td2020vacancy (CallFunction|GetComponents))
  (Utilities|IsValid _td2020vacancy
    (:Is%20Valid
      (bind _accepted (Default|ApplyforResidency _td2020vacancy))
      (return _accepted))
    (:Is%20Not%20Valid
      (Development|PrintString (Utilities|String|Append "Applying for residency cannot continue in >" (Utilities|GetClassDisplayName (Utilities|GetClass self)) "<") true true "(R=1.000000,G=0.093044,B=0.000000,A=1.000000)" 1e+01)
      (return false))))

(fn CheckFirstOfItsKind
  (params (ActorClass :type Building%20Master%20BP%20Class%20Reference))
  (bind _commander (Variables|Default|GetCommander))
  (Utilities|IsValid _commander
    (:Is%20Valid
      (if (Pawn|IsLocallyControlled _commander)
        (bind _outactors (Actor|GetAllActorsOfClass ActorClass))
        (for _array_element _outactors
          (Utilities|IsValid (Variables|/Game/TD2020/Blueprints/GeneralActor.GeneralActor_C|GetCommander _array_element)
            (:Is%20Valid
              (if (and (Pawn|IsLocallyControlled (Variables|/Game/TD2020/Blueprints/GeneralActor.GeneralActor_C|GetCommander _array_element)) (CallFunction|CheckTeams (Variables|/Game/TD2020/Blueprints/GeneralActor.GeneralActor_C|GetCommander _array_element) (Variables|Default|GetCommander)))
                (Math|Integer|IncrementInt (Variables|Default|GetNumberOfSimilarBuilding))))))))))

(fn RMBHit
  (params (InCommander :type Actor%20Object%20Reference))
  (return 0))

(fn GetComponents
  (bind (_rtsselectable _rtsowner _td2020attackable _td2020health _rtsproductioncost _rtsproduction _td2020constructionsite _rtsname _rtsportrait _td2020construction _td2020vacancy _rtsresourcedrain) (|CallParentFunction))
  (return _rtsselectable _rtsowner (Variables|Default|GetTD2020Attackable) (Variables|Default|GetTD2020Health) _rtsproductioncost _rtsproduction _td2020constructionsite _rtsname _rtsportrait _td2020construction _td2020vacancy _rtsresourcedrain))

(fn OnDeath
  (|CallParentFunction)
  (Utilities|IsValid self ; if its not called on destroy
    (:Is%20Valid
      (Actor|DestroyActor))
    (:Is%20Not%20Valid
      _))
  (return 0))

(fn CreateWidgets
  (|CallParentFunction)
  (bind _returnvalue (UserInterface|CreateWidget "/Game/TD2020/Widgets/HUDs/HumanWidgets/WB_Human_InfantryList.WB_Human_InfantryList_C" 0 (Variables|Default|GetCommander) self (Utilities|String|ToString(Text) (Class|RTSNameComponent|GetName (Variables|Default|GetRTSName)))))
  (Default|InitButtons _returnvalue)
  (Variables|Default|SetListWidget _returnvalue)
  (Variables|Default|SetListName "InfantryList")
  (return 0))

(fn SetHealth
  (bind _self self)
  (bind _returnvalue (Utilities|GetClass _self))
  (bind _myactordata (CallFunction|RetrieveActorData _returnvalue))
  (bind _maxhealth (Utilities|Struct|BreakS_MyActor _myactordata))
  (Variables|/Script/TD2020.TD2020HealthComponent|SetMaximumHealth (Variables|Default|GetTD2020Health) _maxhealth)
  (Variables|/Script/TD2020.TD2020HealthComponent|SetCurrentHealth (Variables|Default|GetTD2020Health) _maxhealth))