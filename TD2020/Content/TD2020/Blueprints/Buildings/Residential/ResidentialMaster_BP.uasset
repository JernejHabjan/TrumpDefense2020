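; Master residential building Blueprint that houses NPC tenants and lets them go inside to sleep.
; Residents are kept in a unique list, and residency applications succeed while the count is below the building struct's maximum.
; Entering hides the NPC, pauses its AI controller's stamina-drain timer and switches sleep state.
; Exiting unhides it, resumes drain, clears the stamina-regain timer and switches sleep again.
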(fn ConstructionScript
  (|CallParentFunction))

(fn GetVacancy
  (return (< (.NumberOfOccupants (CallFunction|GetOccupants)) (.MaxResidents (Utilities|Struct|BreakBuilding_STRUCT_02 (Variables|Default|GetBuildingStruct_BP))))))

(fn ApplyforResidency
  (bind _hasvacancy (CallFunction|GetVacancy))
  (return _hasvacancy))

(fn SetNewTenant
  (params (NPC :type NPC%20BP%20Object%20Reference))
  (Utilities|Array|AddUnique (Variables|Default|GetResidents_BP) NPC)
  (return))

(fn EnterBuilding
  (params (NPC :type NPC%20BP%20Object%20Reference))
  (bind _aicontroller (Variables|/Game/TD2020/Blueprints/AI/Characters/0_Base.0_Base_C|GetAIController NPC))
  (Rendering|SetActorHiddenInGame NPC true) ; dissapear
  (Utilities|Time|PauseTimerbyHandle (Variables|/Game/TD2020/Blueprints/AI/CharacterAIController.CharacterAIController_C|GetDepleteStaminaHandle _aicontroller)) ; we no longer deplete stamina
  (Default|SwitchSleep _aicontroller)
  (return true))

(fn ExitBuilding
  (params (NPC :type NPC%20BP%20Object%20Reference))
  (bind _aicontroller (Variables|/Game/TD2020/Blueprints/AI/Characters/0_Base.0_Base_C|GetAIController NPC))
  (Rendering|SetActorHiddenInGame NPC false)
  (Utilities|Time|UnpauseTimerbyHandle (Variables|/Game/TD2020/Blueprints/AI/CharacterAIController.CharacterAIController_C|GetDepleteStaminaHandle _aicontroller)) ; starts depleting stamina again
  (Utilities|Time|ClearandInvalidateTimerbyHandle (Variables|/Game/TD2020/Blueprints/AI/CharacterAIController.CharacterAIController_C|GetRegainStaminaHandle _aicontroller))
  (Default|SwitchSleep _aicontroller)
  (return true))

(fn GetOccupants
  (bind _residents_bp (Variables|Default|GetResidents_BP))
  (bind _returnvalue (Utilities|Array|Length _residents_bp))
  (return (> _returnvalue 0) _returnvalue _residents_bp))