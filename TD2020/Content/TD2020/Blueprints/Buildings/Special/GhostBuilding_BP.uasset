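; Placement preview actor for buildings: a ghost mesh that follows the grid-snapped cursor while the player is in build mode.
; ConstructBuilding briefly spawns the building to copy its mesh, proxy and proximity type, then sets up the ghost at a camera-based stepped yaw.
; GetSurroundingGrid classifies footprint tiles using overlap, resource-proximity and slope checks, swapping OK and error materials.
; GetConstructionStruct packages class, proxy, transform and builder as construction data.
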(event Custom|OnSpawn
  (params (DisplayMesh :type Static%20Mesh%20Object%20Reference) (BuildingClass :type Building%20Master%20BP%20Class%20Reference) (ConstructionProxy :type Construction%20Proxy%20Class%20Reference) (ProximityType :type EProximityType_Enum%20Enum :default "None"))
  (bind _arrow (Variables|Components|GetArrow))
  ;[1 1 1] On Spawn Ghost
  (if (not (Variables|Default|GetIsActive))
    (Variables|Default|SetBuildingClass BuildingClass)
    (Variables|Default|SetConstructionProxy ConstructionProxy)
    (Variables|References|SetDisplayMesh DisplayMesh)
    (Variables|Default|SetProximityType ProximityType)
    (CallFunction|InitProximity)
    (Variables|Default|SetIsActive true) ; so this cant be called again when we have mesh on mouse
    (Variables|/Game/TD2020/Blueprints/Pawns/Pawn_MasterCommander.Pawn_MasterCommander_C|SetBuildModeActive (.AsPawn%20Master%20Commander (Utilities|Casting|CastToPawn_MasterCommander (Game|Player|GetPlayerPawn 0))) true)
    (Components|StaticMesh|SetStaticMesh (Variables|Components|GetGhostBuilding_Mesh) (Variables|References|GetDisplayMesh))
    (CallFunction|OpenTickGate) ; opens custom event
    (CallFunction|SetMaterial (not (Variables|Default|GetIsOverlapping))) ; set ghost material
    (bind _output_get (Variables|Default|SetExtent (.BoxExtent (Collision|GetComponentBounds (Variables|Components|GetGhostBuilding_Mesh)))))
    (Transformation|SetRelativeLocation _arrow (Math|Vector|MakeVector 0.0 (.y _output_get) 0.0) false false)
    (Development|SetHiddeninGame _arrow false false)
    (Transformation|SetActorRotation (Math|Rotator|MakeRotator 0.0 0.0 (+ (CallFunction|SetInitialRotation) 9e+01)))
    (CallFunction|SetBuildingCollisionBox (Variables|Components|GetEntranceCollision) (Variables|Components|GetGhostBuilding_Mesh))))

(event Custom|SetMaterial
  (params (IsError :type Boolean))
  (bind _ghostbuilding_mesh (Variables|Components|GetGhostBuilding_Mesh))
  ;[1 1 1] SetMaterial
  (if (not (Math|Boolean|Equal(Boolean) IsError (Variables|Default|GetIsOverlapping))) ; if equal dont do anything
    (bind _output_get (Variables|Default|SetIsOverlapping IsError))
    (if _output_get
      (Rendering|Material|SetMaterial _ghostbuilding_mesh 0 "/Game/TD2020/Materials/GhostErr_M_Inst.GhostErr_M_Inst") ; set ERR material
      (else
        (Rendering|Material|SetMaterial _ghostbuilding_mesh 0 "/Game/TD2020/Materials/Ghost_M_Inst.Ghost_M_Inst") ; set OK material
      ))))

(event Custom|OpenTickGate
  ;[1 1 1] Tick
  (Utilities|FlowControl|Gate true) ; enters at Open
)

(event Custom|CloseTickGate
  ;[1 1 1] Tick
  (Utilities|FlowControl|Gate true) ; enters at Close
)

(event Custom|KillGhost
  ;[1 1 1] Kill Ghost
  (Variables|Default|SetBuildingClass 0)
  (Variables|Default|SetConstructionProxy 0)
  (CallFunction|CloseTickGate)
  (Variables|References|SetDisplayMesh 0)
  (Variables|Default|SetIsActive false)
  (CallFunction|DeinitializeProximity)
  (Variables|/Game/TD2020/Blueprints/Pawns/Pawn_MasterCommander.Pawn_MasterCommander_C|SetBuildModeActive (.AsPawn%20Master%20Commander (Utilities|Casting|CastToPawn_MasterCommander (Game|Player|GetPlayerPawn 0))) false)
  (Components|StaticMesh|SetStaticMesh (Variables|Components|GetGhostBuilding_Mesh) 0) ; set to empty display mesh
  (Transformation|SetActorRotation "0, 0, 0") ; remove rotation from actors
  (Development|SetHiddeninGame (Variables|Components|GetArrow) true false)
  (Components|Box|SetBoxExtent (Variables|Components|GetEntranceCollision) "0, 0, 0" true))

(event EventTick
  (params (DeltaSeconds :type Float%20%28single-precision%29))
  ;[1 1 1] Tick
  (Utilities|FlowControl|Gate true
    (:Exit
      (Utilities|FlowControl|Delay 0.01)
      (Transformation|SetActorLocation self (CallFunction|SetGridSnapVector) false false))))

(event EventConstructBuilding
  (params (MainBuilding :type Building%20Master%20BP%20Class%20Reference) (Builder :type Base%20Character%20Object%20Reference))
  ;[1 1 1] Construct Building
  (Variables|Default|SetBuilder Builder)
  (bind _returnvalue (Game|SpawnActorfromClass :Class MainBuilding :SpawnTransform (Math|Transform|MakeTransform "0, 0, 0") :CollisionHandlingOverride "Undefined" :Resource_BP 0 :Commander (.AsPawn%20Master%20Commander (Utilities|Casting|CastToPawn_MasterCommander (Game|Player|GetPlayerPawn 0))) :Instigator 0)) ; STORE building in GHOST BUILDING ref (each player has only 1) to spawn it later when clicked down - spawn building temp so we get mesh and proxy
  (Utilities|FlowControl|Sequence
    (:then_0
      (CallFunction|KillGhost)
      (CallFunction|OnSpawn (Variables|/Game/TD2020/Blueprints/Buildings/BuildingMaster_BP.BuildingMaster_BP_C|GetDisplayMesh _returnvalue) (.AsBuilding%20Master%20BP (Utilities|Casting|CastToBuildingMaster_BPClass MainBuilding)) (Variables|/Game/TD2020/Blueprints/Buildings/BuildingMaster_BP.BuildingMaster_BP_C|GetConstructionProxy _returnvalue) (Variables|/Game/TD2020/Blueprints/Buildings/BuildingMaster_BP.BuildingMaster_BP_C|GetProximityType_BP _returnvalue)))
    (:then_1
      (Actor|DestroyActor _returnvalue))))

(event EventBeginPlay
  ;[1 1 1] BeginPlay
  (Variables|References|SetGameStateRef (.AsGS%20My%20GS (Utilities|Casting|CastToGS_MyGS (Game|GetGameState)))))

(fn ConstructionScript)

(fn SetGridSnapVector
  (bind _cursorworldposition (Variables|Default|GetCursorWorldPosition))
  (bind _gridsize (Variables|Grid|GetGridSize))
  (return (Math|Vector|MakeVector (Class|FunctionLibrary|GridSnap (.x _cursorworldposition) _gridsize) (Class|FunctionLibrary|GridSnap (.y _cursorworldposition) _gridsize) (Class|FunctionLibrary|GridSnap (.z _cursorworldposition) _gridsize))))

(fn SetCursorPosition
  (params (CursorLocation :type Vector))
  (Variables|Default|SetCursorWorldPosition CursorLocation)
  (return))

(fn GetConstructionStruct
  (return (Utilities|Struct|MakeConstruction_Struct_02 (Variables|Default|GetBuildingClass) (Variables|Default|GetConstructionProxy) (Math|Transform|MakeTransform (Transformation|GetActorLocation) (Transformation|GetActorRotation) (Variables|/Game/TD2020/Blueprints/Pawns/Pawn_MasterCommander.Pawn_MasterCommander_C|GetActorScaleFactor (.AsPawn%20Master%20Commander (Utilities|Casting|CastToPawn_MasterCommander (Game|Player|GetPlayerPawn 0))))) (Variables|References|GetDisplayMesh) 5e+02 0.5 0 "/Game/TD2020/Textures/SkeletalMeshes/UE4_LOGO_CARD.UE4_LOGO_CARD" (Variables|Default|GetBuilder))))

(fn CheckOverlap
  (bind _overlappingactors (Collision|GetOverlappingActors "/Script/Engine.Actor" :!class /Script/Engine.Actor))
  (if (> (Utilities|Array|Length _overlappingactors) 0)
    (bind _array_element (Utilities|Array|ForEachLoopwithBreak _overlappingactors :!label _label)
      (:LoopBody
        (bind _asresource_resources_master (Utilities|Casting|CastToResource_ResourcesMaster _array_element)
          (:then
            (if (or (and (Utilities|Enum|Equal(Enum) (.ProximityType (Utilities|Struct|BreakResources_Struct (Variables|/Game/TD2020/Blueprints/Resources/Resource_ResourcesMaster.Resource_ResourcesMaster_C|GetResourceStruct _asresource_resources_master))) (Variables|Default|GetProximityType)) (not (Variables|Default|GetForceBadLocation))) (and (Utilities|Enum|Equal(Enum) (Variables|Default|GetProximityType) "None") (not (Variables|Default|GetForceBadLocation))))
              (LocalVariables|SetBadLocation_LOCAL false)
              (else
                (LocalVariables|SetBadLocation_LOCAL true) ; if get one bad overlapp - break
                (goto _label Break))))
          (:CastFailed
            (LocalVariables|SetBadLocation_LOCAL true)
            (goto _label Break))))
      (:Completed
        (return (LocalVariables|GetBadLocation_LOCAL))))
    (elif (Utilities|Enum|NotEqual(Enum) (Variables|Default|GetProximityType) "None")
      (return true)
      (else
        (return false) ; its equal to none - can be placed
      ))))

(fn GetIsOverlapping
  (return (Variables|Default|GetIsOverlapping)))

(fn SetInitialRotation
  (bind _returnvalue (Game|Player|GetPlayerPawn 0))
  (bind _aspawn_master_commander (Utilities|Casting|CastToPawn_MasterCommander _returnvalue))
  (bind _springarm (Variables|/Game/TD2020/Blueprints/Pawns/Pawn_MasterCommander.Pawn_MasterCommander_C|GetSpringArm _aspawn_master_commander))
  (bind _buildingrotationrate (Variables|/Game/TD2020/Blueprints/Pawns/Pawn_MasterCommander.Pawn_MasterCommander_C|GetBuildingRotationRate _aspawn_master_commander))
  (bind _returnvalue_2 (Class|SpringArmComponent|GetTargetRotation _springarm))
  (if (and (< (.yaw _returnvalue_2) _buildingrotationrate) (> (.yaw _returnvalue_2) (* -1 _buildingrotationrate))) ; if its not within parameters, we round
    (return 0.0)
    (else
      (return (* (.ReturnValue (Math|Float|Division(WholeandRemainder) (Math|Conversions|ToFloat(Integer) (Math|Float|Floor (.yaw _returnvalue_2))) _buildingrotationrate)) _buildingrotationrate)))))

(fn InitProximity
  (if (Utilities|Enum|NotEqual(Enum) (Variables|Default|GetProximityType) "None")
    (Default|ShowProximity (Variables|References|GetGameStateRef) (Variables|Default|GetProximityType))
    (return)
    (else
      (return))))

(fn DeinitializeProximity
  (if (Utilities|Enum|NotEqual(Enum) (Variables|Default|GetProximityType) "None")
    (Default|HideProximity (Variables|References|GetGameStateRef))
    (return)
    (else
      (return))))

(fn SetResource
  (params (Resource :type Resource%20Resources%20Master%20Object%20Reference))
  (Variables|Default|SetResourceSet Resource)
  (return))

(fn ClearResource
  (Variables|Default|SetResourceSet 0)
  (return))

(fn GetSurroundingGrid
  (bind _gridsize (Variables|Grid|GetGridSize))
  (bind _gridsize_2 (Variables|Grid|GetGridSize))
  (bind _gridsize_3 (Variables|Grid|GetGridSize))
  (bind _ghostbuilding_mesh (Variables|Components|GetGhostBuilding_Mesh))
  (bind _gridsize_4 (Variables|Grid|GetGridSize))
  (bind _gridsize_5 (Variables|Grid|GetGridSize))
  (bind _returnvalue (Math|Conversions|ToFloat(Integer) _gridsize_4))
  (bind (_min _max) (Components|StaticMesh|GetLocalBounds _ghostbuilding_mesh))
  (bind _returnvalue_2 (Math|Conversions|ToFloat(Integer) _gridsize_3))
  (bind _returnvalue_3 (Math|Conversions|ToFloat(Integer) _gridsize))
  (bind _returnvalue_4 (Math|Conversions|ToFloat(Integer) _gridsize_2))
  (bind (_x _y) (Math|Vector|BreakVector _min))
  (bind (_x_2 _y_2) (Math|Vector|BreakVector _max))
  (bind _returnvalue_5 (/ _y_2 _returnvalue))
  (bind _returnvalue_6 (/ _x _returnvalue_2))
  (bind _returnvalue_7 (/ _y _returnvalue_3))
  (bind _returnvalue_8 (/ _x_2 _returnvalue_4))
  (bind _returnvalue_9 (Math|Float|Ceil _returnvalue_5))
  (bind _returnvalue_10 (Math|Float|Ceil _returnvalue_6))
  (bind _returnvalue_11 (Math|Float|Ceil _returnvalue_7))
  (bind _returnvalue_12 (Math|Float|Ceil _returnvalue_8))
  (bind _returnvalue_13 (- _returnvalue_10 _returnvalue_12))
  (bind _returnvalue_14 (- _returnvalue_11 _returnvalue_9))
  (bind _returnvalue_15 (Math|Integer|Absolute(Integer) _returnvalue_13))
  (bind _returnvalue_16 (Math|Integer|Absolute(Integer) _returnvalue_14))
  (Utilities|Array|Clear (LocalVariables|GetPlacementTypes_LOCAL))
  (Utilities|Array|Clear (LocalVariables|GetGridLocations_LOCAL))
  (for _index (range 0 _returnvalue_16)
    (for _index_2 (range 0 _returnvalue_15)
      (Utilities|Array|Add (LocalVariables|GetGridLocations_LOCAL) (+ (Math|Vector|MakeVector (Math|Conversions|ToFloat(Integer) (- (* _index _gridsize_5) (/ (* _returnvalue_16 (Variables|Grid|GetGridSize)) 2))) (Math|Conversions|ToFloat(Integer) (- (* _index_2 _gridsize_5) (/ (* _returnvalue_15 (Variables|Grid|GetGridSize)) 2))) 0.0) (Transformation|GetActorLocation)))
      (if (CallFunction|CheckOverlap) ; if its overlapping
        (CallFunction|SetMaterial true) ; is overlapping -set error
        (Utilities|Array|Add (LocalVariables|GetPlacementTypes_LOCAL) "NewEnumerator2")
        (else
          (bind _badlocation (Class|FunctionLibrary|CalculateSlope self (.BoxExtent (Collision|GetComponentBounds (Variables|Components|GetGhostBuilding_Mesh)))))
          (if _badlocation
            (CallFunction|SetMaterial true) ; isnt overlapping - unset error if not on slope
            (Utilities|Array|Add (LocalVariables|GetPlacementTypes_LOCAL) "NewEnumerator0")
            (else
              (CallFunction|SetMaterial false) ; isnt overlapping - unset error if not on slope
              (Utilities|Array|Add (LocalVariables|GetPlacementTypes_LOCAL) "NewEnumerator1")))))))
  (Development|PrintString (Utilities|String|Append "Num grid tiles for ghost building->" (Utilities|String|ToString(Integer) (Utilities|Array|Length (LocalVariables|GetPlacementTypes_LOCAL)))))
  (return (LocalVariables|GetGridLocations_LOCAL) (LocalVariables|GetPlacementTypes_LOCAL)))

(fn SetCalendar
  (params (Date :type Array%20of%20Integers))
  (return false))

(fn SetClock
  (params (Time :type Array%20of%20Integers))
  (return false))