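; Per-commander construction manager that queues building proxies, assigns construction offices to them and spawns the commander's starting buildings.
; Each proxy goes to the nearest idle staffed office via an all-actors scan, or becomes a bid, with ProxyStart retrying every second.
; BidManager awards a contractor its closest open bid.
; On completion, the matching queued struct spawns the real building through the Commander and the proxy is destroyed.
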(event Custom|BindConstructionComplete
  (params (Proxy :type Construction%20Proxy%20BP%20Object%20Reference))
  (Utilities|IsValid Proxy ; check if on click not null clicked
    (:Is%20Valid
      (EventDispatchers|BindEventtoConstructionCompleted Proxy (EventDispatchers|CreateEvent :!event Custom|ConstructionCompleted)))))

(event Custom|CheckForContractor
  (params (Proxy :type Construction%20Proxy%20BP%20Object%20Reference))
  (Utilities|FlowControl|Delay 1.0)
  (bind _contractorfound (CallFunction|InitialContractorSearch Proxy))
  (bind _output_get (Variables|Default|SetContractorFound _contractorfound))
  (if (not _output_get)
    (CallFunction|CheckforContractor Proxy)))

(event Custom|ConstructionCompleted
  (params (Proxy :type Construction%20Proxy%20BP%20Object%20Reference))
  (CallFunction|FinishConstruction Proxy))

(event EventBeginPlay
  (Actor|SetOwner (Variables|/Game/TD2020/Blueprints/Pawns/Pawn_MasterCommander.Pawn_MasterCommander_C|GetPlayerController (Variables|Default|GetCommander))))

(fn ConstructionScript)

(fn QueueConstruction
  (params (ConstructionStruct :type Construction%20Struct%2002%20Structure))
  (bind (_buildingclass _proxyclass _transform _displaymesh _goldcost _workhoursrequired) (Utilities|Struct|BreakConstruction_Struct_02 ConstructionStruct))
  (bind _returnvalue (Game|SpawnActorfromClass :Class _proxyclass :SpawnTransform _transform :CollisionHandlingOverride "AlwaysSpawn" :DisplayMesh _displaymesh :GoldCost _goldcost :Commander 0 :Instigator 0)) ; PROXY BUILDING - GRAYED OUT - Gets spawned when placed on ground
  (CallFunction|BindConstructionComplete _returnvalue) ; Custom event - Binds event dispatcher and creates event finished construction
  (Utilities|Array|Add (Variables|Default|GetProxies) _returnvalue)
  (Utilities|Array|Add (Variables|Default|GetQueue) ConstructionStruct)
  (Utilities|IsValid _returnvalue ; check if clicked is not null
    (:Is%20Valid
      (Default|SetConstructionTime _returnvalue _workhoursrequired)
      (CallFunction|InitialContractorSearch _returnvalue))))

(fn FinishConstruction
  (params (Proxy :type Construction%20Proxy%20BP%20Object%20Reference))
  (bind _queue (Variables|Default|GetQueue))
  (bind _commander (Variables|Default|GetCommander))
  (bind _proxies (Variables|Default|GetProxies))
  (bind _output_get (LocalVariables|SetIndex (Utilities|Array|FindItem _proxies Proxy)))
  (LocalVariables|SetBuildingConfiguration (Utilities|Array|Get(acopy) _queue _output_get))
  (Utilities|Array|RemoveIndex _queue (LocalVariables|GetIndex))
  (Utilities|Array|RemoveIndex _proxies (LocalVariables|GetIndex))
  (Default|ROSSpawnActualBuilding _commander (LocalVariables|GetBuildingConfiguration) _commander)
  (Default|CallFinishedConstruction Proxy) ; calls construction office bp to clear job site
  (Actor|DestroyActor Proxy) ; remove proxy
)

(fn InitialContractorSearch
  (params (Proxy :type Construction%20Proxy%20BP%20Object%20Reference))
  (bind _distancetosite_local (LocalVariables|GetDistanceToSite_LOCAL))
  (bind _avaliablebuildings_local (LocalVariables|GetAvaliableBuildings_LOCAL))
  (bind _indexofminvalue (Math|Float|MinOfFloatArray _distancetosite_local))
  (bind _output (Utilities|Array|Get(acopy) _avaliablebuildings_local _indexofminvalue))
  (LocalVariables|SetProxy_LOCAL Proxy)
  (bind _outactors (Actor|GetAllActorsOfClass "/Game/TD2020/Blueprints/Buildings/BuildingMaster_BP.BuildingMaster_BP_C")) ; expensive!!!!!! - it gets all construction offices in level
  (bind _output_get (LocalVariables|SetAllBuildings_LOCAL _outactors)) ; sets them to local variable so we can use them later
  (if (> (Utilities|Array|Length _output_get) 0)
    (for _array_element (LocalVariables|GetAllBuildings_LOCAL)
      (bind _output_get_2 (LocalVariables|SetSelectedConstructor_LOCAL _array_element)) ; construction office
      (bind _td2020construction (Default|GetComponents _output_get_2))
      (Utilities|IsValid _td2020construction ; if has construction component
        (:Is%20Valid
          (if (and (.HasEmployees (Default|GetEmployees _td2020construction)) (not (Default|GetJobStatus _td2020construction))) ; has employees and doesnt have job
            (Utilities|Array|Add (LocalVariables|GetDistanceToSite_LOCAL) (Transformation|GetDistanceTo (LocalVariables|GetSelectedConstructor_LOCAL) (LocalVariables|GetProxy_LOCAL))) ; add distances to array
            (Utilities|Array|AddUnique (LocalVariables|GetAvaliableBuildings_LOCAL) (LocalVariables|GetSelectedConstructor_LOCAL)) ; added because it has same index as distance - can llok by index
          ))))
    (if (> (Utilities|Array|Length (LocalVariables|GetAvaliableBuildings_LOCAL)) 0) ; if no offices set it to construction bid
      (Utilities|IsValid (LocalVariables|GetProxy_LOCAL)
        (:Is%20Valid
          (Variables|/Game/TD2020/Blueprints/Buildings/ConstructionProxy_BP.ConstructionProxy_BP_C|SetContractor (LocalVariables|GetProxy_LOCAL) _output) ; set to nearest construction office
          (bind _td2020construction_2 (Default|GetComponents _output))
          (Default|SetCurrentJob _td2020construction_2 (LocalVariables|GetProxy_LOCAL))
          (return true)))
      (else
        _)))
  (Utilities|Array|AddUnique (Variables|Default|GetConstructionBids) (LocalVariables|GetProxy_LOCAL)) ; we dont have any construction offices
  (return false))

(fn BidManager
  (params (Contractor :type Building%20Master%20BP%20Object%20Reference))
  (LocalVariables|SetContractor_LOCAL Contractor)
  (if (> (Utilities|Array|Length (Variables|Default|GetConstructionBids)) 0)
    (for _array_element (Variables|Default|GetConstructionBids) ; creates array of distances
      (Utilities|Array|Add (LocalVariables|GetDistanceToSites_LOCAL) (Transformation|GetDistanceTo (LocalVariables|GetContractor_LOCAL) _array_element)) ; index of construction bid matches index of distances
    )
    (bind _output_get (LocalVariables|SetJobSites_LOCAL (Utilities|Array|Get(acopy) (Variables|Default|GetConstructionBids) (.IndexOfMinValue (Math|Float|MinOfFloatArray (LocalVariables|GetDistanceToSites_LOCAL))))))
    (bind _returnvalue (Utilities|Array|RemoveItem (Variables|Default|GetConstructionBids) _output_get)) ; remove item
    (if _returnvalue ; didnt remove because of used index
      (Variables|/Game/TD2020/Blueprints/Buildings/ConstructionProxy_BP.ConstructionProxy_BP_C|SetContractor (LocalVariables|GetJobSites_LOCAL) (LocalVariables|GetContractor_LOCAL))
      (return (LocalVariables|GetJobSites_LOCAL) true)
      (else
        _)))
  (return 0 false) ; empty job site if no bids and won bid false
)

(fn ProxyStart
  (params (Proxy :type Construction%20Proxy%20BP%20Object%20Reference) (ConstructionStruct :type Construction%20Struct%2002%20Structure%20%28by%20ref%29))
  (CallFunction|BindConstructionComplete Proxy) ; Custom event - Binds event dispatcher and creates event finished construction
  (Utilities|Array|Add (Variables|Default|GetProxies) Proxy)
  (Utilities|Array|Add (Variables|Default|GetQueue) ConstructionStruct)
  (Utilities|IsValid Proxy ; check if clicked is not null
    (:Is%20Valid
      (Default|SetConstructionTime Proxy (.WorkHoursRequired (Utilities|Struct|BreakConstruction_Struct_02 ConstructionStruct)))
      (bind _contractorfound (CallFunction|InitialContractorSearch Proxy))
      (bind _output_get (Variables|Default|SetContractorFound _contractorfound))
      (if (not _output_get) ; if no contractor has been found - restart search in 1 seconds
        (CallFunction|CheckforContractor Proxy)))))

(fn SpawnInitialBuildings
  (bind _commander (Variables|Default|GetCommander))
  (bind _commander_2 (Variables|Default|GetCommander))
  (bind _commander_3 (Variables|Default|GetCommander))
  (bind _commander_4 (Variables|Default|GetCommander))
  (bind _commander_5 (Variables|Default|GetCommander))
  (bind _commander_6 (Variables|Default|GetCommander))
  (bind _commander_7 (Variables|Default|GetCommander))
  (bind _commander_8 (Variables|Default|GetCommander))
  (bind _commander_9 (Variables|Default|GetCommander))
  (bind _commander_10 (Variables|Default|GetCommander))
  (bind _commander_11 (Variables|Default|GetCommander))
  (bind _commander_12 (Variables|Default|GetCommander))
  (bind _returnvalue (Transformation|GetActorTransform _commander_6))
  (bind _returnvalue_2 (Transformation|GetActorTransform _commander_4))
  (bind _returnvalue_3 (Transformation|GetActorTransform _commander_9))
  (bind _returnvalue_4 (Transformation|GetActorTransform _commander_12))
  (bind _returnvalue_5 (Transformation|GetActorTransform _commander_8))
  (bind _returnvalue_6 (Transformation|GetActorTransform _commander_3))
  (bind _location (Math|Transform|BreakTransform _returnvalue_3))
  (bind _location_2 (Math|Transform|BreakTransform _returnvalue_6))
  (if (Class|KismetSystemLibrary|IsStandalone)
    (Utilities|FlowControl|Sequence
      (:then_0
        ;[1 1 1] Construction office
        (Default|SpawnActualBuilding _commander_10 (Utilities|Struct|MakeConstruction_Struct_02 "/Game/TD2020/Blueprints/Buildings/AllBuildings/TownHall.TownHall_C" 0 (Math|Transform|MakeTransform (Math|Vector|MakeVector (.x _location) (.y _location) 0.0) "0,90.000000, 0") 0 0.0 0.0 0 "/Game/TD2020/Textures/Thumbnails/Buildings/Icon_Building_TownHall.Icon_Building_TownHall") _commander_10))
      (:then_1
        ;[1 1 1] Construction office
        (Default|SpawnActualBuilding _commander_2 (Utilities|Struct|MakeConstruction_Struct_02 "/Game/TD2020/Blueprints/Buildings/AllBuildings/ConstructionOffice_BP.ConstructionOffice_BP_C" 0 (Math|Transform|MakeTransform (Math|Vector|MakeVector (- (.x _location_2) 1e+03) (.y _location_2) 0.0) "0,90.000000, 0") 0 0.0 0.0 0 "/Game/TD2020/Textures/StaticMeshes/Items/AK_diffuse.AK_diffuse") _commander_2))
      (:then_2
        ;[1 1 1] Apartment
        (Default|SpawnActualBuilding _commander (Utilities|Struct|MakeConstruction_Struct_02 "/Game/TD2020/Blueprints/Buildings/AllBuildings/ApartmentSmall_BP.ApartmentSmall_BP_C" 0 (Math|Transform|MakeTransform (Math|Vector|MakeVector (+ (.x (.location _returnvalue_2)) 1e+03) (.y (.location _returnvalue_2)) 0.0) "0,90.000000, 0") 0 0.0 0.0 0 "/Game/TD2020/Textures/StaticMeshes/RTSBuildings/Apartments.Apartments") _commander))
      (:then_3
        ;[1 1 1] Barracks
        (Default|SpawnActualBuilding _commander_5 (Utilities|Struct|MakeConstruction_Struct_02 "/Game/TD2020/Blueprints/Buildings/AllBuildings/HumanBarracks.HumanBarracks_C" 0 (Math|Transform|MakeTransform (Math|Vector|MakeVector (.x (.location _returnvalue_5)) (+ (.y (.location _returnvalue_5)) 1e+03) 0.0) "0,90.000000, 0") 0 0.0 0.0 0 "/Game/TD2020/Meshes/InfinityBladeWeapons/Weapons/Blade/Axes/Blade_ExecutionerAxe/T_Blade_ExecutionerAxe1_N.T_Blade_ExecutionerAxe1_N") _commander_5))
      (:then_4
        ;[1 1 1] MiningShack
        (Default|SpawnActualBuilding _commander_7 (Utilities|Struct|MakeConstruction_Struct_02 "/Game/TD2020/Blueprints/Buildings/AllBuildings/MiningShack_BP.MiningShack_BP_C" 0 (Math|Transform|MakeTransform (Math|Vector|MakeVector (.x (.location _returnvalue)) (+ (.y (.location _returnvalue)) -1e+03) 0.0) "0,90.000000, 0") 0 0.0 0.0 0 "/Game/TD2020/Meshes/InfinityBladeWeapons/Weapons/Blade/Axes/Blade_ExecutionerAxe/T_Blade_ExecutionerAxe1_N.T_Blade_ExecutionerAxe1_N") _commander_7)))
    (else
      (Utilities|FlowControl|Sequence
        (:then_2
          ;[1 1 1] Barracks
          (Default|ROSSpawnActualBuilding _commander_11 (Utilities|Struct|MakeConstruction_Struct_02 "/Game/TD2020/Blueprints/Buildings/AllBuildings/HumanBarracks.HumanBarracks_C" 0 (Math|Transform|MakeTransform (Math|Vector|MakeVector (.x (.location _returnvalue_4)) (+ (.y (.location _returnvalue_4)) 1e+03) 0.0) "0,90.000000, 0") 0 0.0 0.0 0 "/Game/TD2020/Meshes/InfinityBladeWeapons/Weapons/Blade/Axes/Blade_ExecutionerAxe/T_Blade_ExecutionerAxe1_N.T_Blade_ExecutionerAxe1_N") _commander_11))))))