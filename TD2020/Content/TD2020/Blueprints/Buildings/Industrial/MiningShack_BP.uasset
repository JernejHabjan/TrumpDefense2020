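; Mining Shack is an industrial building Blueprint for the TD2020 RTS, built on a parent building class.
; Its construction script fills the building struct with its name, type, occupation, employee cap and avatar.
; GetOccupants reports the employee list and count as its occupants.
; GetComponents passes through the parent's RTS and TD2020 components and adds its resource drain component; the event graph holds no active logic.
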(event EventBeginPlay
  (|CallParentFunction))

(event Collision|EventActorBeginOverlap
  (params (OtherActor :type Actor%20Object%20Reference)))

(event EventTick
  (params (DeltaSeconds :type Float%20%28single-precision%29)))

(fn ConstructionScript
  (|CallParentFunction)
  (Variables|Default|SetBuildingStruct_BP (Utilities|Struct|MakeBuilding_STRUCT_02 self "NewEnumerator2" "Mining Shack" "NewEnumerator2" 3 0 "/Game/TD2020/Textures/StaticMeshes/vertical_planks_done.vertical_planks_done")))

(fn GetOccupants
  (bind _employees_bp (Variables|Default|GetEmployees_BP))
  (bind _returnvalue (Utilities|Array|Length _employees_bp))
  (return (> _returnvalue 0) _returnvalue _employees_bp))

(fn GetComponents
  (bind (_rtsselectable _rtsowner _rtsattackable _rtshealth _rtsproductioncost _rtsproduction _rtsconstructionsite _rtsportrait _td2020construction _td2020vacancy) (|CallParentFunction))
  (return _rtsselectable _rtsowner _rtsattackable _rtshealth _rtsproductioncost _rtsproduction _rtsconstructionsite _rtsportrait _td2020construction _td2020vacancy (Variables|Default|GetRTSResourceDrain)))