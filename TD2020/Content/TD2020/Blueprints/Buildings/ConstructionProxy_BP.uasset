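; Construction proxy that stands in for a building under construction, showing its mesh in a ghost material with fitted hitbox, entrance and rally point.
; Each tick, if the player commander's gold covers the cost, registered workers advance a game-speed-scaled clock, more workers building faster.
; Work progress drives RTSHealth toward the construction time.
; On completion, or immediately with InstaBuild, it fires ConstructionCompleted, frees and unhides workers, then destroys itself.
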(event Custom|AdjustTime
  (params (TimeUnit :type Float%20%28single-precision%29))
  ;[1 1 1] Adjust time
  (Variables|Time|SetTimeUnit TimeUnit))

(event EventBeginPlay
  (bind _gamestateref (Variables|Default|GetGameStateRef))
  ;[1 1 1] Begin Play
  (|CallParentFunction)
  (Utilities|IsValid _gamestateref
    (:Is%20Valid
      (EventDispatchers|BindEventtoUpdateGameSpeed _gamestateref (EventDispatchers|CreateEvent :!event Custom|AdjustTime)) ; bind proxy to dispatcher
      (Variables|Time|SetTimeUnit (Default|GetCurrentTimeUnit (Variables|Default|GetGameStateRef)))
      (Class|RTSConstructionSiteComponent|StartConstruction (Variables|Default|GetRTSConstructionSite)))
    (:Is%20Not%20Valid
      (Development|PrintString "Game state ref is invalid in construction proxy bp" true true "(R=1.000000,G=0.113484,B=0.000000,A=1.000000)" 3.0))))

(event EventTick
  (params (DeltaSeconds :type Float%20%28single-precision%29))
  ;[1 1 1] Event Tick
  (Variables|Time|SetDelta DeltaSeconds)
  (if (not (Variables|Default|GetIsConstructionCompleted))
    (if (Variables|Default|GetInstaBuild)
      (Default|CallConstructionCompleted self :!label _label) ; calls event that is bound to it (construction complete)...
      (CallFunction|ConstructionComplete)
      (Actor|DestroyActor)
      (else
        ;;[1 1 1] ToCheck
        (bind _newparam (CallFunction|CheckResourceAvaliablity))
        (if _newparam ; 3h 0min 0 sec in - DO ONCE CHECK?
          (CallFunction|DoWork)
          (if (>= (Variables|Default|GetWorkTimeSpent) (Variables|Default|GetConstructionTime))
            (Variables|Default|SetIsConstructionCompleted true) ; is completed
            (goto _label)))))))

(fn ConstructionScript
  (bind _hitbox (Variables|Default|GetHitBox))
  (bind _actorstaticmesh (Variables|Default|GetActorStaticMesh))
  (bind _actorstaticmesh_2 (Variables|Default|GetActorStaticMesh))
  (bind _returnvalue (Transformation|GetWorldLocation _hitbox))
  (bind _max (Components|StaticMesh|GetLocalBounds _actorstaticmesh))
  (bind _returnvalue_2 (/ (.z _max) 2.0))
  (Components|StaticMesh|SetStaticMesh _actorstaticmesh_2 (Variables|References|GetDisplayMesh))
  (Rendering|Material|SetMaterial _actorstaticmesh_2 0 "/Game/TD2020/Materials/Ghost_M_Inst.Ghost_M_Inst") ; ghost material instance
  (CallFunction|SetBuildingCollisionBox (Variables|Default|GetEntranceCollision) (Variables|Default|GetActorStaticMesh))
  (Transformation|SetWorldLocation (Variables|Components|GetEntrance) (Transformation|GetWorldLocation (Variables|Components|GetEntranceSphere)) false false)
  (Default|SetRally (Variables|Default|GetTD2020RallyComponent) (Transformation|GetWorldLocation (Variables|Components|GetEntrance)))
  (Components|Box|SetBoxExtent _hitbox (Math|Vector|MakeVector (.x _max) (.y _max) _returnvalue_2) true)
  (Transformation|SetWorldLocation _hitbox (Math|Vector|MakeVector (.x _returnvalue) (.y _returnvalue) (+ (.z _returnvalue) _returnvalue_2)) false false))

(fn SetConstructionTime
  (params (WorkHours :type Float%20%28single-precision%29))
  (bind _output_get (Variables|Default|SetConstructionTime (* WorkHours 6e+01)))
  (Variables|/Script/RTSPlugin.RTSHealthComponent|SetMaximumHealth (Variables|Default|GetRTSHealth) _output_get)
  (return))

(fn DoWork
  (bind _active_workers (CallFunction|GetWorkforce))
  (if (> _active_workers 0.0)
    (bind _output_get (Variables|Time|SetClockwork (.ClockworkOut (Class|FunctionLibrary|SetClockwork (Variables|Time|GetDelta) (/ (Variables|Time|GetTimeUnit) _active_workers) (Variables|Time|GetClockwork)))))
    (bind _output_get_2 (Variables|Default|SetWorkTimeSpent (* _output_get 6e+01)))
    (Variables|/Script/RTSPlugin.RTSHealthComponent|SetCurrentHealth (Variables|Default|GetRTSHealth) _output_get_2)
    (Variables|Default|SetGoldSpent (+ (Variables|Default|GetGoldSpent) 1e+01))
    (return)
    (else
      (return))))

(fn GetWorkforce
  (bind _activeworkers (Variables|References|GetActiveWorkers))
  (return (Math|Conversions|ToFloat(Integer) (Utilities|Array|Length _activeworkers)) _activeworkers))

(fn ReporttoShift
  (params (Worker :type NPC%20BP%20Object%20Reference))
  (Utilities|Array|Add (Variables|References|GetActiveWorkers) Worker)
  (return))

(fn ConstructionComplete
  (if (> (.Active%20Workers (CallFunction|GetWorkforce)) 0.0)
    (for _array_element (Variables|References|GetActiveWorkers)
      (Default|SetIsBusy _array_element false) ; when construction is completed, free all workers - is busy = false
      (Rendering|SetActorHiddenInGame _array_element false) ; set actors visible
    )
    (Variables|References|SetActiveWorkers (Utilities|Array|MakeArray 0)) ; clear array
    (return)
    (else
      (return))))

(fn LeaveShift
  (params (Employee :type NPC%20BP%20Object%20Reference))
  (if (> (Utilities|Array|FindItem (Variables|References|GetActiveWorkers) Employee) -1)
    (Rendering|SetActorHiddenInGame Employee false)
    (bind _returnvalue (Utilities|Array|RemoveItem (Variables|References|GetActiveWorkers) Employee)) ; if is in workers array  - remove it
    (return _returnvalue)
    (else
      (return false))))

(fn CheckResourceAvaliablity
  (bind _aspawn_master_commander (Utilities|Casting|CastToPawn_MasterCommander (Game|Player|GetPlayerPawn 0)))
  (Utilities|FlowControl|Sequence
    (:then_0
      (if (>= (- (Variables|/Game/TD2020/Blueprints/Pawns/Pawn_MasterCommander.Pawn_MasterCommander_C|GetGold _aspawn_master_commander) (Variables|Default|GetGoldCost)) 0.0) ; check gold
        (LocalVariables|SetHasGold true :!label _label)
        (if (LocalVariables|GetHasGold) ; check all resources
          (LocalVariables|SetCanBuild true)
          (else
            (LocalVariables|SetCanBuild false)))
        (elif (== (Variables|Default|GetGoldCost) 0.0) ; if first time building ok
          (goto _label)
          (else
            (LocalVariables|SetCanBuild false))))
      (return (LocalVariables|GetCanBuild)))))

(fn GetComponents
  (return (Variables|Default|GetRTSSelectable) (Variables|Default|GetRTSOwner) (Variables|Default|GetRTSAttackable) (Variables|Default|GetRTSHealth) 0 0 (Variables|Default|GetRTSConstructionSite) (Variables|Default|GetRTSName) (Variables|Default|GetRTSPortrait) 0 0 0))