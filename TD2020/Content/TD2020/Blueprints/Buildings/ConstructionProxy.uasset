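; Construction-site placeholder for a building, showing its mesh in a ghost material while workers build it.
; On BeginPlay it starts the RTS construction site and orders its builder to construct.
; Tick advances a game-speed-aware clock scaled by active workers; completion, or InstaBuild, fires the completion dispatcher, frees workers and destroys the proxy.
; Payment and attribute setup are disconnected, and the resource check always passes.
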(event Custom|AdjustTime
  (params (SpeedMultiplier :type Float%20%28single-precision%29) (Speed :type Integer) (TimeUnit :type Float%20%28single-precision%29))
  ;[1 1 1] Adjust time
  (Variables|Time|SetTimeUnit TimeUnit))

(event EventBeginPlay
  ;[1 1 1] Begin Play
  (|CallParentFunction)
  (EventDispatchers|BindEventtoUpdateGameSpeed (Variables|Default|GetGameStateRef) (EventDispatchers|CreateEvent :!event Custom|AdjustTime)) ; bind proxy to dispatcher
  (Variables|Time|SetTimeUnit (Variables|/Game/TD2020/Blueprints/Logics/GS_MyGS.GS_MyGS_C|GetTimeUnit (Variables|Default|GetGameStateRef)))
  (CallFunction|SetConstructionTime)
  (Class|RTSConstructionSiteComponent|StartConstruction (Variables|Default|GetRTSConstructionSite)) ; start only on server
  (CallFunction|SetAttributes)
  (Default|IssueConstructOrder (Variables|/Game/TD2020/Blueprints/AI/Characters/BaseCharacter.BaseCharacter_C|GetAIController (Variables|Default|GetBuilder)) self)
  ;[1 1 1] Pay all if insta pay is enabled
  (if (Variables|/Game/TD2020/Blueprints/Logics/GM_GameplayGM.GM_GameplayGM_C|GetInstaPay (.AsGM%20Gameplay%20GM (Utilities|Casting|CastToGM_GameplayGM (Game|GetGameMode))))
    (bind _canbuild_ (CallFunction|CheckResourceAvaliablity))
    (if _canbuild_
      (CallFunction|PayProxy (.ProductionCost (Utilities|Struct|BreakS_MyActor (CallFunction|RetrieveActorData (Variables|Default|GetBuiltClass)))))
      (else
        (Actor|DestroyActor)))))

(event EventTick
  (params (DeltaSeconds :type Float%20%28single-precision%29))
  ;[1 1 1] Event Tick
  (Variables|Time|SetDelta DeltaSeconds)
  (if (not (Variables|Default|GetIsConstructionCompleted))
    (if (Variables|/Game/TD2020/Blueprints/Logics/GM_GameplayGM.GM_GameplayGM_C|GetInstaBuild (.AsGM%20Gameplay%20GM (Utilities|Casting|CastToGM_GameplayGM (Game|GetGameMode))))
      (Default|CallConstructionCompleted self :!label _label) ; calls event that is bound to it (construction complete)...
      (CallFunction|ConstructionComplete)
      (Actor|DestroyActor)
      (else
        ;;[1 1 1] ToCheck
        (bind _canbuild_ (CallFunction|CheckResourceAvaliablity))
        (if _canbuild_ ; 3h 0min 0 sec in - DO ONCE CHECK?
          (CallFunction|DoWork)
          (if (>= (Variables|Default|GetWorkTimeSpent) (Variables|Default|GetConstructionTime))
            (Variables|Default|SetIsConstructionCompleted true) ; is completed
            (goto _label)))))))

(fn ConstructionScript
  (bind _hitbox (Variables|Default|GetHitBox))
  (bind _actorstaticmesh (Variables|Default|GetActorStaticMesh))
  (bind _actorstaticmesh_2 (Variables|Default|GetActorStaticMesh))
  (bind _returnvalue (Transformation|GetWorldLocation _hitbox))
  (bind _max (Components|StaticMesh|GetLocalBounds _actorstaticmesh))
  (bind _returnvalue_2 (/ (.z _max) 2.0))
  (|CallParentFunction)
  (Components|StaticMesh|SetStaticMesh _actorstaticmesh_2 (Variables|References|GetDisplayMesh))
  (Rendering|Material|SetMaterial _actorstaticmesh_2 0 "/Game/TD2020/Materials/Ghost_M_Inst.Ghost_M_Inst") ; ghost material instance
  (CallFunction|SetBuildingCollisionBox (Variables|Components|GetEntranceCollision) (Variables|Default|GetActorStaticMesh))
  (Transformation|SetWorldLocation (Variables|Components|GetEntrance) (Transformation|GetWorldLocation (Variables|Components|GetEntranceSphere)) false false)
  (Default|SetRally (Variables|Default|GetTD2020RallyComponent) (Transformation|GetWorldLocation (Variables|Components|GetEntrance)))
  (Components|Box|SetBoxExtent _hitbox (Math|Vector|MakeVector (.x _max) (.y _max) _returnvalue_2) true)
  (Transformation|SetWorldLocation _hitbox (Math|Vector|MakeVector (.x _returnvalue) (.y _returnvalue) (+ (.z _returnvalue) _returnvalue_2)) false false))

(fn SetConstructionTime
  (Variables|Default|SetConstructionTime (* (.ProductionTime (Utilities|Struct|BreakS_MyActor (CallFunction|RetrieveActorData (Variables|Default|GetBuiltClass)))) 6e+01))
  (return))

(fn DoWork
  (bind _active_workers (CallFunction|GetWorkforce))
  (if (> _active_workers 0.0)
    (bind _output_get (Variables|Time|SetClockwork (.ClockworkOut (Class|FunctionLibrary|SetClockwork (Variables|Time|GetDelta) (/ (Variables|Time|GetTimeUnit) _active_workers) (Variables|Time|GetClockwork)))))
    (bind _output_get_2 (Variables|Default|SetWorkTimeSpent (* _output_get 6e+01)))
    (if (Variables|/Game/TD2020/Blueprints/Logics/GM_GameplayGM.GM_GameplayGM_C|GetInstaPay (.AsGM%20Gameplay%20GM (Utilities|Casting|CastToGM_GameplayGM (Game|GetGameMode))))
      _
      (else
        _))
    (return)
    (else
      (return))))

(fn GetWorkforce
  (bind _activeworkers (Variables|References|GetActiveWorkers))
  (return (Math|Conversions|ToFloat(Integer) (Utilities|Array|Length _activeworkers)) _activeworkers))

(fn ReporttoShift
  (params (Worker :type NPC%20Object%20Reference))
  (Utilities|Array|Add (Variables|References|GetActiveWorkers) Worker)
  (return))

(fn ConstructionComplete
  (if (> (.Active%20Workers (CallFunction|GetWorkforce)) 0.0)
    (for _array_element (Variables|References|GetActiveWorkers)
      (Default|SetIsBusy _array_element false) ; when construction is completed, free all workers - is busy = false
      (Rendering|SetActorHiddenInGame _array_element false) ; set actors visible
    )
    (Variables|References|SetActiveWorkers (Utilities|Array|MakeArray 0)) ; clear array
    (return)
    (else
      (return))))

(fn LeaveShift
  (params (Employee :type NPC%20Object%20Reference))
  (if (> (Utilities|Array|FindItem (Variables|References|GetActiveWorkers) Employee) -1)
    (Rendering|SetActorHiddenInGame Employee false)
    (bind _returnvalue (Utilities|Array|RemoveItem (Variables|References|GetActiveWorkers) Employee)) ; if is in workers array  - remove it
    (return _returnvalue)
    (else
      (Rendering|SetActorHiddenInGame false)
      (return false))))

(fn CheckResourceAvaliablity
  (bind _aspc_gameplay_pc (Utilities|Casting|CastToPC_GameplayPC (Game|GetPlayerController 0)))
  (LocalVariables|SetHasResources true)
  (if (LocalVariables|GetHasResources) ; check all resources
    (LocalVariables|SetCanBuild true)
    (else
      (LocalVariables|SetCanBuild false)))
  (return (LocalVariables|GetCanBuild)))

(fn GetComponents
  (bind (_rtsselectable _rtsowner _td2020attackable _rtshealth _rtsproductioncost _rtsproduction _rtsconstructionsite _rtsname _rtsportrait _td2020construction _td2020vacancy _rtsresourcedrain) (|CallParentFunction))
  (return _rtsselectable _rtsowner _td2020attackable _rtshealth _rtsproductioncost _rtsproduction (Variables|Default|GetRTSConstructionSite) _rtsname _rtsportrait _td2020construction _td2020vacancy _rtsresourcedrain))

(fn IsFirstBuilding?
  (params (BuildingClass :type Building%20Master%20BP%20Class%20Reference))
  (LocalVariables|SetIsFirst true)
  (bind _outactors (Actor|GetAllActorsOfClass 0))
  (bind _array_element (Utilities|Array|ForEachLoopwithBreak _outactors :!label _label)
    (:LoopBody
      (if (and (== (Utilities|GetClass _array_element) BuildingClass) (CallFunction|CheckTeams _array_element self))
        (LocalVariables|SetIsFirst false)
        (goto _label Break)))
    (:Completed
      (return (LocalVariables|GetIsFirst)))))

(fn PayProxy
  (params (Resources :type Map%20of%20TD2020%20Resource%20Type%20Class%20References%20to%20Float%20%28single-precision%29s))
  ;[1 1 1] Todo reconnect later
)

(fn SetAttributes)