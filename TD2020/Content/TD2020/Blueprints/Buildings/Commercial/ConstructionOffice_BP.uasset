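; Construction Office commercial building that bids for construction jobs and assigns them to its employees.
; While it has occupants, a looping timer bids through the player commander's ConstructionManager, pausing once a job site is won.
; The manager's FinishedConstruction event clears the finished site and resumes bidding.
; AssignEmployeeJob hands registered employees the current site and its entrance location.
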(event Custom|FinishedConstruction
  (params (JobSiteProxy :type Construction%20Proxy%20BP%20Object%20Reference))
  ;[1 1 1] FinishedConstruction
  (if (== JobSiteProxy (Variables|Default|GetCurrentJobSite)) ; if jobsite is this one that this office has
    (Variables|Default|SetCurrentJobSite 0) ; clear variable
    (Utilities|Time|UnpauseTimerbyHandle (Variables|Default|GetBidTimerHandle))))

(event Custom|BidTimerEvent
  ;[1 1 1] BidTimerEvent
  (if (.HasOccupants (CallFunction|GetOccupants)) ; if we have employees - bid for job
    (bind _bidsuccessful (CallFunction|BidforJob))
    (if _bidsuccessful ; if we have bid
      (Utilities|Time|PauseTimerbyHandle (Variables|Default|GetBidTimerHandle)) ; not checking anymore untill finished construction
    )))

(event EventBeginPlay
  ;[1 1 1] BeginPlay
  (|CallParentFunction) ; initialize stuff in parent
  (bind _aspawn_master_commander (Utilities|Casting|CastToPawn_MasterCommander (Game|Player|GetPlayerPawn 0)))
  (Utilities|IsValid (Variables|/Game/TD2020/Blueprints/Units/Commanders/Pawn_MasterCommander.Pawn_MasterCommander_C|GetConstructionManagerRef _aspawn_master_commander)
    (:Is%20Valid
      (bind _output_get (Variables|References|SetConstructionManagerRef (Variables|/Game/TD2020/Blueprints/Units/Commanders/Pawn_MasterCommander.Pawn_MasterCommander_C|GetConstructionManagerRef _aspawn_master_commander)))
      (EventDispatchers|BindEventtoFinishedConstruction _output_get (EventDispatchers|CreateEvent :!event Custom|FinishedConstruction))
      (bind _returnvalue (Utilities|Time|SetTimerbyEvent (EventDispatchers|CreateEvent :!event Custom|BidTimerEvent) 1.0 true)) ; at begin play it starts this timer - checks for job every 1 second
      (Variables|Default|SetBidTimerHandle _returnvalue))))

(fn ConstructionScript
  (|CallParentFunction)
  (Variables|Default|SetBuildingStruct_BP (Utilities|Struct|MakeBuilding_STRUCT_02 self "NewEnumerator1" "Construction Office" "NewEnumerator1" 5 0 "/Game/TD2020/Textures/StaticMeshes/RTSBuildings/Workshed.Workshed")))

(fn GetJobStatus
  (return (Utilities|IsValid (Variables|Default|GetCurrentJobSite))))

(fn SetCurrentJob
  (params (JobSiteProxy :type Construction%20Proxy%20BP%20Object%20Reference))
  (Variables|Default|SetCurrentJobSite JobSiteProxy)
  (return))

(fn BidforJob
  (if (CallFunction|GetJobStatus) ; we wanna bid for job if were not working for a job
    (return false) ; if we have a job return false
    (else
      (bind (_jobsite _wonbid) (Default|BidManager (Variables|References|GetConstructionManagerRef) self))
      (LocalVariables|SetJobSite_LOCAL _jobsite) ; if we didnt get bid, job site is null
      (if _wonbid
        (Variables|Default|SetCurrentJobSite (LocalVariables|GetJobSite_LOCAL))
        (return true) ; successful
        (else
          (return false) ; we send back to person thats calling for bid for job that bid is not successful
        )))))

(fn AssignEmployeeJob
  (params (Employee :type NPC%20BP%20Object%20Reference))
  (bind _currentjobsite (Variables|Default|GetCurrentJobSite))
  (if (and (!= (Utilities|Array|FindItem (Variables|Default|GetEmployees_BP) Employee) -1) (!= (Variables|Default|GetCurrentJobSite) 0))
    (return true _currentjobsite (Transformation|GetWorldLocation (Variables|/Game/TD2020/Blueprints/Buildings/Construction/ConstructionProxy_BP.ConstructionProxy_BP_C|GetEntrance _currentjobsite)))
    (else
      (return false 0 "0, 0, 0"))))