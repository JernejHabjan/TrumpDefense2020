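; DefenseMaster is a base Blueprint for defensive tower buildings that detect and track enemies.
; SightRange overlaps maintain a Targets list of 0_Base-derived actors and a TargetLocked flag, cleared on any exit, while ShootRange overlaps toggle InFiringRange.
; OnDamaged calls the parent, then passes a valid damage causer to OnEnemySight if damage is positive and EnemyToFight is invalid.
; Fire and OnEnemySight are empty stubs here.
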(event OnComponentBeginOverlap(SightRange)
  (params (OverlappedComponent :type Primitive%20Component%20Object%20Reference) (OtherActor :type Actor%20Object%20Reference) (OtherComp :type Primitive%20Component%20Object%20Reference) (OtherBodyIndex :type Integer) (bFromSweep :type Boolean) (SweepResult :type Hit%20Result%20Structure%20%28by%20ref%29))
  ;[1 1 1] When entering the tower sight radius set the target to attack and set the targetLocaed value to true
  (if (Utilities|ClassIsChildOf (Utilities|GetClass OtherActor) "/Game/TD2020/Blueprints/AI/Characters/0_Base.0_Base_C")
    (Utilities|Array|AddUnique (Variables|Default|GetTargets) OtherActor)
    (Variables|Default|SetTargetLocked? true)))

(event OnComponentEndOverlap(SightRange)
  (params (OverlappedComponent :type Primitive%20Component%20Object%20Reference) (OtherActor :type Actor%20Object%20Reference) (OtherComp :type Primitive%20Component%20Object%20Reference) (OtherBodyIndex :type Integer))
  ;[1 1 1] When exiting the tower sight radius set targetLocked to false
  (Variables|Default|SetTargetLocked? false)
  (Utilities|Array|RemoveItem (Variables|Default|GetTargets) OtherActor))

(event OnComponentBeginOverlap(ShootRange)
  (params (OverlappedComponent :type Primitive%20Component%20Object%20Reference) (OtherActor :type Actor%20Object%20Reference) (OtherComp :type Primitive%20Component%20Object%20Reference) (OtherBodyIndex :type Integer) (bFromSweep :type Boolean) (SweepResult :type Hit%20Result%20Structure%20%28by%20ref%29))
  ;[1 1 1] Begin overlap
  (if (Utilities|ClassIsChildOf (Utilities|GetClass OtherActor) "/Game/TD2020/Blueprints/AI/Characters/0_Base.0_Base_C")
    (Variables|Default|SetInFiringRange? true)))

(event OnComponentEndOverlap(ShootRange)
  (params (OverlappedComponent :type Primitive%20Component%20Object%20Reference) (OtherActor :type Actor%20Object%20Reference) (OtherComp :type Primitive%20Component%20Object%20Reference) (OtherBodyIndex :type Integer))
  ;[1 1 1] End overlap
  (Variables|Default|SetInFiringRange? false))

(fn ConstructionScript
  (|CallParentFunction))

(fn Fire)

(fn OnDamaged
  (params (InDamage :type Float%20%28single-precision%29) (InDamageCauser :type Actor%20Object%20Reference))
  (bind _currenthealth (|CallParentFunction InDamage InDamageCauser))
  (if (> _currenthealth 0)
    (Utilities|IsValid (Variables|Default|GetEnemyToFight)
      (:Is%20Valid
        _)
      (:Is%20Not%20Valid
        (Utilities|IsValid InDamageCauser
          (:Is%20Valid
            (CallFunction|OnEnemySight InDamageCauser))
          (:Is%20Not%20Valid
            _)))))
  (return _currenthealth))

(fn OnEnemySight
  (params (InEnemy :type Actor%20Object%20Reference))
  (return 0))