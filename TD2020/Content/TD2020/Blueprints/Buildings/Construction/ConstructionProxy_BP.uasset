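; Construction proxy that stands in for a building under construction, showing a ghost-material mesh with selection visuals, a camera-facing health bar and a WB_Proxy HUD.
; Tick currently completes construction immediately: it calls the completion dispatcher, frees assigned workers, then removes the HUD and destroys the actor.
; Worker-scaled timing following game speed and gold checks exist, but that branch is disconnected.
; A gate and timeline can move the commander pawn to the site.
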(event Custom|AdjustTime
  (params (TimeUnit :type Float%20%28single-precision%29))
  ;[1 1 1] Adjust time
  (Variables|Time|SetTimeUnit TimeUnit))

(event Custom|OpenFollowGate
  (bind _returnvalue (Transformation|GetActorLocation))
  ;[1 1 1] Event Tick
  (Development|PrintString "OPENED GATE")
  (Utilities|FlowControl|Gate true) ; enters at Open
)

(event Custom|CloseFollowGate
  (bind _returnvalue (Transformation|GetActorLocation))
  ;[1 1 1] Event Tick
  (Utilities|FlowControl|Gate true) ; enters at Close
)

(event Custom|LerpToConstruction
  ;[1 1 1] LerpToConstruction
  (bind _speed (Timeline|Timeline_0 PlayFromStart) ; update is kinda like tick - lerps between old and new location
    (:Update
      (Transformation|SetActorLocation (Variables|Default|GetCommander) (Class|FunctionLibrary|HUDLerpLocation (Transformation|GetActorLocation (Variables|Default|GetCommander)) (Transformation|GetActorLocation) _speed) false false))
    (:Finished)))

(event EventBeginPlay
  ;[1 1 1] Begin Play
  (bind _aspawn_master_commander (Utilities|Casting|CastToPawn_MasterCommander (Game|Player|GetPlayerPawn 0)))
  (Variables|Default|SetCommander _aspawn_master_commander)
  (bind _output_get (Variables|References|SetGameStateRef (.AsGS%20My%20GS (Utilities|Casting|CastToGS_MyGS (Game|GetGameState)))))
  (EventDispatchers|BindEventtoUpdateGameSpeed _output_get (EventDispatchers|CreateEvent :!event Custom|AdjustTime)) ; bind proxy to dispatcher
  (Variables|Time|SetTimeUnit (Default|GetCurrentTimeUnit (Variables|References|GetGameStateRef)))
  (Variables|References|SetControllerRef (.AsPC%20Gameplay%20PC (Utilities|Casting|CastToPC_GameplayPC (Game|GetPlayerController 0))))
  (bind _returnvalue (UserInterface|CreateWidget "/Game/TD2020/Widgets/HUDs/WB_Proxy.WB_Proxy_C" (Game|GetPlayerController 0) self (Variables|References|GetControllerRef)))
  (Variables|References|SetProxyHUD _returnvalue)
  (Utilities|Array|SetArrayElem (Variables|Default|GetTags) 0 (Utilities|String|StringToName (.TeamName (Utilities|Struct|BreakEntity_Struct (Variables|Default|GetEntityStruct))))) ; set team
)

(event EventTick
  (params (DeltaSeconds :type Float%20%28single-precision%29))
  (bind _returnvalue (Transformation|GetActorLocation))
  (bind _proxyhud (Variables|References|GetProxyHUD))
  ;[1 1 1] Event Tick
  (Variables|Time|SetDelta DeltaSeconds)
  (Utilities|FlowControl|Sequence
    (:then_0
      (Utilities|FlowControl|Gate true
        (:Exit
          (Transformation|SetActorLocation (Variables|Default|GetCommander) (Math|Vector|MakeVector (.x _returnvalue) (.y _returnvalue) (.z (Transformation|GetActorLocation))) false false))))
    (:then_1
      (CallFunction|RotateHealthBartoPlayer)
      (if (not (Variables|Default|GetIsConstructionCompleted))
        (Default|CallConstructionCompleted self) ; calls event that is bound to it (construction complete)...
        (CallFunction|ConstructionComplete)
        (Utilities|IsValid _proxyhud
          (:Is%20Valid
            (if (UserInterface|Viewport|IsinViewport _proxyhud)
              (Default|RemoveHUD (Variables|References|GetProxyHUD)))
            (Utilities|FlowControl|Delay 0.2)
            (Actor|DestroyActor)))))))

(fn ConstructionScript
  (bind _staticmesh (Variables|Components|GetStaticMesh))
  (Components|StaticMesh|SetStaticMesh _staticmesh (Variables|References|GetDisplayMesh))
  (Rendering|Material|SetMaterial _staticmesh 0 "/Game/TD2020/Materials/Ghost_M_Inst.Ghost_M_Inst") ; ghost material instance
  (Class|FunctionLibrary|SetBuildingEntrance (Variables|Components|GetEntrance) (Variables|Components|GetStaticMesh))
  (Class|FunctionLibrary|SetBuildingCollisionBox (Variables|Components|GetCollision) (Variables|Components|GetStaticMesh)))

(fn SetConstructionTime
  (params (WorkHours :type Float%20%28single-precision%29))
  (Variables|Default|SetConstructionTime (* WorkHours 1.0))
  (return))

(fn DoWork
  (bind _active_workers (CallFunction|GetWorkforce))
  (if (> _active_workers 0.0)
    (bind _output_get (Variables|Time|SetClockwork (.ClockworkOut (Class|FunctionLibrary|SetClockwork (Variables|Time|GetDelta) (/ (Variables|Time|GetTimeUnit) _active_workers) (Variables|Time|GetClockwork)))))
    (Variables|Default|SetWorkTimeSpent (* _output_get 6e+01))
    (Variables|Default|SetGoldSpent (+ (Variables|Default|GetGoldSpent) 1e+01))
    (return)
    (else
      (return))))

(fn GetWorkforce
  (bind _activeworkers (Variables|References|GetActiveWorkers))
  (return (Math|Conversions|ToFloat(Integer) (Utilities|Array|Length _activeworkers)) _activeworkers))

(fn ReporttoShift
  (params (Worker :type NPC%20BP%20Object%20Reference))
  (Utilities|Array|Add (Variables|References|GetActiveWorkers) Worker)
  (return))

(fn ConstructionComplete
  (if (> (.Active%20Workers (CallFunction|GetWorkforce)) 0.0)
    (for _array_element (Variables|References|GetActiveWorkers)
      (Default|SetIsBusy _array_element false) ; when construction is completed, free all workers - is busy = false
      (Rendering|SetActorHiddenInGame _array_element false) ; set actors visible
    )
    (Variables|References|SetActiveWorkers (Utilities|Array|MakeArray 0)) ; clear array
    (return)
    (else
      (return))))

(fn LeaveShift
  (params (Employee :type NPC%20BP%20Object%20Reference))
  (if (> (Utilities|Array|FindItem (Variables|References|GetActiveWorkers) Employee) -1)
    (bind _returnvalue (Utilities|Array|RemoveItem (Variables|References|GetActiveWorkers) Employee)) ; if is in workers array  - remove it
    (return _returnvalue)
    (else
      (return false))))

(fn CheckResourceAvaliablity
  (bind _aspawn_master_commander (Utilities|Casting|CastToPawn_MasterCommander (Game|Player|GetPlayerPawn 0)))
  (Utilities|FlowControl|Sequence
    (:then_0
      (if (>= (- (Variables|/Game/TD2020/Blueprints/Units/Commanders/Pawn_MasterCommander.Pawn_MasterCommander_C|GetGold _aspawn_master_commander) (Variables|Default|GetGoldCost)) 0.0) ; check gold
        (LocalVariables|SetHasGold true :!label _label)
        (if (LocalVariables|GetHasGold) ; check all resources
          (LocalVariables|SetCanBuild true)
          (else
            (LocalVariables|SetCanBuild false)))
        (elif (== (Variables|Default|GetGoldCost) 0.0) ; if first time building ok
          (goto _label)
          (else
            (LocalVariables|SetCanBuild false))))
      (return (LocalVariables|GetCanBuild)))))

(fn RotateHealthBartoPlayer
  (Transformation|SetWorldRotation (Variables|Default|GetHealthBar) (Math|Rotator|FindLookatRotation (Transformation|GetWorldLocation (Variables|Default|GetHealthBar)) (Camera|GetCameraLocation (Game|GetPlayerCameraManager 0))) false false))

(fn SetSelected
  (params (Selected? :type Boolean) (InPawn :type Pawn%20Master%20Commander%20Object%20Reference))
  (bind _returnvalue (Pawn|IsLocallyControlled InPawn))
  (Utilities|IsValid InPawn
    (:Is%20Valid
      (if _returnvalue
        (Rendering|SetVisibility (Variables|Default|GetSelected) Selected? false)
        (Rendering|SetVisibility (Variables|Default|GetCursorToWorld) Selected? false))
      (return _returnvalue))))

(fn AddRally
  (params (Location :type Vector :default "0, 0, 0") (Action :type String) (Actor :type Actor%20Object%20Reference))
  (return 0))

(fn GetRallies
  (return "0, 0, 0" 0 0))

(fn ImNotSelected
  (params (InPawn :type Pawn%20Master%20Commander%20Object%20Reference))
  (CallFunction|SetSelected false InPawn)
  (return 0))

(fn ImSelected
  (params (InPawn :type Pawn%20Master%20Commander%20Object%20Reference))
  (CallFunction|SetSelected true InPawn)
  (return 0))

(fn RemoveRallies
  (return 0))

(fn RMBHit
  (params (InCommander :type Actor%20Object%20Reference))
  (return 0))