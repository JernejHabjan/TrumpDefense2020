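; Manager that runs building construction for a commander, from grayed-out proxy to finished building, and spawns the starting office, apartment and barracks.
; Queued proxies get the nearest staffed, idle construction office by straight-line distance, or wait as bids.
; BidManager gives a requesting contractor its nearest waiting bid.
; On completion, parallel Proxies and Queue arrays supply the config for spawning the real building through the commander, then the proxy is destroyed.
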(event Custom|BindConstructionComplete
  (params (Proxy :type Construction%20Proxy%20BP%20Object%20Reference))
  (Utilities|IsValid Proxy ; check if on click not null clicked
    (:Is%20Valid
      (EventDispatchers|BindEventtoConstructionCompleted Proxy (EventDispatchers|CreateEvent :!event Custom|ConstructionCompleted)))))

(event Custom|ConstructionCompleted
  (params (Proxy :type Construction%20Proxy%20BP%20Object%20Reference))
  (CallFunction|FinishConstruction Proxy))

(event EventBeginPlay
  (bind _commanderspawn (Variables|Default|GetCommanderSpawn))
  (Variables|Default|SetPlayerController (.AsPC%20Gameplay%20PC (Utilities|Casting|CastToPC_GameplayPC (Game|GetPlayerController 0))))
  (Utilities|IsValid _commanderspawn
    (:Is%20Valid
      (Variables|Default|SetCommander _commanderspawn))
    (:Is%20Not%20Valid
      (Variables|Default|SetCommander (.AsPawn%20Master%20Commander (Utilities|Casting|CastToPawn_MasterCommander (Game|Player|GetPlayerPawn 0)))))))

(fn ConstructionScript)

(fn QueueConstruction
  (params (ConstructionStruct :type Construction%20Struct%2002%20Structure))
  (bind (_buildingclass _proxyclass _transform _displaymesh _goldcost _workhoursrequired) (Utilities|Struct|BreakConstruction_Struct_02 ConstructionStruct))
  (bind _returnvalue (Game|SpawnActorfromClass :Class _proxyclass :SpawnTransform _transform :CollisionHandlingOverride "AlwaysSpawn" :DisplayMesh _displaymesh :GoldCost _goldcost :Instigator 0)) ; PROXY BUILDING - GRAYED OUT - Gets spawned when placed on ground
  (CallFunction|BindConstructionComplete _returnvalue) ; Custom event - Binds event dispatcher and creates event finished construction
  (Utilities|Array|Add (Variables|Default|GetProxies) _returnvalue)
  (Utilities|Array|Add (Variables|Default|GetQueue) ConstructionStruct)
  (Utilities|IsValid _returnvalue ; check if clicked is not null
    (:Is%20Valid
      (Default|SetConstructionTime _returnvalue _workhoursrequired)
      (CallFunction|InitialContractorSearch _returnvalue))))

(fn FinishConstruction
  (params (Proxy :type Construction%20Proxy%20BP%20Object%20Reference))
  (bind _returnvalue (Game|Player|GetPlayerPawn 0))
  (bind _queue (Variables|Default|GetQueue))
  (bind _proxies (Variables|Default|GetProxies))
  (bind _aspawn_master_commander (Utilities|Casting|CastToPawn_MasterCommander _returnvalue))
  (bind _output_get (LocalVariables|SetIndex (Utilities|Array|FindItem _proxies Proxy)))
  (LocalVariables|SetBuildingConfiguration (Utilities|Array|Get(acopy) _queue _output_get))
  (Utilities|Array|RemoveIndex _queue (LocalVariables|GetIndex))
  (Utilities|Array|RemoveIndex _proxies (LocalVariables|GetIndex))
  ;[1 0.06933 0] TODO ENTITY STRUCT
  (Default|ROSSpawnActualBuilding _aspawn_master_commander (LocalVariables|GetBuildingConfiguration) (.AsPC%20Gameplay%20PC (Utilities|Casting|CastToPC_GameplayPC (Game|GetPlayerController 0))) _aspawn_master_commander)
  (Default|CallFinishedConstruction Proxy) ; calls construction office bp to clear job site
  (Actor|DestroyActor Proxy) ; remove proxy
)

(fn InitialContractorSearch
  (params (Proxy :type Construction%20Proxy%20BP%20Object%20Reference))
  (LocalVariables|SetProxy_LOCAL Proxy)
  (bind _outactors (Actor|GetAllActorsOfClass "/Game/TD2020/Blueprints/Buildings/Commercial/ConstructionOffice_BP.ConstructionOffice_BP_C")) ; expensive!!!!!! - it gets all construction offices in level
  (bind _output_get (LocalVariables|SetAllConstructionOffices_LOCAL _outactors)) ; sets them to local variable so we can use them later
  (if (> (Utilities|Array|Length _output_get) 0)
    (for _array_element (LocalVariables|GetAllConstructionOffices_LOCAL) ; fills arrays with length and offices
      (bind _output_get_2 (LocalVariables|SetSelectedOffice_LOCAL _array_element)) ; construction office
      (if (and (.HasOccupants (Default|GetOccupants _output_get_2)) (not (Default|GetJobStatus _output_get_2))) ; has employees and doesnt have job
        (Utilities|Array|Add (LocalVariables|GetDistanceToSite_LOCAL) (Transformation|GetDistanceTo (LocalVariables|GetSelectedOffice_LOCAL) (LocalVariables|GetProxy_LOCAL))) ; add distances to array
        (Utilities|Array|AddUnique (LocalVariables|GetAvaliableConstructionOffices_LOCAL) (LocalVariables|GetSelectedOffice_LOCAL)) ; added because it has same index as distance - can llok by index
      ))
    (if (> (Utilities|Array|Length (LocalVariables|GetAvaliableConstructionOffices_LOCAL)) 0) ; if no offices set it to construction bid
      (bind _output_get_3 (Variables|/Game/TD2020/Blueprints/Buildings/Construction/ConstructionProxy_BP.ConstructionProxy_BP_C|SetContractor (LocalVariables|GetProxy_LOCAL) (Utilities|Array|Get(acopy) (LocalVariables|GetAvaliableConstructionOffices_LOCAL) (.IndexOfMinValue (Math|Float|MinOfFloatArray (LocalVariables|GetDistanceToSite_LOCAL)))))) ; set to nearest construction office
      (Default|SetCurrentJob _output_get_3 (LocalVariables|GetProxy_LOCAL))
      (return)
      (else
        _)))
  (Utilities|Array|AddUnique (Variables|Default|GetConstructionBids) (LocalVariables|GetProxy_LOCAL)) ; we dont have any construction offices
  (return))

(fn BidManager
  (params (Contractor :type Construction%20Office%20BP%20Object%20Reference))
  (LocalVariables|SetContractor_LOCAL Contractor)
  (if (> (Utilities|Array|Length (Variables|Default|GetConstructionBids)) 0)
    (for _array_element (Variables|Default|GetConstructionBids) ; creates array of distances
      (Utilities|Array|Add (LocalVariables|GetDistanceToSites_LOCAL) (Transformation|GetDistanceTo (LocalVariables|GetContractor_LOCAL) _array_element)) ; index of construction bid matches index of distances
    )
    (bind _output_get (LocalVariables|SetJobSites_LOCAL (Utilities|Array|Get(acopy) (Variables|Default|GetConstructionBids) (.IndexOfMinValue (Math|Float|MinOfFloatArray (LocalVariables|GetDistanceToSites_LOCAL))))))
    (bind _returnvalue (Utilities|Array|RemoveItem (Variables|Default|GetConstructionBids) _output_get)) ; remove item
    (if _returnvalue ; didnt remove because of used index
      (Variables|/Game/TD2020/Blueprints/Buildings/Construction/ConstructionProxy_BP.ConstructionProxy_BP_C|SetContractor (LocalVariables|GetJobSites_LOCAL) (LocalVariables|GetContractor_LOCAL))
      (return (LocalVariables|GetJobSites_LOCAL) true)
      (else
        _)))
  (return 0 false) ; empty job site if no bids and won bid false
)

(fn ProxyStart
  (params (Proxy :type Construction%20Proxy%20BP%20Object%20Reference) (ConstructionStruct :type Construction%20Struct%2002%20Structure%20%28by%20ref%29))
  (CallFunction|BindConstructionComplete Proxy) ; Custom event - Binds event dispatcher and creates event finished construction
  (Utilities|Array|Add (Variables|Default|GetProxies) Proxy)
  (Utilities|Array|Add (Variables|Default|GetQueue) ConstructionStruct)
  (Utilities|IsValid Proxy ; check if clicked is not null
    (:Is%20Valid
      (Default|SetConstructionTime Proxy (.GoldCost (Utilities|Struct|BreakConstruction_Struct_02 ConstructionStruct)))
      (CallFunction|InitialContractorSearch Proxy))))

(fn SpawnInitialBuildings
  (bind _commander (Variables|Default|GetCommander))
  (bind _commander_2 (Variables|Default|GetCommander))
  (bind _commander_3 (Variables|Default|GetCommander))
  (bind _commander_4 (Variables|Default|GetCommander))
  (bind _commander_5 (Variables|Default|GetCommander))
  (bind _commander_6 (Variables|Default|GetCommander))
  (bind _commander_7 (Variables|Default|GetCommander))
  (bind _commander_8 (Variables|Default|GetCommander))
  (bind _commander_9 (Variables|Default|GetCommander))
  (bind _commander_10 (Variables|Default|GetCommander))
  (bind _returnvalue (Transformation|GetActorTransform _commander_3))
  (bind _returnvalue_2 (Transformation|GetActorTransform _commander_2))
  (bind _returnvalue_3 (Transformation|GetActorTransform _commander_7))
  (bind _returnvalue_4 (Transformation|GetActorTransform _commander_9))
  (if (Class|KismetSystemLibrary|IsStandalone)
    (Utilities|FlowControl|Sequence
      (:then_0
        ;[1 1 1] Construction office
        (Default|SpawnActualBuilding _commander_10 (Utilities|Struct|MakeConstruction_Struct_02 "/Game/TD2020/Blueprints/Buildings/Commercial/ConstructionOffice_BP.ConstructionOffice_BP_C" 0 (Transformation|GetActorTransform (Variables|Default|GetCommander)) 0 0.0 0.0 0 "/Game/TD2020/Textures/StaticMeshes/Items/AK_diffuse.AK_diffuse") (Variables|Default|GetPlayerController) _commander_10 (Utilities|Struct|MakeEntity_Struct (Utilities|String|ToString(Name) (Utilities|Array|Get(acopy) (Variables|/Script/Engine.Actor|GetTags (Variables|Default|GetCommander)))) "EntityName" 50 50 "/Game/TD2020/Textures/StaticMeshes/Items/AK_diffuse.AK_diffuse" 0 0.0 0.0)))
      (:then_1
        ;[1 1 1] Apartment
        (Default|SpawnActualBuilding _commander (Utilities|Struct|MakeConstruction_Struct_02 "/Game/TD2020/Blueprints/Buildings/Residential/ApartmentSmall_BP.ApartmentSmall_BP_C" 0 (Math|Transform|MakeTransform (Math|Vector|MakeVector (+ (.x (.location _returnvalue_2)) 1e+03) (.y (.location _returnvalue_2)) (.z (.location _returnvalue_2))) "0, 0, 0" "0.500000,0.500000,0.500000") 0 0.0 0.0 0 "/Game/TD2020/Textures/StaticMeshes/RTSBuildings/Apartments.Apartments") (Variables|Default|GetPlayerController) _commander (Utilities|Struct|MakeEntity_Struct (Utilities|String|ToString(Name) (Utilities|Array|Get(acopy) (Variables|/Script/Engine.Actor|GetTags (Variables|Default|GetCommander)))) "ApartmentSmall" 50 50 "/Game/TD2020/Textures/StaticMeshes/RTSBuildings/Apartments.Apartments" 0 0.0 0.0)))
      (:then_2
        ;[1 1 1] Barracks
        (Default|SpawnActualBuilding _commander_4 (Utilities|Struct|MakeConstruction_Struct_02 "/Game/TD2020/Blueprints/Buildings/Army/HumanBarracks.HumanBarracks_C" 0 (Math|Transform|MakeTransform (Math|Vector|MakeVector (.x (.location _returnvalue)) (+ (.y (.location _returnvalue)) 1e+03) (.z (.location _returnvalue)))) 0 0.0 0.0 0 "/Game/TD2020/Meshes/InfinityBladeWeapons/Weapons/Blade/Axes/Blade_ExecutionerAxe/T_Blade_ExecutionerAxe1_N.T_Blade_ExecutionerAxe1_N") (Variables|Default|GetPlayerController) _commander_4 (Utilities|Struct|MakeEntity_Struct (Utilities|String|ToString(Name) (Utilities|Array|Get(acopy) (Variables|/Script/Engine.Actor|GetTags (Variables|Default|GetCommander)))) "Barracks" 50 50 "/Game/TD2020/Meshes/InfinityBladeWeapons/Weapons/Blade/Axes/Blade_ExecutionerAxe/T_Blade_ExecutionerAxe1_N.T_Blade_ExecutionerAxe1_N"))))
    (else
      (Utilities|FlowControl|Sequence
        (:then_0
          ;[1 1 1] Construction office
          (Default|ROSSpawnActualBuilding _commander_5 (Utilities|Struct|MakeConstruction_Struct_02 "/Game/TD2020/Blueprints/Buildings/Commercial/ConstructionOffice_BP.ConstructionOffice_BP_C" 0 (Transformation|GetActorTransform (Variables|Default|GetCommander)) 0 0.0 0.0 0 "/Game/TD2020/Textures/StaticMeshes/Items/AK_diffuse.AK_diffuse") (Variables|Default|GetPlayerController) _commander_5 (Utilities|Struct|MakeEntity_Struct (Utilities|String|ToString(Name) (Utilities|Array|Get(acopy) (Variables|/Script/Engine.Actor|GetTags (Variables|Default|GetCommander)))) "EntityName" 50 50 "/Game/TD2020/Textures/StaticMeshes/Items/AK_diffuse.AK_diffuse" 0 0.0 0.0)))
        (:then_1
          ;[1 1 1] Apartment
          (Default|ROSSpawnActualBuilding _commander_6 (Utilities|Struct|MakeConstruction_Struct_02 "/Game/TD2020/Blueprints/Buildings/Residential/ApartmentSmall_BP.ApartmentSmall_BP_C" 0 (Math|Transform|MakeTransform (Math|Vector|MakeVector (+ (.x (.location _returnvalue_3)) 1e+03) (.y (.location _returnvalue_3)) (.z (.location _returnvalue_3))) "0, 0, 0" "0.500000,0.500000,0.500000") 0 0.0 0.0 0 "/Game/TD2020/Textures/StaticMeshes/RTSBuildings/Apartments.Apartments") (Variables|Default|GetPlayerController) _commander_6 (Utilities|Struct|MakeEntity_Struct (Utilities|String|ToString(Name) (Utilities|Array|Get(acopy) (Variables|/Script/Engine.Actor|GetTags (Variables|Default|GetCommander)))) "ApartmentSmall" 50 50 "/Game/TD2020/Textures/StaticMeshes/RTSBuildings/Apartments.Apartments" 0 0.0 0.0)))
        (:then_2
          ;[1 1 1] Barracks
          (Default|ROSSpawnActualBuilding _commander_8 (Utilities|Struct|MakeConstruction_Struct_02 "/Game/TD2020/Blueprints/Buildings/Army/HumanBarracks.HumanBarracks_C" 0 (Math|Transform|MakeTransform (Math|Vector|MakeVector (.x (.location _returnvalue_4)) (+ (.y (.location _returnvalue_4)) 1e+03) (.z (.location _returnvalue_4)))) 0 0.0 0.0 0 "/Game/TD2020/Meshes/InfinityBladeWeapons/Weapons/Blade/Axes/Blade_ExecutionerAxe/T_Blade_ExecutionerAxe1_N.T_Blade_ExecutionerAxe1_N") (Variables|Default|GetPlayerController) _commander_8 (Utilities|Struct|MakeEntity_Struct (Utilities|String|ToString(Name) (Utilities|Array|Get(acopy) (Variables|/Script/Engine.Actor|GetTags (Variables|Default|GetCommander)))) "Barracks" 50 50 "/Game/TD2020/Meshes/InfinityBladeWeapons/Weapons/Blade/Axes/Blade_ExecutionerAxe/T_Blade_ExecutionerAxe1_N.T_Blade_ExecutionerAxe1_N")))))))