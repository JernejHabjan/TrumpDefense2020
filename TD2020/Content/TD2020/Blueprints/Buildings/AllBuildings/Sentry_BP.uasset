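; Sentry_BP is a defensive tower building for the TD2020 RTS game, built on a parent building Blueprint.
; On BeginPlay it hands its gun mesh, danger-detection capsule and sight-range capsule to TD2020AttackBuildingComponent.
; Damage runs the parent handling, then passes the instigator to the attack component's OnDamaged.
; Construction and component lookup defer to the parent.
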(event EventBeginPlay
  (bind _td2020attackbuildingcomponent (Variables|Default|GetTD2020AttackBuildingComponent))
  ;[1 1 1] Begin play
  (Variables|/Game/TD2020/Blueprints/Components/TD2020AttackBuildingComponent.TD2020AttackBuildingComponent_C|SetFireMesh _td2020attackbuildingcomponent (Variables|Default|GetTower1_Gun))
  (Variables|/Game/TD2020/Blueprints/Components/TD2020AttackComponent.TD2020AttackComponent_C|SetDangerDetectionCapsule _td2020attackbuildingcomponent (Variables|Default|GetDangerDetection))
  (Variables|/Game/TD2020/Blueprints/Components/TD2020AttackComponent.TD2020AttackComponent_C|SetSightRangeCapsule _td2020attackbuildingcomponent (Variables|Default|GetSightRange)))

(fn ConstructionScript
  (|CallParentFunction))

(fn GetComponents
  (bind (_rtsselectable _rtsowner _rtsattackable _rtshealth _rtsproductioncost _rtsproduction _rtsconstructionsite _rtsname _rtsportrait _td2020construction _td2020vacancy _rtsresourcedrain) (|CallParentFunction))
  (return _rtsselectable _rtsowner _rtsattackable _rtshealth _rtsproductioncost _rtsproduction _rtsconstructionsite _rtsname _rtsportrait _td2020construction _td2020vacancy _rtsresourcedrain))

(fn OnDamaged
  (params (Damage :type Float%20%28single-precision%29) (DamageType :type Damage%20Type%20Object%20Reference) (InstigatedBy :type Controller%20Object%20Reference) (DamageCauser :type Actor%20Object%20Reference))
  (|CallParentFunction Damage DamageType InstigatedBy DamageCauser)
  (bind _return (Default|OnDamaged (Variables|Default|GetTD2020AttackBuildingComponent) InstigatedBy))
  (return _return))