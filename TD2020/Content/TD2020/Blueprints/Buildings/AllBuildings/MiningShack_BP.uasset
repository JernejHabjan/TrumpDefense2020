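; Mining Shack building Blueprint for an RTS game, derived from a shared building parent.
; Its construction script fills the building struct with its name, type, occupation, employee cap and avatar.
; GetOccupants reports occupancy from the employee array.
; GetComponents passes through the parent's RTS and TD2020 components and supplies its own resource drain component.
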(event EventBeginPlay
  (|CallParentFunction))

(fn ConstructionScript
  (|CallParentFunction)
  (Variables|Default|SetBuildingStruct (Utilities|Struct|MakeBuilding_STRUCT_02 self "NewEnumerator2" "Mining Shack" "NewEnumerator2" 3 0 "/Game/TD2020/Textures/StaticMeshes/RTSBuildings/vertical_planks_done.vertical_planks_done")))

(fn GetOccupants
  (bind _employees_bp (Variables|Default|GetEmployees_BP))
  (bind _returnvalue (Utilities|Array|Length _employees_bp))
  (return (> _returnvalue 0) _returnvalue _employees_bp))

(fn GetComponents
  (bind (_rtsselectable _rtsowner _rtsattackable _rtshealth _rtsproductioncost _rtsproduction _rtsconstructionsite _rtsname _rtsportrait _td2020construction _td2020vacancy) (|CallParentFunction))
  (return _rtsselectable _rtsowner _rtsattackable _rtshealth _rtsproductioncost _rtsproduction _rtsconstructionsite _rtsname _rtsportrait _td2020construction _td2020vacancy (Variables|Default|GetRTSResourceDrain)))