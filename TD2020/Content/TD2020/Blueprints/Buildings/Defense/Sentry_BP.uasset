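; Sentry turret defense building that tracks a target and fires projectiles at it.
; Each Tick, while TargetLocked, it picks the first Targets entry with HP left, turns the gun toward it with interpolated yaw and clamped pitch, and fires if InFiringRange; otherwise it idles in a slow spin.
; A Delay re-called from Tick paces Projectile_BP spawns at the BarrelEnd socket.
; Targets, TargetLocked and InFiringRange are not set in these graphs.
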(event Custom|UpdateTurretRotation
  (bind _currenttarget (Variables|Default|GetCurrentTarget))
  (bind _tower1_gun (Variables|Default|GetTower1_Gun))
  (bind _returnvalue (Transformation|GetActorLocation _currenttarget))
  (bind _returnvalue_2 (Transformation|GetWorldLocation _tower1_gun))
  (bind _returnvalue_3 (Math|Rotator|FindLookatRotation _returnvalue_2 _returnvalue))
  (bind (_roll _pitch _yaw) (Math|Rotator|BreakRotator _returnvalue_3))
  ;[1 1 1] Update turret rotation
  (Transformation|SetWorldRotation (Variables|Default|GetTower1_Gun) (Math|Interpolation|RInterpTo (Transformation|GetWorldRotation (Variables|Default|GetTower1_Gun)) (Math|Rotator|MakeRotator 0.0 (Math|Float|ClampAngle _pitch -3e+01 5e+01) _yaw) (Variables|Default|GetDeltaTime) (Variables|Default|GetInterpLockOnSpeed)) false false))

(event Custom|Idle
  (bind _tower1_gun (Variables|Default|GetTower1_Gun))
  (bind _returnvalue (Transformation|GetWorldRotation _tower1_gun))
  ;[1 1 1] Idle
  (Transformation|SetWorldRotation (Variables|Default|GetTower1_Gun) (Math|Interpolation|RInterpTo _returnvalue (Math|Rotator|MakeRotator 0.0 0.0 (+ (.Yaw (Math|Rotator|BreakRotator _returnvalue)) 1.0)) (Variables|Default|GetDeltaTime) (Variables|Default|GetInterpIdleSpeed)) false false))

(event EventBeginPlay
  ;[1 1 1] Begin Play
  (|CallParentFunction) ; This node is disabled and will not be called.\nDrag off pins to build functionality.
)

(event EventTick
  (params (DeltaSeconds :type Float%20%28single-precision%29))
  ;[1 1 1] Tick
  (Variables|Default|SetDeltaTime DeltaSeconds)
  (if (Variables|Default|GetTargetLocked?)
    (bind _array_element (Utilities|Array|ForEachLoopwithBreak (Variables|Default|GetTargets) :!label _label)
      (:LoopBody
        (bind _as0_base (Utilities|Casting|CastTo0_Base _array_element))
        (if (> (.CurrentHP (Utilities|Struct|BreakEntity_Struct (Variables|/Game/TD2020/Blueprints/AI/Characters/0_Base.0_Base_C|GetEntity_Struct _as0_base))) 0)
          (Variables|Default|SetCurrentTarget _array_element)
          (goto _label Break)))
      (:Completed
        (CallFunction|UpdateTurretRotation)
        (if (Variables|Default|GetInFiringRange?)
          (CallFunction|Fire))))
    (else
      (CallFunction|Idle))))

(event EventFire
  ;[1 1 1] Fire
  (Utilities|FlowControl|Delay (Variables|Default|GetShootingDelay))
  (Game|SpawnActorfromClass "/Game/TD2020/Blueprints/Items/SpecificItems/Projectiles/Projectile_BP.Projectile_BP_C" (Transformation|GetSocketTransform (Variables|Default|GetTower1_Gun) "BarrelEnd" "RTS_World") "Undefined" 0 0 0.0 0)
  (Development|PrintString "FIRe"))

(fn ConstructionScript
  (|CallParentFunction))