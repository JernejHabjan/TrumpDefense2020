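; Base actor for selectable, team-owned RTS entities in TD2020, with stubbed widget, damage, death and right-click functions.
; On BeginPlay it caches its Commander's controller, and the authority copies team and ownership from the Commander.
; Selection by a locally controlled pawn shows its UI list and rally markers, managed through TD2020RallyComponent.
; A timeline lerps the Commander to the actor, then opens a delayed Tick gate that keeps it following in XY.
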(event Custom|LerpToCharacter
  ;[1 1 1] Lerp
  (bind _speed (Timeline|LerpTimeline PlayFromStart)
    (:Update
      (Transformation|SetActorLocation (Variables|Default|GetCommander) (Class|FunctionLibrary|HUDLerpLocation (Transformation|GetActorLocation (Variables|Default|GetCommander)) (Transformation|GetActorLocation) _speed) false false))
    (:Finished
      (CallFunction|OpenFollowGate))))

(event Custom|CloseFollowGate
  (bind _returnvalue (Transformation|GetActorLocation))
  (bind _commander (Variables|Default|GetCommander))
  ;[1 1 1] EventTick - TICKS SET IN 0_BASE
  (Utilities|FlowControl|Gate true) ; enters at Close
)

(event Custom|OpenFollowGate
  (bind _returnvalue (Transformation|GetActorLocation))
  (bind _commander (Variables|Default|GetCommander))
  ;[1 1 1] EventTick - TICKS SET IN 0_BASE
  (Utilities|FlowControl|Gate true) ; enters at Open
)

(event EventBeginPlay
  (bind _commander (Variables|Default|GetCommander))
  (bind _commander_2 (Variables|Default|GetCommander))
  (bind _returnvalue (Components|GetOwner _commander_2))
  (bind _ascontroller (Utilities|Casting|CastToController _returnvalue))
  ;[1 1 1] BeginPlay
  (Utilities|IsValid _commander
    (:Is%20Valid
      (Variables|Default|SetControllerRef (Variables|/Game/TD2020/Blueprints/Pawns/Pawn_MasterCommander.Pawn_MasterCommander_C|GetPlayerController _commander))
      (CallFunction|CreateWidgets)
      ;;[1 1 1] TODO WHERE TO PLACE THIS
      (Networking|SwitchHasAuthority
        (:Authority
          (bind _teamname (Default|GetTeamName (Variables|Default|GetCommander)))
          (CallFunction|SetTeamName _teamname)
          (Class|RTSOwnerComponent|SetPlayerOwner (Variables|Components|GetRTSOwner) _ascontroller)
          (Actor|SetOwner _ascontroller)
          (Variables|Default|SetGameStateRef (.AsGS%20My%20GS (Utilities|Casting|CastToGS_MyGS (Game|GetGameState)))))))
    (:Is%20Not%20Valid
      (Development|PrintString (Utilities|String|Append "commander in my actor is invalid for -> " (Utilities|GetClassDisplayName (Utilities|GetClass self))) true true "(R=1.000000,G=0.066736,B=0.000000,A=1.000000)" 1e+01))))

(event EventTick
  (params (DeltaSeconds :type Float%20%28single-precision%29))
  (bind _returnvalue (Transformation|GetActorLocation))
  (bind _commander (Variables|Default|GetCommander))
  ;[1 1 1] EventTick - TICKS SET IN 0_BASE
  (Utilities|FlowControl|Delay 0.1)
  (Utilities|FlowControl|Gate true
    (:Exit
      (Transformation|SetActorLocation _commander (Math|Vector|MakeVector (.x _returnvalue) (.y _returnvalue) (.z (Transformation|GetActorLocation _commander))) false false))))

(event Game|Damage|EventAnyDamage
  (params (Damage :type Float%20%28single-precision%29) (DamageType :type Damage%20Type%20Object%20Reference) (InstigatedBy :type Controller%20Object%20Reference) (DamageCauser :type Actor%20Object%20Reference))
  ;[1 1 1] Recieve damage
  (CallFunction|OnDamaged Damage DamageType InstigatedBy DamageCauser))

(event EventDestroyed
  ;[1 1 1] destroyed
  (CallFunction|OnDeath))

(fn ConstructionScript
  (Default|SetRallyMeshes (Variables|Default|GetTD2020RallyComponent) (Variables|Default|GetRallyStaticMesh) (Variables|Default|GetRallySkeletalMesh)))

(fn OnDeath
  (return 0))

(fn SetSelected
  (params (Selected? :type Boolean) (InPawn :type Pawn%20Master%20Commander%20Object%20Reference))
  (bind _listwidget (Variables|Default|GetListWidget))
  (Variables|Default|SetSelected Selected?)
  (if (Pawn|IsLocallyControlled InPawn)
    (bind _aswb_main_ui (Utilities|Casting|CastToWB_MainUI (Variables|/Game/TD2020/Blueprints/Pawns/Pawn_MasterCommander.Pawn_MasterCommander_C|GetWB_MainUI InPawn)))
    (if (Variables|Default|GetSelected)
      (Variables|/Game/TD2020/Widgets/HUDs/WB_MainUI.WB_MainUI_C|SetInfantryList _aswb_main_ui _listwidget)
      ;[1 1 1] TODO toj wrong - lahko bi settu samo en list ne pa več na isto
      (Variables|/Game/TD2020/Widgets/HUDs/WB_MainUI.WB_MainUI_C|SetActionList _aswb_main_ui _listwidget)
      (Default|ShowDesiredList _aswb_main_ui (Variables|Default|GetListName))
      (Default|SetRallyVisibility (Variables|Default|GetTD2020RallyComponent) true)
      (return 0))))

(fn SetRally
  (params (Rally :type Vector))
  (Default|SetRally (Variables|Default|GetTD2020RallyComponent) Rally))

(fn CreateWidgets
  (return 0))

(fn OnDamaged
  (params (Damage :type Float%20%28single-precision%29) (DamageType :type Damage%20Type%20Object%20Reference) (InstigatedBy :type Controller%20Object%20Reference) (DamageCauser :type Actor%20Object%20Reference))
  (return 0))

(fn AddRally
  (params (Location :type Vector :default "0, 0, 0") (Action :type String) (Actor :type Actor%20Object%20Reference))
  (Default|AddRally (Variables|Default|GetTD2020RallyComponent) Location Action Actor)
  (return 0))

(fn GetComponents
  (return (Variables|Components|GetRTSSelectable) (Variables|Components|GetRTSOwner) (Variables|Components|GetRTSAttackable) (Variables|Components|GetRTSHealth) 0 0 0 (Variables|Components|GetRTSName) (Variables|Components|GetRTSPortrait) 0 0 0))

(fn GetListName
  (return (Variables|Default|GetListName)))

(fn GetRallies
  (bind _td2020rallycomponent (Variables|Default|GetTD2020RallyComponent))
  (bind (_startlocation _rallylocations _rallyactions) (Default|GetRallies _td2020rallycomponent))
  (return _startlocation _rallylocations _rallyactions))

(fn GetTeamName
  (return (.TeamName (Utilities|Struct|BreakEntity_Struct (Variables|Default|GetEntityStruct)))))

(fn ImNotSelected
  (params (InPawn :type Pawn%20Master%20Commander%20Object%20Reference))
  (bind _return (CallFunction|SetSelected false InPawn))
  (return _return))

(fn ImSelected
  (params (InPawn :type Pawn%20Master%20Commander%20Object%20Reference))
  (bind _return (CallFunction|SetSelected true InPawn))
  (return _return))

(fn RemoveRallies
  (Default|RemoveRallies (Variables|Default|GetTD2020RallyComponent))
  (return 0))

(fn RMBHit
  (params (InCommander :type Actor%20Object%20Reference))
  (return 0))

(fn SetTeamName
  (params (TeamName :type String))
  (Utilities|Struct|SetmembersinEntity_Struct (Variables|Default|GetEntityStruct) TeamName)
  (return 0))