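; Construction office component for a building that employs workers and takes on construction job sites.
; A looping timer, started via the job-timer events, calls BidForJob when employees exist, pausing on success until the construction manager reports that site finished.
; BidForJob's hard-wired true branch always returns false, so the manager bid is never reached.
; Hiring is capped by the building's data, and employees receive the current site's entrance as job location.
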(event Custom|FinishedConstruction
  (params (JobSiteProxy :type Construction%20Proxy%20Object%20Reference))
  ;[1 1 1] FinishedConstruction
  (if (== JobSiteProxy (Variables|Private|GetCurrentJobSite)) ; if jobsite is this one that this office has
    (Variables|Private|SetCurrentJobSite 0) ; clear variable
    (Utilities|Time|UnpauseTimerbyHandle (Variables|Private|GetBidTimerHandle))))

(event Custom|ROS_JobTimers
  (params (Commander :type Pawn%20Master%20Commander%20Object%20Reference))
  ;[1 1 1] ROS job timers
  (CallFunction|ROCJobTimers Commander))

(event Custom|ROC_JobTimers
  (params (Target :type Pawn%20Master%20Commander%20Object%20Reference))
  ;[1 1 1] ROC_JobTimers
  (bind _output_get (Variables|Private|SetConstructionManagerRef (Variables|/Game/TD2020/Blueprints/Pawns/Pawn_MasterCommander.Pawn_MasterCommander_C|GetConstructionManagerRef Target)))
  (EventDispatchers|BindEventtoFinishedConstruction _output_get (EventDispatchers|CreateEvent :!event Custom|FinishedConstruction))
  (bind _returnvalue (Utilities|Time|SetTimerbyEvent (EventDispatchers|CreateEvent :!event Custom|BidTimerEvent) 1.0 true)) ; at begin play it starts this timer - checks for job every 1 second
  (Variables|Private|SetBidTimerHandle _returnvalue))

(event Custom|BidTimerEvent
  ;[1 1 1] BidTimerEvent
  (if (.HasEmployees (CallFunction|GetEmployees)) ; if we have employees - bid for job
    (bind _bidsuccessful (CallFunction|BidforJob))
    (if _bidsuccessful ; if we have bid
      (Utilities|Time|PauseTimerbyHandle (Variables|Private|GetBidTimerHandle)) ; not checking anymore untill finished construction
    )))

(event EventBeginPlay
  ;[1 1 1] BeginPlay
  (bind _asbuilding_master_bp (Utilities|Casting|CastToBuildingMaster_BP (Components|GetOwner)))
  (Variables|Private|SetOwner _asbuilding_master_bp))

(fn BidforJob
  (if true ; we wanna bid for job if were not working for a job
    (return false) ; if we have a job return false
    (else
      (bind (_jobsite _wonbid) (Default|BidManager (Variables|Private|GetConstructionManagerRef) (Variables|Private|GetOwner)))
      (Variables|private|SetJobSite_LOCAL _jobsite) ; if we didnt get bid, job site is null
      (if _wonbid
        (Variables|Private|SetCurrentJobSite (Variables|private|GetJobSite_LOCAL))
        (return true) ; successful
        (else
          (return false) ; we send back to person thats calling for bid for job that bid is not successful
        )))))

(fn GetJobStatus
  (return (Utilities|IsValid (Variables|Private|GetCurrentJobSite))))

(fn SetCurrentJob
  (params (CurrentJobSite :type Construction%20Proxy%20Object%20Reference))
  (Variables|Private|SetCurrentJobSite CurrentJobSite)
  (return))

(fn HireEmployee
  (params (Applicant :type NPC%20Object%20Reference))
  (Variables|Private|SetApplicant_LOCAL Applicant)
  (if (CallFunction|CanEmploy?)
    (Utilities|Array|AddUnique (Variables|Private|GetEmployees_BP) (Variables|Private|GetApplicant_LOCAL))
    (return true (Variables|Private|GetOwner))
    (else
      (return false 0))))

(fn GetEmployees
  (bind _employees_bp (Variables|Private|GetEmployees_BP))
  (bind _returnvalue (Utilities|Array|Length _employees_bp))
  (return (> _returnvalue 0) _returnvalue _employees_bp))

(fn AssignEmployeeJob
  (params (Employee :type NPC%20Object%20Reference%20%28by%20ref%29))
  (bind _currentjobsite (Variables|Private|GetCurrentJobSite))
  (bind _applicant_local (Variables|Private|GetApplicant_LOCAL))
  ;[1 0 0.7384] TODO ??? - če npc ni bil zaposlen v tej bajti ni mogu iz nje delat (prej je bil connection iz true
  (if (!= (Utilities|Array|FindItem (Variables|Private|GetEmployees_BP) Employee) -1)
    _
    (else
      _))
  (if (!= (Variables|Private|GetCurrentJobSite) 0)
    (Utilities|IsValid (Variables|Private|GetCurrentJobSite)
      (:Is%20Valid
        (return true _currentjobsite (Transformation|GetWorldLocation (Variables|/Game/TD2020/Blueprints/Buildings/ConstructionProxy.ConstructionProxy_C|GetEntrance _currentjobsite))))
      (:Is%20Not%20Valid
        (Utilities|IsValid _applicant_local
          (:Is%20Valid
            (Rendering|SetActorHiddenInGame _applicant_local false))
          (:Is%20Not%20Valid
            _)))))
  (return false 0 "0, 0, 0"))

(fn CanEmploy?
  (return (< (.NumberOfEmployees (CallFunction|GetEmployees)) (CallFunction|GetMaxEmployees))))

(fn GetMaxEmployees
  (return (Utilities|Struct|BreakS_MyActor (CallFunction|RetrieveActorData (Utilities|GetClass (Variables|Private|GetOwner))))))