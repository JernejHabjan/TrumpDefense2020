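; Attack combat component for a TD2020 BaseCharacter that relays combat events to the unit's AI Blackboard.
; BeginPlay caches the owner and Blackboard key names, printing an error on other actor types.
; Enemy sighting, disengage and visibility overrides update target keys, while commander moves store a pre-fight location, set the override flag and disengage.
; Friendly capsule bumps can set a BumpMove key, depending on override and enemy state, to free stuck units.
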(event EventBeginPlay
  ;[1 1 1] Begin play- set owner / set BBK keys
  (|CallParentFunction)
  (bind _asbase_character (Utilities|Casting|CastToBaseCharacter (Components|GetOwner))
    (:then
      (Variables|Default|SetOwner _asbase_character)
      (Variables|BBK|SetBBK_OverrideAllOtherActions "OverrideAllOtherActions")
      (Variables|BBK|SetBBK_PreFightLocation "PreFightLocation")
      (Variables|BBK|SetBBK_EnemyToFight "EnemyToFight")
      (Variables|BBK|SetBBK_EnemyVisible "EnemyVisible")
      (Variables|BBK|SetBBK_WeaponRange "WeaponRange")
      (Variables|BBK|SetBBK_DisengagePreFightRange "DisengagePreFightRange")
      (Variables|BBK|SetBBK_DisengageEnemyRange "DisengageEnemyRange")
      (Variables|BBK|SetBBK_CurrentlyAttack "CurrentlyAttack")
      (Variables|BBK|SetBBK_BumpMove "BumpMove"))
    (:CastFailed
      (Development|PrintString "Err - This component should be attached to 0_Base" true true "(R=1.000000,G=0.000000,B=0.018539,A=1.000000)" 1e+01))))

(fn MovetobyCommander
  (params (InLocation :type Vector))
  (bind _owner (Variables|Default|GetOwner))
  (bind _returnvalue (AI|GetBlackboard _owner))
  (AI|Components|Blackboard|SetValueasVector _returnvalue (Variables|BBK|GetBBK_PreFightLocation) InLocation)
  (bind _output_get (Variables|/Game/TD2020/Blueprints/AI/Characters/BaseCharacter.BaseCharacter_C|SetOverrideAllOtherActions _owner true))
  (AI|Components|Blackboard|SetValueasBool _returnvalue (Variables|BBK|GetBBK_OverrideAllOtherActions) _output_get)
  (CallFunction|Disengage))

(fn Disengage
  (bind _owner (Variables|Default|GetOwner))
  (bind _returnvalue (AI|GetBlackboard _owner))
  (|CallParentFunction)
  (Utilities|IsValid _returnvalue
    (:Is%20Valid
      (AI|Components|Blackboard|SetValueasObject _returnvalue (Variables|BBK|GetBBK_EnemyToFight) 0)
      (AI|Components|Blackboard|SetValueasBool _returnvalue (Variables|BBK|GetBBK_EnemyVisible) false)
      (return 0))))

(fn OnEnemySight
  (params (InEnemy :type Actor%20Object%20Reference))
  (bind _owner (Variables|Default|GetOwner))
  (bind _returnvalue (AI|GetBlackboard _owner))
  (|CallParentFunction InEnemy)
  (Utilities|IsValid (AI|GetBlackboard (Variables|Default|GetOwner))
    (:Is%20Valid
      (AI|Components|Blackboard|SetValueasObject _returnvalue (Variables|BBK|GetBBK_EnemyToFight) InEnemy)
      (AI|Components|Blackboard|SetValueasBool _returnvalue (Variables|BBK|GetBBK_EnemyVisible) true)
      (return 0))))

(fn OnBumpFriendly
  (params (InCapsuleColision :type Object%20Object%20Reference) (InActor :type Actor%20Object%20Reference))
  (Utilities|Casting|CastToCapsuleComponent InCapsuleColision)
  (if (CallFunction|CheckTeams (Variables|Default|GetOwner) InActor)
    (if (Variables|/Game/TD2020/Blueprints/AI/Characters/BaseCharacter.BaseCharacter_C|GetOverrideAllOtherActions (Variables|Default|GetOwner))
      (Utilities|IsValid (Variables|Default|GetEnemyToFight)
        (:Is%20Valid
          _))
      (else
        (Utilities|IsValid (Variables|Default|GetEnemyToFight)
          (:Is%20Not%20Valid
            _))))
    (Utilities|IsValid (AI|GetBlackboard (Variables|Default|GetOwner))
      (:Is%20Valid
        (AI|Components|Blackboard|SetValueasBool (AI|GetBlackboard (Variables|Default|GetOwner)) (Variables|BBK|GetBBK_BumpMove) true)
        (return)))))

(fn SetEnemyVisiblility
  (params (Visible? :type Boolean))
  (bind _owner (Variables|Default|GetOwner))
  (bind _returnvalue (AI|GetBlackboard _owner))
  (Utilities|IsValid _returnvalue
    (:Is%20Valid
      (AI|Components|Blackboard|SetValueasBool _returnvalue (Variables|BBK|GetBBK_EnemyVisible) Visible?))))