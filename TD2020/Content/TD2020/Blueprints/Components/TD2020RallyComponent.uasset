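; Actor component for MyActor owners that stores rally points as parallel arrays of locations, actions and target actors.
; AddRally appends entries and, on owners with an RTSProductionComponent, moves the rally marker to the new location.
; The marker is a static or skeletal mesh passed in, hidden initially and toggled by SetRallyVisibility.
; While the owner is selected, UpdateRallyToActor refreshes an actor-targeted rally location, but skips index 0.
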(event EventBeginPlay
  (bind _asmy_actor (Utilities|Casting|CastToMyActor (Components|GetOwner))
    (:then
      (Variables|Default|SetOwner _asmy_actor))
    (:CastFailed
      (Development|PrintString "Rally component should be set to MyActor children" true true "(R=1.000000,G=0.000000,B=0.011716,A=1.000000)" 1e+01))))

(fn GetRallies
  (return (Transformation|GetActorLocation (Components|GetOwner)) (Variables|Default|GetRallyLocations) (Variables|Default|GetRallyActions)))

(fn AddRally
  (params (Location :type Vector%20%28by%20ref%29) (Action :type String%20%28by%20ref%29) (Actor :type Actor%20Object%20Reference%20%28by%20ref%29))
  (bind _returnvalue (Utilities|Array|Add (Variables|Default|GetRallyLocations) Location))
  (Utilities|Array|Add (Variables|Default|GetRallyActions) Action)
  (Utilities|Array|Add (Variables|Default|GetRallyActors) Actor)
  (Utilities|IsValid (Actor|GetComponentbyClass (Components|GetOwner) "/Script/RealTimeStrategy.RTSProductionComponent")
    (:Is%20Valid
      (CallFunction|SetRally (Utilities|Array|Get(acopy) (Variables|Default|GetRallyLocations) _returnvalue))
      (return))))

(fn SetRally
  (params (Rally :type Vector))
  (bind _rallystaticmesh (Variables|Components|GetRallyStaticMesh))
  (bind _rallyskeletalmesh (Variables|Components|GetRallySkeletalMesh))
  (Utilities|IsValid _rallystaticmesh
    (:Is%20Valid
      (Transformation|SetWorldLocation _rallystaticmesh Rally false false))
    (:Is%20Not%20Valid
      _))
  (Utilities|IsValid _rallyskeletalmesh
    (:Is%20Valid
      (Transformation|SetWorldLocation _rallyskeletalmesh Rally false false))
    (:Is%20Not%20Valid
      (Development|PrintString "Error - no static or skeletal mesh valid for rally point - make sure you called parent construction script on component owners to set rally meshes" true true "(R=1.000000,G=0.000000,B=0.061617,A=1.000000)" 1e+01))))

(fn SetRallyMeshes
  (params (RallyStaticMesh :type Static%20Mesh%20Component%20Object%20Reference) (RallySkeletalMesh :type Skeletal%20Mesh%20Component%20Object%20Reference))
  (bind _output_get (Variables|Components|SetRallyStaticMesh RallyStaticMesh))
  (Utilities|IsValid _output_get
    (:Is%20Valid
      (Rendering|SetVisibility _output_get false false))
    (:Is%20Not%20Valid
      _))
  (bind _output_get_2 (Variables|Components|SetRallySkeletalMesh RallySkeletalMesh))
  (Utilities|IsValid _output_get_2
    (:Is%20Valid
      (Rendering|SetVisibility _output_get_2 false false))))

(fn RemoveRallies
  (Utilities|Array|Clear (Variables|Default|GetRallyLocations))
  (Utilities|Array|Clear (Variables|Default|GetRallyActions))
  (Utilities|Array|Clear (Variables|Default|GetRallyActors))
  (Variables|Default|SetFirstRallyToActorIndex -1))

(fn UpdateRallytoActor
  (if (Variables|/Game/TD2020/Blueprints/MyActor.MyActor_C|GetSelected (Variables|Default|GetOwner))
    (bind _index (Utilities|FlowControl|ForLoopwithBreak 0 (- (Utilities|Array|Length (Variables|Default|GetRallyActors)) 1) :!label _label)
      (:LoopBody
        (Utilities|IsValid (Utilities|Array|Get(acopy) (Variables|Default|GetRallyActors) _index)
          (:Is%20Valid
            (Variables|Default|SetFirstRallyToActorIndex _index)
            (goto _label Break))))
      (:Completed
        (if (> (Variables|Default|GetFirstRallyToActorIndex) 0) ; if we get index
          (Utilities|Array|SetArrayElem (Variables|Default|GetRallyLocations) (Variables|Default|GetFirstRallyToActorIndex) (Transformation|GetActorLocation (Utilities|Array|Get(acopy) (Variables|Default|GetRallyActors) (Variables|Default|GetFirstRallyToActorIndex)))) ; set that rally location to his location
        )))))

(fn GetRallyPoint
  (bind _rallystaticmesh (Variables|Components|GetRallyStaticMesh))
  (bind _rallyskeletalmesh (Variables|Components|GetRallySkeletalMesh))
  (Utilities|IsValid _rallystaticmesh
    (:Is%20Valid
      (return (Transformation|GetWorldLocation _rallystaticmesh)))
    (:Is%20Not%20Valid
      (Utilities|IsValid _rallyskeletalmesh
        (:Is%20Valid
          (return (Transformation|GetWorldLocation _rallyskeletalmesh)))
        (:Is%20Not%20Valid
          (return "0, 0, 0"))))))

(fn SetRallyVisibility
  (params (Visible? :type Boolean))
  (bind _rallyskeletalmesh (Variables|Components|GetRallySkeletalMesh))
  (bind _rallystaticmesh (Variables|Components|GetRallyStaticMesh))
  (Utilities|IsValid _rallystaticmesh
    (:Is%20Valid
      (Rendering|SetVisibility _rallystaticmesh Visible? false))
    (:Is%20Not%20Valid
      _))
  (Utilities|IsValid _rallyskeletalmesh
    (:Is%20Valid
      (Rendering|SetVisibility _rallyskeletalmesh Visible? false))))