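; Action component for TD2020 that drives a polling loop for an MCTS (Monte Carlo tree search) action search.
; While EnableMCTS is set, Tick prints any best-action string held in Bla, clears it, then calls RetrieveAllData after a one-second Delay.
; RetrieveAllData and CallPythonComponentMethod have empty bodies here, so the search and any Python link are not implemented in this graph.
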(event EventTick
  (params (DeltaSeconds :type Float%20%28single-precision%29))
  (if (Variables|Default|GetEnableMCTS)
    (if (Utilities|Enum|NotEqual(Enum) (Variables|Default|Getbla) "")
      (Development|PrintString (Utilities|String|Append "SET IS FUL- RETRIEVED BEST ACTION    " (Variables|Default|Getbla)))
      (Variables|Default|Setbla ""))
    (Utilities|FlowControl|Delay 1.0)
    (CallFunction|RetrieveAllData)))

(fn RetrieveAllData)