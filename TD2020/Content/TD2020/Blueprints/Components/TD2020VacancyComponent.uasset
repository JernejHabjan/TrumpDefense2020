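; Actor component for TD2020 buildings that tracks resident NPCs and whether the building has room for more.
; It caches its BuildingMaster_BP owner on BeginPlay and reads the resident limit from that building's BuildingStruct.
; A residency application succeeds while the occupant count is below that limit.
; Adding a tenant appends the NPC uniquely to the resident list without rechecking capacity.
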(event EventBeginPlay
  (bind _asbuilding_master_bp (Utilities|Casting|CastToBuildingMaster_BP (Components|GetOwner)))
  (Variables|Default|SetOwner _asbuilding_master_bp))

(fn GetVacancy
  (return (< (.NumberOfOccupants (CallFunction|GetOccupants)) (CallFunction|GetMaxOccupants))))

(fn ApplyforResidency
  (return (CallFunction|GetVacancy)))

(fn SetNewTenant
  (params (NPC :type NPC%20BP%20Object%20Reference%20%28by%20ref%29))
  (Utilities|Array|AddUnique (Variables|Default|GetResidents_BP) NPC))

(fn GetOccupants
  (bind _residents_bp (Variables|Default|GetResidents_BP))
  (bind _returnvalue (Utilities|Array|Length _residents_bp))
  (return (> _returnvalue 0) _returnvalue _residents_bp))

(fn GetMaxOccupants
  (return (.MaxResidents (Utilities|Struct|BreakBuilding_STRUCT_02 (Variables|/Game/TD2020/Blueprints/Buildings/BuildingMaster_BP.BuildingMaster_BP_C|GetBuildingStruct (Variables|Default|GetOwner))))))