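; Base combat component for RTS units that tracks an enemy and combat state, leaving the attack and sight-overlap responses as stubs.
; Danger-capsule overlaps flag opposing characters or projectile issuers, and damage flags the instigator, when no enemy is set.
; Two seconds after engaging, a sphere trace passes the enemy to nearby idle teammates, who can relay it onward.
; LookAtEnemy yaws toward the target, but its InCombat timer logic is disconnected.
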(event Custom|AttackEnemy
  ;[1 1 1] Attack - to be overwritten
)

(event Custom|OnComponentEndOverlap_SightRangeCapsule
  (params (OverlappedComponent :type Primitive%20Component%20Object%20Reference) (OtherActor :type Actor%20Object%20Reference) (OtherComp :type Primitive%20Component%20Object%20Reference) (OtherBodyIndex :type Integer))
  ;[1 1 1] Sight range End overlap
  (Protected|SightEndOverlap OverlappedComponent OtherActor OtherComp OtherBodyIndex))

(event Custom|OnComponentBeginOverlap_DangerDetectionCapsule
  (params (OverlappedComponent :type Primitive%20Component%20Object%20Reference) (OtherActor :type Actor%20Object%20Reference) (OtherComp :type Primitive%20Component%20Object%20Reference) (OtherBodyIndex :type Integer) (bFromSweep :type Boolean) (SweepResult :type Hit%20Result%20Structure%20%28by%20ref%29))
  ;[1 1 1] Danger detection begin overlap
  (Protected|RangeBeginOverlap OverlappedComponent OtherActor OtherComp OtherBodyIndex bFromSweep SweepResult))

(event Custom|OnComponentEndOverlap_DangerDetectionCapsule
  (params (OverlappedComponent :type Primitive%20Component%20Object%20Reference) (OtherActor :type Actor%20Object%20Reference) (OtherComp :type Primitive%20Component%20Object%20Reference) (OtherBodyIndex :type Integer))
  ;[1 1 1] Danger detection end overlap
  (Protected|RangeEndOverlap OverlappedComponent OtherActor OtherComp OtherBodyIndex))

(event Custom|OnComponentBeginOverlap_SightRangeCapsule
  (params (OverlappedComponent :type Primitive%20Component%20Object%20Reference) (OtherActor :type Actor%20Object%20Reference) (OtherComp :type Primitive%20Component%20Object%20Reference) (OtherBodyIndex :type Integer) (bFromSweep :type Boolean) (SweepResult :type Hit%20Result%20Structure%20%28by%20ref%29))
  ;[1 1 1] Sight range begin overlap
  (Protected|SightBeginOverlap OverlappedComponent OtherActor OtherComp OtherBodyIndex bFromSweep SweepResult))

(event EventBeginPlay
  (bind _sightrangecapsule (Variables|Components|GetSightRangeCapsule))
  (bind _dangerdetectioncapsule (Variables|Components|GetDangerDetectionCapsule))
  ;[1 1 1] Begin play - init components and bind them to evnts
  (Utilities|FlowControl|Delay 0.01)
  (Utilities|IsValid (Variables|Components|GetDangerDetectionCapsule)
    (:Is%20Valid
      (Collision|BindEventtoOnComponentBeginOverlap _dangerdetectioncapsule (EventDispatchers|CreateEvent :!event Custom|OnComponentBeginOverlap_DangerDetectionCapsule))
      (Collision|BindEventtoOnComponentEndOverlap _dangerdetectioncapsule (EventDispatchers|CreateEvent :!event Custom|OnComponentEndOverlap_DangerDetectionCapsule))
      (Protected|RangeBeginOverlap 0 0 0 0 false))
    (:Is%20Not%20Valid
      _))
  (Utilities|IsValid (Variables|Components|GetSightRangeCapsule)
    (:Is%20Valid
      (Collision|AssignOnComponentBeginOverlap _sightrangecapsule (EventDispatchers|CreateEvent :!event Custom|OnComponentBeginOverlap_SightRangeCapsule))
      (Collision|BindEventtoOnComponentEndOverlap _sightrangecapsule (EventDispatchers|CreateEvent :!event Custom|OnComponentEndOverlap_SightRangeCapsule))
      (Protected|SightBeginOverlap 0 0 0 0 false) ; check if any actors are overlaping on spawn
    )))

(fn OnEnemySight
  (params (InEnemy :type Actor%20Object%20Reference))
  (Variables|Default|SetEnemyToFight InEnemy)
  (Variables|Default|SetInCombat true)
  (Utilities|Time|SetTimerbyFunctionName 0 "UnitedWeStand" 2.0) ; 2 sec delay to allow our teammates to find their own enemy before helping me
  (return 0))

(fn Disengage
  (Variables|Default|SetEnemyToFight 0)
  (Variables|Default|SetInCombat false)
  (return 0))

(fn OnDangerDetected
  (params (InActor :type Actor%20Object%20Reference))
  (Utilities|IsValid (Variables|Default|GetEnemyToFight)
    (:Is%20Not%20Valid
      (Utilities|Casting|CastToBaseCharacter InActor
        (:then
          (if (not (CallFunction|CheckTeams (Components|GetOwner) InActor))
            (CallFunction|OnEnemySight InActor)))
        (:CastFailed
          (bind _asmaster_item (Utilities|Casting|CastToMasterItem InActor))
          (Utilities|IsValid (Variables|/Game/TD2020/Blueprints/Items/MasterItem.MasterItem_C|GetDamageIssuer _asmaster_item)
            (:Is%20Valid
              (if (not (CallFunction|CheckTeams (Components|GetOwner) (Variables|/Game/TD2020/Blueprints/Items/MasterItem.MasterItem_C|GetDamageIssuer _asmaster_item)))
                (CallFunction|OnEnemySight (Variables|/Game/TD2020/Blueprints/Items/MasterItem.MasterItem_C|GetDamageIssuer _asmaster_item)) ; if not on my team and he fired - add him to my enemy
              ))))))))

(fn OnDamaged
  (params (InstigatedBy :type Actor%20Object%20Reference))
  (bind _returnvalue (Components|GetOwner))
  (bind _returnvalue_2 (Actor|GetComponentbyClass _returnvalue "/Script/RealTimeStrategy.RTSHealthComponent"))
  (Utilities|IsValid _returnvalue_2
    (:Is%20Valid
      (if (> (Class|RTSHealthComponent|GetCurrentHealth _returnvalue_2) 0.0)
        (Utilities|IsValid (Variables|Default|GetEnemyToFight)
          (:Is%20Valid
            _)
          (:Is%20Not%20Valid
            (Utilities|IsValid InstigatedBy
              (:Is%20Valid
                (CallFunction|OnEnemySight InstigatedBy))
              (:Is%20Not%20Valid
                _)))))
      (return 0))))

(fn UnitedWeStand
  (bind _returnvalue (Components|GetOwner))
  (bind _returnvalue_2 (Transformation|GetActorLocation _returnvalue))
  (bind _outhits (Collision|MultiSphereTraceForObjects _returnvalue_2 (+ _returnvalue_2 "0, 0,1.000000") 2e+03 (Utilities|Array|MakeArray "ObjectTypeQuery2" "ObjectTypeQuery3") false 0 "None")) ; radius of call for help
  (for _array_element _outhits
    (if (CallFunction|CheckTeams (Components|GetOwner) (.HitActor (Collision|BreakHitResult _array_element))) ; if teammate
      (Utilities|IsValid (Actor|GetComponentbyClass (.HitActor (Collision|BreakHitResult _array_element)) "TD2020AttackComponent_MY_C")
        (:Is%20Valid
          (Private|DistressCall (Actor|GetComponentbyClass (.HitActor (Collision|BreakHitResult _array_element)) "TD2020AttackComponent_MY_C") (Variables|Default|GetEnemyToFight)) ; give teammate my enemy
        )))))

(fn DistressCall
  (params (InEnemy :type Actor%20Object%20Reference))
  (Utilities|IsValid InEnemy
    (:Is%20Valid
      (Utilities|IsValid (Variables|Default|GetEnemyToFight)
        (:Is%20Valid
          _)
        (:Is%20Not%20Valid
          (CallFunction|OnEnemySight InEnemy))))
    (:Is%20Not%20Valid
      _))
  (return 0))

(fn LookatEnemy
  (bind _returnvalue (Components|GetOwner))
  (bind _returnvalue_2 (Transformation|GetActorRotation _returnvalue))
  (Utilities|IsValid (Variables|Default|GetEnemyToFight)
    (:Is%20Valid
      (Transformation|SetActorRotation _returnvalue (Math|Rotator|MakeRotator (.roll _returnvalue_2) (.pitch _returnvalue_2) (.yaw (Math|Rotator|FindLookatRotation (Transformation|GetActorLocation (Components|GetOwner)) (Transformation|GetActorLocation (Variables|Default|GetEnemyToFight)))))) ; Rotate actor towards enemy
      (return))
    (:Is%20Not%20Valid
      (CallFunction|Disengage) ; enemy is dead
      (return))))

(fn OnRepinCombat)

(fn SightBeginOverlap
  (params (OverlappedComponent :type Primitive%20Component%20Object%20Reference) (OtherActor :type Actor%20Object%20Reference) (OtherComp :type Primitive%20Component%20Object%20Reference) (OtherBodyIndex :type Integer) (FromSweep :type Boolean) (SweepResult :type Hit%20Result%20Structure))
  (return 0))

(fn SightEndOverlap
  (params (OverlappedComponent :type Primitive%20Component%20Object%20Reference) (OtherActor :type Actor%20Object%20Reference) (OtherComp :type Primitive%20Component%20Object%20Reference) (OtherBodyIndex :type Integer))
  (return 0))

(fn RangeBeginOverlap
  (params (OverlappedComponent :type Primitive%20Component%20Object%20Reference) (OtherActor :type Actor%20Object%20Reference) (OtherComp :type Primitive%20Component%20Object%20Reference) (OtherBodyIndex :type Integer) (FromSweep :type Boolean) (SweepResult :type Hit%20Result%20Structure))
  (Private|OnDangerDetected OtherActor)
  (return 0))

(fn RangeEndOverlap
  (params (OverlappedComponent :type Primitive%20Component%20Object%20Reference) (OtherActor :type Actor%20Object%20Reference) (OtherComp :type Primitive%20Component%20Object%20Reference) (OtherBodyIndex :type Integer))
  (return 0))