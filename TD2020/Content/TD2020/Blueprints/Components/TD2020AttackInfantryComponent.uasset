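; Attack component for TD2020 infantry that handles weapons and attack animations for AI-controlled units.
; On BeginPlay it spawns primary and secondary weapons, attaches them to mesh sockets, and equips the primary, which sets fighting style, behavior tree and blackboard ranges.
; AttackEnemy branches on fighting style: rifle and bow aim then fire, while sword plays a montage with timed damage.
; Blackboard flags track attacks, and OnDeath destroys the weapons.
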(event Custom|ROS_SpawnInitialWeapons
  (Utilities|FlowControl|Delay 0.01) ; for behavior tree to start correctly
  (CallFunction|SpawnInitialWeapons))

(event Custom|MC_PlayMontage
  (params (InAnimMontage :type Anim%20Montage%20Object%20Reference))
  ;[1 1 1] Montage
  (bind _returnvalue (Animation|PlayAnimMontage (Variables|Default|GetOwner) InAnimMontage 1.0 "None"))
  (Variables|Default|SetAnimDelay _returnvalue))

(event Custom|ROS_StopMontage
  ;[1 1 1] Montage
  (CallFunction|MCStopMontage))

(event Custom|MC_StopMontage
  (bind _owner (Variables|Default|GetOwner))
  ;[1 1 1] Montage
  (bind _returnvalue (Animation|GetCurrentMontage _owner :!class /Script/Engine.Character))
  (Animation|StopAnimMontage _owner _returnvalue)
  (bind _asmaster_mele (Utilities|Casting|CastToMasterMele (Variables|Weapons|GetWeaponInHand)))
  (Default|SetDamageEnable _asmaster_mele false))

(event EventAttackEnemy
  (|CallParentFunction)
  (Utilities|AttackFire))

(event EventBeginPlay
  (|CallParentFunction)
  (CallFunction|ROSSpawnInitialWeapons))

(fn SpawnInitialWeapons
  (bind _owner (Variables|Default|GetOwner))
  (bind _owner_2 (Variables|Default|GetOwner))
  (bind _returnvalue (Game|SpawnActorfromClass (Variables|Weapons|GetPrimaryWeaponClass) (Transformation|GetActorTransform _owner_2) "Undefined" _owner_2 _owner_2 0))
  (bind _output_get (Variables|Weapons|SetWeaponInHand _returnvalue))
  (Utilities|Array|SetArrayElem (Variables|Weapons|GetWeapons) 0 _output_get true)
  (bind _returnvalue_2 (Game|SpawnActorfromClass (Variables|Weapons|GetSecondaryWeaponClass) (Transformation|GetActorTransform _owner) "Undefined" _owner _owner 0))
  (Utilities|Array|SetArrayElem (Variables|Weapons|GetWeapons) 1 _returnvalue_2 true)
  (CallFunction|EquipWeapon)
  (for (_array_element _array_index) (Variables|Weapons|GetWeapons)
    (if (> _array_index 0)
      (bind _asmaster_weapon (Utilities|Casting|CastToMasterWeapon _array_element))
      (Transformation|AttachComponentToComponent _asmaster_weapon (Variables|/Script/Engine.Character|GetMesh (Variables|Default|GetOwner)) (Variables|/Game/TD2020/Blueprints/Items/MasterWeapon.MasterWeapon_C|GetAttachOffHandSocket _asmaster_weapon) "SnapToTarget" "SnapToTarget" "SnapToTarget" true))))

(fn EquipWeapon
  (params (InWeaponIndexNumber :type Integer))
  (bind _owner (Variables|Default|GetOwner))
  (bind _owner_2 (Variables|Default|GetOwner))
  (bind _asmaster_weapon (Utilities|Casting|CastToMasterWeapon (Variables|Weapons|GetWeaponInHand)))
  (Transformation|AttachComponentToComponent _asmaster_weapon (Variables|/Script/Engine.Character|GetMesh (Variables|Default|GetOwner)) (Variables|/Game/TD2020/Blueprints/Items/MasterWeapon.MasterWeapon_C|GetAttachOffHandSocket _asmaster_weapon) "SnapToTarget" "SnapToTarget" "SnapToTarget" true)
  (bind _output_get (Variables|Weapons|SetWeaponInHand (Utilities|Array|Get(acopy) (Variables|Weapons|GetWeapons))))
  (bind _asmaster_weapon_2 (Utilities|Casting|CastToMasterWeapon _output_get))
  (Variables|Weapons|SetFightingStyle (Variables|/Game/TD2020/Blueprints/Items/MasterWeapon.MasterWeapon_C|GetFightingStyle _asmaster_weapon_2))
  (Transformation|AttachComponentToComponent _asmaster_weapon_2 (Variables|/Script/Engine.Character|GetMesh _owner_2) (Variables|/Game/TD2020/Blueprints/Items/MasterWeapon.MasterWeapon_C|GetAttachInHandSocket _asmaster_weapon_2) "SnapToTarget" "SnapToTarget" "SnapToTarget" true)
  (Class|ITD2020|SwitchBehaviorTree(Message) (Pawn|GetController _owner_2) (Variables|/Game/TD2020/Blueprints/Items/MasterWeapon.MasterWeapon_C|GetBehaviorTree _asmaster_weapon_2))
  (AI|Components|Blackboard|SetValueasFloat (AI|GetBlackboard _owner) (Variables|Default|GetBBK_WeaponRange) (Variables|/Game/TD2020/Blueprints/Items/MasterWeapon.MasterWeapon_C|GetWeaponRange _asmaster_weapon_2))
  (AI|Components|Blackboard|SetValueasFloat (AI|GetBlackboard _owner) (Variables|Default|GetBBK_DisengagePreFightRange) (Variables|Default|GetDisengagePreFightRange))
  (AI|Components|Blackboard|SetValueasFloat (AI|GetBlackboard _owner) (Variables|Default|GetBBK_DisengageEnemyRange) (Variables|Default|GetDisengageEnemyRange)))

(fn OnDeath
  (for _array_element (Variables|Weapons|GetWeapons)
    (Actor|DestroyActor _array_element)))