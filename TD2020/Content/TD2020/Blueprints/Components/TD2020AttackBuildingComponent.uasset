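; Turret attack component for a BuildingMaster_BP building that finds targets and shoots BasicRifleBullet projectiles at them.
; Inherited sight and danger capsule overlaps pick a target with a portrait component, checked by distance, and set whether it is in firing range.
; Tick turns the FireSocket mesh toward living targets with clamped pitch, fires through a Delay when in range, and rescans or idly spins when targetless.
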(event Custom|UpdateTurretRotation
  (bind _firemesh (Variables|Components|GetFireMesh))
  (bind _enemytofight (Variables|Default|GetEnemyToFight))
  (bind _returnvalue (Transformation|GetActorLocation _enemytofight))
  (bind _returnvalue_2 (Transformation|GetWorldLocation _firemesh))
  (bind _returnvalue_3 (Math|Rotator|FindLookatRotation _returnvalue_2 _returnvalue))
  (bind (_roll _pitch _yaw) (Math|Rotator|BreakRotator _returnvalue_3))
  ;[1 1 1] Update turret rotation
  (Transformation|SetWorldRotation (Variables|Components|GetFireMesh) (Math|Interpolation|RInterpTo (Transformation|GetWorldRotation (Variables|Components|GetFireMesh)) (Math|Rotator|MakeRotator 0.0 (Math|Float|ClampAngle _pitch -8e+01 5e+01) _yaw) (Variables|Default|GetDeltaTime) (Variables|Default|GetInterpLockOnSpeed)) false false))

(event Custom|Idle
  (bind _firemesh (Variables|Components|GetFireMesh))
  (bind _returnvalue (Transformation|GetWorldRotation _firemesh))
  ;[1 1 1] Idle - Rotate turret
  (Transformation|SetWorldRotation (Variables|Components|GetFireMesh) (Math|Interpolation|RInterpTo _returnvalue (Math|Rotator|MakeRotator 0.0 0.0 (+ (.Yaw (Math|Rotator|BreakRotator _returnvalue)) 1.0)) (Variables|Default|GetDeltaTime) (Variables|Default|GetInterpIdleSpeed)) false false))

(event EventAttackEnemy
  (bind _owner (Variables|Default|GetOwner))
  ;[1 1 1] Attack - Spawns projectile at fire socket position
  (Utilities|FlowControl|Delay (Variables|Default|GetAttackDelay))
  (Game|SpawnActorfromClass "/Game/TD2020/Blueprints/Items/SpecificItems/Projectiles/BasicRifleBullet.BasicRifleBullet_C" (Transformation|GetSocketTransform (Variables|Components|GetFireMesh) (Variables|Default|GetFireSocket) "RTS_World") "Undefined" _owner _owner 0)
  (Development|PrintString "Fire"))

(event EventTick
  (params (DeltaSeconds :type Float%20%28single-precision%29))
  ;[1 1 1] Tick - Update rotation and fire if any target in range, else update idle
  (bind _output_get (Variables|Default|SetDeltaTime DeltaSeconds))
  (|CallParentFunction _output_get)
  (Utilities|IsValid (Variables|Default|GetOwner)
    (:Is%20Valid
      (Utilities|IsValid (Variables|Default|GetEnemyToFight)
        (:Is%20Valid
          (Utilities|IsValid (Actor|GetComponentbyClass (Variables|Default|GetEnemyToFight) "/Script/RTSPlugin.RTSHealthComponent")
            (:Is%20Valid
              (if (> (Variables|/Script/RTSPlugin.RTSHealthComponent|GetCurrentHealth (Actor|GetComponentbyClass (Variables|Default|GetEnemyToFight) "/Script/RTSPlugin.RTSHealthComponent")) 0.0)
                (CallFunction|UpdateTurretRotation)
                (if (Variables|Default|GetInFiringRange?) :!label _label
                  (CallFunction|AttackEnemy))
                (else
                  (Variables|Default|SetEnemyToFight 0 :!label _label_2))))
            (:Is%20Not%20Valid
              (goto _label_2))))
        (:Is%20Not%20Valid
          (CallFunction|SightBeginOverlap 0 0 0 0 false)
          (Utilities|IsValid (Variables|Default|GetEnemyToFight)
            (:Is%20Valid
              (CallFunction|RangeBeginOverlap 0 0 0 0 false)
              (goto _label))
            (:Is%20Not%20Valid
              (CallFunction|Idle))))))))

(event EventBeginPlay
  ;[1 1 1] Begin play - Set owner / Find component on parent that includes FireSocket name
  (|CallParentFunction)
  (Utilities|FlowControl|Delay 0.01)
  (bind _asbuilding_master_bp (Utilities|Casting|CastToBuildingMaster_BP (Components|GetOwner))
    (:then
      (Variables|Default|SetOwner _asbuilding_master_bp)
      (bind _array_element (Utilities|Array|ForEachLoopwithBreak (Actor|GetComponentsByClass (Variables|Default|GetOwner) "/Script/Engine.StaticMeshComponent") :!label _label)
        (:LoopBody
          (if (Transformation|DoesSocketExist _array_element (Variables|Default|GetFireSocket))
            (Variables|Components|SetFireMesh _array_element)
            (goto _label Break)))))
    (:CastFailed
      (Development|PrintString "Err - This component should be attached to BuildingMasterBP" true true "(R=1.000000,G=0.000000,B=0.018539,A=1.000000)" 1e+01))))

(fn SightBeginOverlap
  (params (OverlappedComponent :type Primitive%20Component%20Object%20Reference) (OtherActor :type Actor%20Object%20Reference) (OtherComp :type Primitive%20Component%20Object%20Reference) (OtherBodyIndex :type Integer) (FromSweep :type Boolean) (SweepResult :type Hit%20Result%20Structure))
  (bind _sightrangecapsule (Variables|Default|GetSightRangeCapsule))
  (bind _overlappingactors (Collision|GetOverlappingActors _sightrangecapsule "/Script/Engine.Actor" :!class /Script/Engine.PrimitiveComponent))
  (bind _enemytofight (Private|FindEnemyinRange _overlappingactors _sightrangecapsule))
  (|CallParentFunction OverlappedComponent OtherActor OtherComp OtherBodyIndex FromSweep SweepResult)
  (Utilities|IsValid _enemytofight
    (:Is%20Valid
      (Utilities|IsValid (Variables|Default|GetEnemyToFight) ; if first one
        (:Is%20Valid
          _)
        (:Is%20Not%20Valid
          (Variables|Default|SetEnemyToFight _enemytofight)))
      (return 0))
    (:Is%20Not%20Valid
      (Variables|Default|SetEnemyToFight 0))))

(fn SightEndOverlap
  (params (OverlappedComponent :type Primitive%20Component%20Object%20Reference) (OtherActor :type Actor%20Object%20Reference) (OtherComp :type Primitive%20Component%20Object%20Reference) (OtherBodyIndex :type Integer))
  (bind _sightrangecapsule (Variables|Default|GetSightRangeCapsule))
  (bind _overlappingactors (Collision|GetOverlappingActors _sightrangecapsule "/Script/Engine.Actor" :!class /Script/Engine.PrimitiveComponent))
  (bind _enemytofight (Private|FindEnemyinRange _overlappingactors _sightrangecapsule))
  (|CallParentFunction OverlappedComponent OtherActor OtherComp OtherBodyIndex)
  (Utilities|IsValid _enemytofight
    (:Is%20Valid
      (Utilities|IsValid (Variables|Default|GetEnemyToFight)
        (:Is%20Valid
          _)
        (:Is%20Not%20Valid
          (Variables|Default|SetEnemyToFight _enemytofight)))
      (return 0))
    (:Is%20Not%20Valid
      (Variables|Default|SetEnemyToFight 0))))

(fn RangeBeginOverlap
  (params (OverlappedComponent :type Primitive%20Component%20Object%20Reference) (OtherActor :type Actor%20Object%20Reference) (OtherComp :type Primitive%20Component%20Object%20Reference) (OtherBodyIndex :type Integer) (FromSweep :type Boolean) (SweepResult :type Hit%20Result%20Structure))
  (bind _dangerdetectioncapsule (Variables|Default|GetDangerDetectionCapsule))
  (bind _overlappingactors (Collision|GetOverlappingActors _dangerdetectioncapsule "/Script/Engine.Actor" :!class /Script/Engine.PrimitiveComponent))
  (bind _enemytofight (Private|FindEnemyinRange _overlappingactors _dangerdetectioncapsule))
  (|CallParentFunction OverlappedComponent OtherActor OtherComp OtherBodyIndex FromSweep SweepResult)
  (Utilities|IsValid _enemytofight
    (:Is%20Valid
      (if (or (not (Utilities|IsValid (Variables|Default|GetEnemyToFight))) (not (Variables|Default|GetInFiringRange?)))
        (Variables|Default|SetEnemyToFight _enemytofight)
        (Variables|Default|SetInFiringRange? true))
      (return 0))))

(fn RangeEndOverlap
  (params (OverlappedComponent :type Primitive%20Component%20Object%20Reference) (OtherActor :type Actor%20Object%20Reference) (OtherComp :type Primitive%20Component%20Object%20Reference) (OtherBodyIndex :type Integer))
  (bind _dangerdetectioncapsule (Variables|Default|GetDangerDetectionCapsule))
  (|CallParentFunction OverlappedComponent OtherActor OtherComp OtherBodyIndex)
  (Utilities|IsValid (Private|FindEnemyinRange (Collision|GetOverlappingActors _dangerdetectioncapsule "/Script/Engine.Actor" :!class /Script/Engine.PrimitiveComponent) _dangerdetectioncapsule)
    (:Is%20Valid
      _)
    (:Is%20Not%20Valid
      (Variables|Default|SetInFiringRange? false)))
  (return 0))

(fn FindEnemyinRange
  (params (Actors :type Array%20of%20Actor%20Object%20References) (Capsule :type Capsule%20Component%20Object%20Reference))
  (LocalVariables|SetEnemyToFight_LOCAL 0)
  (bind _array_element (Utilities|Array|ForEachLoopwithBreak Actors :!label _label)
    (:LoopBody
      (Utilities|IsValid (Actor|GetComponentbyClass _array_element "/Script/RTSPlugin.RTSPortraitComponent")
        (:Is%20Valid
          (if (Private|InRange _array_element Capsule)
            (if (!= _array_element (Variables|Default|GetOwner))
              (LocalVariables|SetEnemyToFight_LOCAL _array_element)
              (goto _label Break))))))
    (:Completed
      (return (LocalVariables|GetEnemyToFight_LOCAL)))))

(fn InRange
  (params (Actor :type Actor%20Object%20Reference) (Capsule :type Capsule%20Component%20Object%20Reference))
  (if (and (Utilities|IsValid (Variables|Default|GetOwner)) (Utilities|IsValid Capsule))
    (return (<= (Math|Vector|VectorLength (- (Transformation|GetActorLocation Actor) (Transformation|GetActorLocation (Variables|Default|GetOwner)))) (Variables|/Script/Engine.CapsuleComponent|GetCapsuleRadius Capsule)))))