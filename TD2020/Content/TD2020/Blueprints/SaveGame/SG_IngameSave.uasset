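; SG_IngameSave is a save game object that holds the state of an in-game session.
; It stores time and speed values, gameplay toggles for building, payment, stamina, jobs, timeouts and condition checking, plus player controller, actor and map data.
; A single Set function copies all of these inputs into the member variables in one call, with no other logic.
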(fn Set
  (params (TimeUnit :type Float%20%28single-precision%29) (TimePlayed :type Float%20%28single-precision%29) (SpeedMultiplier :type Float%20%28single-precision%29) (TimeoutMinutes :type Integer) (InstaBuild :type Boolean) (InstaPay :type Boolean) (EnableStamina :type Boolean) (EnableCriticalStamina :type Boolean) (AutomaticallyCheckJob :type Boolean) (EnableTimeout :type Boolean) (EnableConditionChecking :type Boolean) (PlayerControllerSave :type Array%20of%20Player%20Controller%20Save%20Structures) (MyActorSave :type Array%20of%20My%20Actor%20Save%20Structures) (MapInfo :type Map%20Info%20Struct%20Structure))
  (Variables|Default|SetTimeUnit TimeUnit)
  (Variables|Default|SetTimePlayed TimePlayed)
  (Variables|Default|SetSpeedMultiplier SpeedMultiplier)
  (Variables|Default|SetTimeoutMinutes TimeoutMinutes)
  (Variables|Default|SetInstaBuild InstaBuild)
  (Variables|Default|SetInstaPay InstaPay)
  (Variables|Default|SetEnableStamina EnableStamina)
  (Variables|Default|SetEnableCriticalStamina EnableCriticalStamina)
  (Variables|Default|SetAutomaticallyCheckJob AutomaticallyCheckJob)
  (Variables|Default|SetEnableTimeout EnableTimeout)
  (Variables|Default|SetEnableConditionChecking EnableConditionChecking)
  (Variables|Default|SetPlayerControllerSave PlayerControllerSave)
  (Variables|Default|SetMyActorSave1 MyActorSave)
  (Variables|Default|SetMapInfo MapInfo))