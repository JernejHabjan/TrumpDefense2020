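; GeneralActor is a TD2020 actor Blueprint, apparently a base for selectable, commander-owned objects.
; It exposes its selectable, owner, name and portrait components through GetComponents.
; GetTeamName asks the Commander, falling back to "Neutral" when none is valid.
; Selection, rally, right-click, list-name and team-setting functions are stubs returning defaults or doing nothing, and the event graph is unused.
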(event EventBeginPlay)

(event Collision|EventActorBeginOverlap
  (params (OtherActor :type Actor%20Object%20Reference)))

(event EventTick
  (params (DeltaSeconds :type Float%20%28single-precision%29)))

(fn ConstructionScript)

(fn AddRally
  (params (Location :type Vector :default "0, 0, 0") (Action :type String) (Actor :type Actor%20Object%20Reference))
  (return 0))

(fn GetComponents
  (return (Variables|Default|GetTD2020Selectable) (Variables|Default|GetTD2020Owner) 0 0 0 0 0 (Variables|Default|GetTD2020Name) (Variables|Default|GetTD2020Portrait) 0 0 0))

(fn GetListName
  (return "None"))

(fn GetRallies
  (return "0, 0, 0" 0 0))

(fn GetTeamName
  (bind _commander (Variables|Default|GetCommander))
  (Utilities|IsValid _commander
    (:Is%20Valid
      (bind _teamname (Default|GetTeamName _commander))
      (return _teamname))
    (:Is%20Not%20Valid
      (return "Neutral"))))

(fn ImNotSelected
  (params (InPawn :type Pawn%20Master%20Commander%20Object%20Reference))
  (return 0))

(fn ImSelected
  (params (InPawn :type Pawn%20Master%20Commander%20Object%20Reference))
  (return 0))

(fn RemoveRallies
  (return 0))

(fn RMBHit
  (params (InCommander :type Actor%20Object%20Reference))
  (return 0))

(fn SetTeamName
  (params (TeamName :type String))
  (return 0))