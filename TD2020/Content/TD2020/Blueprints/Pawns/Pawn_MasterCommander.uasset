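; Base RTS commander pawn that handles a player's selection, unit orders, spawning and UI action lists.
; On begin play it spawns construction manager and ghost building helpers, triggers initial buildings and registers with a TensorFlow component.
; ROS events route spawns through MC events gated by authority, while move orders scatter units around navigable points.
; Rally commands reach units or their AI controllers via interface messages, appending on multi-select and replacing otherwise.
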(event Custom|ROS_AddRally
  (params (Condition :type Boolean) (Location :type Vector) (Action :type String) (Actor :type Actor%20Object%20Reference) (SelectedActors :type Array%20of%20Actor%20Object%20References))
  ;[1 1 1] Add rally
  (Commands|AddRallyCommand Condition Location Action Actor SelectedActors))

(event Custom|MC_SpawnActualBuilding
  (params (ConstructionStruct :type Construction%20Struct%2002%20Structure) (LocalCommander :type Pawn%20Master%20Commander%20Object%20Reference))
  ;[1 1 1] Spawn Actual Building
  (Networking|SwitchHasAuthority
    (:Authority
      (BuildingPlacement|SpawnActualBuilding ConstructionStruct LocalCommander))))

(event Custom|ROS_MoveSelectedUnitsTo
  (params (InUnits :type Array%20of%20Actor%20Object%20References) (InLocation :type Vector))
  ;[1 1 1] Move Units to
  (CallFunction|MoveSelectedUnitsto InUnits InLocation))

(event Custom|ROS_ActionQueue
  (params (Character :type Base%20Character%20Object%20Reference))
  (bind _returnvalue (AI|GetAIController Character))
  ;[1 1 1] ROS Action Queue
  (Utilities|IsValid _returnvalue
    (:Is%20Valid
      (bind _ascharacter_aicontroller (Utilities|Casting|CastToCharacterAIController _returnvalue))
      (Default|ActionQueue _ascharacter_aicontroller))))

(event Custom|ROS_SpawnProxyBuilding
  (params (ConstructionStruct :type Construction%20Struct%2002%20Structure) (Commander :type Pawn%20Master%20Commander%20Object%20Reference))
  ;[1 1 1] Spawn Proxy Building
  (CallFunction|MCSpawnProxyBuilding ConstructionStruct Commander))

(event Custom|ROS_RemoveRallies
  (params (Target :type Actor%20Object%20Reference))
  ;[1 1 1] Add rally
  (Class|ITD2020|RemoveRallies(Message) Target))

(event Custom|ROS_SpawnActualBuilding
  (params (ConstructionStruct :type Construction%20Struct%2002%20Structure) (LocalCommander :type Pawn%20Master%20Commander%20Object%20Reference))
  ;[1 1 1] Spawn Actual Building
  (CallFunction|MCSpawnActualBuilding ConstructionStruct LocalCommander))

(event Custom|MC_SpawnProxyBuilding
  (params (ConstructionStruct :type Construction%20Struct%2002%20Structure) (Commander :type Pawn%20Master%20Commander%20Object%20Reference))
  ;[1 1 1] Spawn Proxy Building
  (Networking|SwitchHasAuthority
    (:Authority
      (BuildingPlacement|SpawnProxyBuilding ConstructionStruct Commander))))

(event Custom|ROS_MoveUnitTo
  (params (Actor :type Actor%20Object%20Reference) (InLocation :type Vector))
  ;[1 1 1] Move Units to
  (CallFunction|MoveUnitto Actor InLocation))

(event Custom|ROS_SpawnUnit
  (params (InUnit :type Base%20Character%20Class%20Reference) (InSpawnPoint :type Transform) (InCommander :type Pawn%20Object%20Reference) (InSpawnFlagLocation :type Vector))
  ;[1 1 1] Spawn unit - spawn them on server - because player controller is only on server - dont multicast
  (CallFunction|MCSpawnUnit InUnit InSpawnPoint InCommander InSpawnFlagLocation))

(event Custom|ROS_BeginPlay
  ;[1 1 1] Ros begin play
  (CallFunction|MCBeginPlay))

(event Custom|EOS_CreateWidgets
  ;[1 1 1] Create widgets
  (CallFunction|CreateWidgets))

(event Custom|MC_SpawnUnit
  (params (InUnit :type Base%20Character%20Class%20Reference) (InSpawnPoint :type Transform) (InCommander :type Pawn%20Object%20Reference) (InSpawnFlagLocation :type Vector))
  ;[1 1 1] Spawn unit - spawn them on server - because player controller is only on server - dont multicast
  (Networking|SwitchHasAuthority
    (:Authority
      (UnitSpawning|SpawnUnit InUnit InSpawnPoint InCommander InSpawnFlagLocation))))

(event Custom|MC_BeginPlay
  ;[1 1 1] ROC begin play
  (CallFunction|CreateReferences)
  (Class|RTSOwnerComponent|SetPlayerOwner (Variables|Default|GetRTSOwner) (.AsController (Utilities|Casting|CastToController (Components|GetOwner)))))

(event EventBeginPlay
  (bind _constructionmanagerref (Variables|References|GetConstructionManagerRef))
  (bind _asgi_my_gi (Utilities|Casting|CastToGI_MyGI (Game|GetGameInstance)))
  ;[1 1 1] Begin play
  (if (CallFunction|GetValidMap (Game|GetGameInstance))
    (Utilities|FlowControl|Sequence
      (:then_0
        (CallFunction|ROSBeginPlay)
        (Utilities|IsValid _constructionmanagerref
          (:Is%20Valid
            (Default|SpawnInitialBuildings _constructionmanagerref) ; If you want something to spawn for both players on start - spawn from construction manager for example
          )))
      (:then_1
        (Default|SetPlayerTensorflow (Variables|Default|GetCmpTensorflow) self)))))

(fn ConstructionScript)

(fn IsMoving
  (params (AxisX :type Float%20%28single-precision%29) (AxisY :type Float%20%28single-precision%29))
  (return (or (> (Math|Float|Absolute(Float) AxisX) 0.0) (> (Math|Float|Absolute(Float) AxisY) 0.0))))

(fn SetNPCSpawnPoint
  (bind _returnvalue (Game|GetPlayerController 0))
  (bind _aspc_gameplay_pc (Utilities|Casting|CastToPC_GameplayPC _returnvalue))
  (bind _location (CallFunction|SetCursorWorldPosition _aspc_gameplay_pc 1e+04))
  (Variables|Camera|SetCursorWorldPosition (Math|Vector|MakeVector (.x _location) (.y _location) (+ (.z _location) 1e+02)))
  (return (Math|Transform|MakeTransform (Variables|Camera|GetCursorWorldPosition) "0, 0, 0" (Variables|Construction|GetActorScaleFactor))))

(fn SpawnUnit
  (params (InUnit :type Base%20Character%20Class%20Reference) (InSpawnPoint :type Transform) (InCommander :type Pawn%20Object%20Reference) (InSpawnFlagLocation :type Vector))
  (bind _aspawn_master_commander (Utilities|Casting|CastToPawn_MasterCommander InCommander))
  (LocalVariables|SetLoc InSpawnFlagLocation)
  (bind _returnvalue (Game|SpawnActorfromClass InUnit InSpawnPoint "AdjustIfPossibleButAlwaysSpawn" _aspawn_master_commander _aspawn_master_commander 0))
  (Pawn|SpawnDefaultController _returnvalue)
  (bind _asgm_gameplay_gm (Utilities|Casting|CastToGM_GameplayGM (Game|GetGameMode))
    (:then
      (if (Variables|/Game/TD2020/Blueprints/Logics/GM_GameplayGM.GM_GameplayGM_C|GetMiddleOfTileMove _asgm_gameplay_gm)
        _
        (else
          (LocalVariables|SetLoc (Math|Vector|MakeVector (.X (Math|Vector|BreakVector (.RandomLocation (Class|NavigationSystemV1|GetRandomPointinNavigableRadius (LocalVariables|GetLoc) 3e+02 0 0)))) (.Y (Math|Vector|BreakVector (.RandomLocation (Class|NavigationSystemV1|GetRandomPointinNavigableRadius (LocalVariables|GetLoc) 3e+02 0 0)))) (+ (.Z (Math|Vector|BreakVector (.RandomLocation (Class|NavigationSystemV1|GetRandomPointinNavigableRadius (LocalVariables|GetLoc) 3e+02 0 0)))) 1e+02)))))
      (Class|ITD2020|MovebyCommander(Message) _returnvalue (LocalVariables|GetLoc)))
    (:CastFailed
      (Class|ITD2020|MovebyCommander(Message) _returnvalue (LocalVariables|GetLoc)))))

(fn MoveSelectedUnitsto
  (params (InUnits :type Array%20of%20Actor%20Object%20References) (InLocation :type Vector))
  (for _array_element InUnits
    (Class|ITD2020|MovebyCommander(Message) _array_element (.RandomLocation (Class|NavigationSystemV1|GetRandomPointinNavigableRadius InLocation (* (Utilities|Array|Length InUnits) 2e+01) 0 0)))))

(fn SpawnActualBuilding
  (params (ConstructionStruct :type Construction%20Struct%2002%20Structure) (LocalCommander :type Pawn%20Master%20Commander%20Object%20Reference))
  (bind (_buildingclass _transform) (Utilities|Struct|BreakConstruction_Struct_02 ConstructionStruct))
  (Game|SpawnActorfromClass _buildingclass _transform "Undefined" 0 0 LocalCommander 0))

(fn SpawnProxyBuilding
  (params (ConstructionStruct :type Construction%20Struct%2002%20Structure) (Commander :type Pawn%20Master%20Commander%20Object%20Reference))
  (bind (_buildingclass _proxyclass _transform _displaymesh _builder) (Utilities|Struct|BreakConstruction_Struct_02 ConstructionStruct))
  (bind _returnvalue (Game|SpawnActorfromClass _proxyclass _transform "Undefined" 0 _displaymesh _buildingclass _builder Commander 0))
  (Default|ProxyStart (Variables|References|GetConstructionManagerRef) _returnvalue ConstructionStruct))

(fn CreateWidgets
  (return 0))

(fn MoveUnitto
  (params (Actor :type Actor%20Object%20Reference) (InLocation :type Vector))
  (Class|ITD2020|MovebyCommander(Message) Actor (.RandomLocation (Class|NavigationSystemV1|GetRandomPointinNavigableRadius InLocation 5e+01 0 0))))

(fn SelectActor
  (params (Actor :type Actor%20Object%20Reference))
  (Utilities|IsValid Actor
    (:Is%20Valid
      (bind _rtsselectable (Class|ITD2020|GetComponents(Message) Actor))
      (Utilities|IsValid _rtsselectable
        (:Is%20Valid
          (Class|RTSSelectableComponent|SelectActor _rtsselectable)
          (Utilities|Casting|CastToBaseCharacter Actor
            (:then
              (Variables|Selection|SetSelectedAnyNPCS? true))
            (:CastFailed
              _))
          (if (not (Utilities|Array|ContainsItem (Variables|Selection|GetCurrentSelectedActors) Actor))
            (Utilities|Array|Add (Variables|Selection|GetCurrentSelectedActors) Actor)
            (Class|ITD2020|ImSelected(Message) Actor self)))))))

(fn DeselectActor
  (params (Actor :type Actor%20Object%20Reference) (MultipleDeselect? :type Boolean))
  (bind _wb_mainui (Variables|Widgets|GetWB_MainUI))
  (if (Utilities|Array|ContainsItem (Variables|Selection|GetCurrentSelectedActors) Actor) ; if false it, we may be deselecting enemy units
    (Utilities|Array|RemoveItem (Variables|Selection|GetCurrentSelectedActors) Actor))
  (Utilities|IsValid Actor
    (:Is%20Valid
      (Class|ITD2020|ImNotSelected(Message) Actor self))
    (:Is%20Not%20Valid
      _))
  (Default|SwapSelectedActorWidget _wb_mainui) ; clear profile pic and data
  (Default|RemovefromSelection (Variables|/Game/TD2020/Widgets/HUDs/WB_MainUI.WB_MainUI_C|GetWB_Selection _wb_mainui) Actor)
  ;[1 1 1] RTS
  (Utilities|IsValid Actor
    (:Is%20Valid
      (Class|RTSSelectableComponent|DeselectActor (Actor|GetComponentbyClass Actor "/Script/RealTimeStrategy.RTSSelectableComponent"))
      (if (not MultipleDeselect?) ; if running deselect all actors - call clear selections instead of running for loops in WB Selection widget for each actor
        ;[1 1 1] Selection tab - little icons
        (Default|RemovefromSelection (Variables|/Game/TD2020/Widgets/HUDs/WB_MainUI.WB_MainUI_C|GetWB_Selection (Variables|Widgets|GetWB_MainUI)) Actor)))))

(fn AddRallyCommand
  (params (MultipleSelection? :type Boolean) (Location :type Vector) (Action :type String) (Actor :type Actor%20Object%20Reference) (SelectedActors :type Array%20of%20Actor%20Object%20References))
  (LocalVariables|SetLocation_LOCAL Location)
  (LocalVariables|SetAction_LOCAL Action)
  (LocalVariables|SetActor_LOCAL Actor)
  (if MultipleSelection? ; if holding shift while
    (for _array_element SelectedActors
      (bind _asbase_character (Utilities|Casting|CastToBaseCharacter _array_element)
        (:then
          (Class|ITD2020|AddRally(Message) (Variables|/Game/TD2020/Blueprints/AI/Characters/BaseCharacter.BaseCharacter_C|GetAIController _asbase_character) (LocalVariables|GetLocation_LOCAL) (LocalVariables|GetAction_LOCAL) (LocalVariables|GetActor_LOCAL)))
        (:CastFailed
          (Class|ITD2020|AddRally(Message) _array_element (LocalVariables|GetLocation_LOCAL) (LocalVariables|GetAction_LOCAL) (LocalVariables|GetActor_LOCAL)))))
    (else
      (for _array_element_2 SelectedActors
        (bind _asbase_character_2 (Utilities|Casting|CastToBaseCharacter _array_element_2)
          (:then
            (Default|RemoveRallies (Variables|/Game/TD2020/Blueprints/AI/Characters/BaseCharacter.BaseCharacter_C|GetAIController _asbase_character_2))
            (Class|ITD2020|AddRally(Message) (Variables|/Game/TD2020/Blueprints/AI/Characters/BaseCharacter.BaseCharacter_C|GetAIController _asbase_character_2) (LocalVariables|GetLocation_LOCAL) (LocalVariables|GetAction_LOCAL) (LocalVariables|GetActor_LOCAL)))
          (:CastFailed
            (Class|ITD2020|RemoveRallies(Message) _array_element_2)
            (Class|ITD2020|AddRally(Message) _array_element_2 (LocalVariables|GetLocation_LOCAL) (LocalVariables|GetAction_LOCAL) (LocalVariables|GetActor_LOCAL))))))))

(fn StopCommand
  (for _array_element (Variables|Selection|GetCurrentSelectedActors)
    (bind _rallylocations (Class|ITD2020|GetRallies(Message) _array_element))
    (LocalVariables|SetTempRallyLocations _rallylocations)
    (if (Variables|Selection|GetMultipleSelection)
      (if (> (Utilities|Array|Length (LocalVariables|GetTempRallyLocations)) 1)
        (CallFunction|ROSAddRally (Variables|Selection|GetMultipleSelection) (Utilities|Array|Get(acopy) (LocalVariables|GetTempRallyLocations) (- (Utilities|Array|Length (LocalVariables|GetTempRallyLocations)) 1)) "Stop" 0 (Variables|Selection|GetCurrentSelectedActors))
        (else
          (CallFunction|ROSAddRally (Variables|Selection|GetMultipleSelection) (Transformation|GetActorLocation _array_element) "Stop" 0 (Variables|Selection|GetCurrentSelectedActors) :!label _label)))
      (else
        (goto _label)))))

(fn DeselectActors
  (params (Array :type Array%20of%20Actor%20Object%20References))
  (for _array_element Array
    (Selection|DeselectActor _array_element true))
  (Utilities|Array|Clear Array)
  ;[1 1 1] Selection tab - little icons
  (Default|ClearSelections (Variables|/Game/TD2020/Widgets/HUDs/WB_MainUI.WB_MainUI_C|GetWB_Selection (Variables|Widgets|GetWB_MainUI))))

(fn SetCurrentActionList
  (params (Issuer :type Actor%20Object%20Reference) (Action :type Action%20Struct%20Structure) (ParentListName :type Name))
  (bind _wb_mainui (Variables|Widgets|GetWB_MainUI))
  (Variables|Default|SetCurrentExecutingAction (.ActionName (Utilities|Struct|BreakAction_Struct Action)))
  (bind _returnvalue (UserInterface|CreateWidget "/Game/TD2020/Widgets/HUDs/HumanWidgets/WB_CurrentActionList.WB_CurrentActionList_C" 0 self Issuer Action ParentListName))
  (bind _output_get (Variables|Default|SetWB_CurrentAction _returnvalue))
  (Variables|/Game/TD2020/Widgets/HUDs/WB_MainUI.WB_MainUI_C|SetCurrentActionList _wb_mainui _output_get)
  (Default|ShowDesiredList _wb_mainui "CurrentActionList"))

(fn PromptingAction
  (params (KeyPressed :type String))
  (bind _wb_mainui (Variables|Widgets|GetWB_MainUI))
  (bind _wb_mainui_2 (Variables|Widgets|GetWB_MainUI))
  (bind _infantrylist (Variables|/Game/TD2020/Widgets/HUDs/WB_MainUI.WB_MainUI_C|GetInfantryList _wb_mainui_2))
  (LocalVariables|SetKey KeyPressed)
  (Utilities|IsValid _wb_mainui
    (:Is%20Valid
      (Utilities|IsValid _infantrylist
        (:Is%20Valid
          (switch name (Default|GetListShown _wb_mainui)
            (:BuildingList
              (Default|CheckShortcuts (Variables|/Game/TD2020/Widgets/HUDs/WB_MainUI.WB_MainUI_C|GetBuildingList _wb_mainui_2) (LocalVariables|GetKey)))
            (:InfantryList
              (Default|CheckShortcuts _infantrylist (LocalVariables|GetKey)))
            (:ActionList
              (Default|CheckShortcuts (Variables|/Game/TD2020/Widgets/HUDs/WB_MainUI.WB_MainUI_C|GetActionList (Variables|Widgets|GetWB_MainUI)) (LocalVariables|GetKey)))))))))

(fn SelectActors
  (params (Actors :type Array%20of%20Actor%20Object%20References))
  (Default|SelectActors (Variables|Widgets|GetWB_MainUI) Actors)
  (for _array_element Actors
    (Selection|SelectActor _array_element)))

(fn ExitPressedF
  (if (not (Variables|Camera|GetPauseScreenShown?))
    (UserInterface|Viewport|AddtoViewport (Variables|Widgets|GetWB_Pause) 0)
    (Input|SetInputModeUIOnly (Game|GetPlayerController 0) (Variables|Widgets|GetWB_Pause) "LockAlways") ; disables our keyboard functions
    (Variables|Camera|SetDisableCamNav true)
    (Widget|SetIsEnabled (Variables|Widgets|GetWB_MainUI) false) ; disable creating buildings
    (Variables|Camera|SetPauseScreenShown? true)))

(fn CreateReferences
  (Variables|References|SetGS_MyGS (.AsGS%20My%20GS (Utilities|Casting|CastToGS_MyGS (Game|GetGameState))))
  (Variables|References|SetPlayerController (.AsPC%20Gameplay%20PC (Utilities|Casting|CastToPC_GameplayPC (Game|GetPlayerController 0))))
  (bind _returnvalue (Game|SpawnActorfromClass "/Game/TD2020/Blueprints/Buildings/Special/ConstructionManager_BP.ConstructionManager_BP_C" (Math|Transform|MakeTransform "0, 0, 0" "0, 0, 0" (Variables|Construction|GetActorScaleFactor)) "AlwaysSpawn" (Variables|References|GetPlayerController) (Variables|References|GetGS_MyGS) (Variables|References|GetPlayerController) self 0))
  (Variables|References|SetConstructionManagerRef _returnvalue)
  (bind _returnvalue_2 (Game|SpawnActorfromClass "/Game/TD2020/Blueprints/Buildings/Special/GhostBuilding_BP.GhostBuilding_BP_C" (Math|Transform|MakeTransform "0, 0, 0" "0, 0, 0" (Variables|Construction|GetActorScaleFactor)) "AlwaysSpawn" (Variables|References|GetPlayerController) (Variables|References|GetPlayerController) 0))
  (Variables|References|SetGhostBuildingRef _returnvalue_2))

(fn AddRally
  (params (Location :type Vector :default "0, 0, 0") (Action :type String) (Actor :type Actor%20Object%20Reference))
  (return 0))

(fn GetComponents
  (return 0 0 0 0 0 0 0 0 0 0 0 0))

(fn GetListName
  (return "None"))

(fn GetRallies
  (return "0, 0, 0" 0 0))

(fn GetTeamName
  (return (Utilities|String|ToString(Name) (.TeamName (Utilities|Struct|BreakPlayerInfo_Struct (Variables|Default|GetPlayerInfo))))))

(fn ImNotSelected
  (params (InPawn :type Pawn%20Master%20Commander%20Object%20Reference))
  (return 0))

(fn ImSelected
  (params (InPawn :type Pawn%20Master%20Commander%20Object%20Reference))
  (return 0))

(fn RemoveRallies
  (return 0))

(fn RMBHit
  (params (InCommander :type Actor%20Object%20Reference))
  (return 0))

(fn SetCalendar
  (params (Date :type Array%20of%20Integers))
  (return false))

(fn SetClock
  (params (Time :type Array%20of%20Integers))
  (return false))

(fn SetTeamName
  (params (TeamName :type String))
  (Utilities|Struct|SetmembersinPlayerInfo_Struct (Variables|Default|GetPlayerInfo) (Utilities|String|StringToName TeamName))
  (return 0))