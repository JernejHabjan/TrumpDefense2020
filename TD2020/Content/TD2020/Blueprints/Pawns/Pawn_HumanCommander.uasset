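; Human faction commander pawn that specializes a parent commander with the Humans cursor and building menu.
; On BeginPlay it runs the parent logic, then sets the default hardware cursor to the Humans texture.
; Its CreateWidgets override calls the parent, creates the Human building list widget with itself as commander, plugs it into the main UI and initializes its buttons.
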(event EventBeginPlay
  ;[1 1 1] Begin play
  (|CallParentFunction)
  (bind _output_get (Variables|Default|SetCursorName "TD2020/Textures/Cursors/HumansCursor"))
  (Class|WidgetBlueprintLibrary|SetHardwareCursor "Default" _output_get))

(fn ConstructionScript
  (|CallParentFunction))

(fn CreateWidgets
  (|CallParentFunction)
  (bind _returnvalue (UserInterface|CreateWidget "/Game/TD2020/Widgets/HUDs/HumanWidgets/WB_Human_BuildingList.WB_Human_BuildingList_C" (Game|GetPlayerController 0) self (Utilities|Name|MakeLiteralName "BuildingList")))
  (bind _output_get (Variables|Default|SetWB_BuildingList _returnvalue))
  (bind _output_get_2 (Variables|/Game/TD2020/Widgets/HUDs/WB_MainUI.WB_MainUI_C|SetBuildingList (Variables|Default|GetWB_MainUI) _output_get))
  (Default|InitButtons _output_get_2)
  (return 0))