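; Loading-screen pawn that possesses itself on BeginPlay and streams the initial sublevels while showing progress through the game instance's loading widget.
; A self-calling LoopBack event issues latent, hidden level loads one by one with a delay, updating the text and progress bar.
; It then reveals the sublevels and removes the widget, with optional timeline camera fades and particle slow-motion.
; Holding left mouse gates camera panning.
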(event Custom|LoopBack
  (bind _sublevellistinitial (Variables|Default|GetSubLevelListInitial))
  (bind _howmanychunkshaveloaded (Variables|Default|GetHowManyChunksHaveLoaded))
  (bind _mygameinstanceref (Variables|Default|GetMyGameInstanceRef))
  (bind _output (Utilities|Array|Get(acopy) _sublevellistinitial _howmanychunkshaveloaded))
  (bind _loadingscreenwb (Variables|/Game/TD2020/Blueprints/Logics/GI_MyGI.GI_MyGI_C|GetLoadingScreenWB _mygameinstanceref))
  ;[1 1 1] Loading screen progress bar
  (if (not (Variables|Default|GetDoneWithLoadingLoop))
    (if (>= (Variables|Default|GetHowManyChunksHaveLoaded) (Utilities|Array|Length (Variables|Default|GetSubLevelListInitial)))
      (Variables|Default|SetDoneWithLoadingLoop true)
      (CallFunction|LoopBack)
      (else
        (Default|SetDisplayText (Variables|Default|GetMyGameInstanceRef) _output)
        (Game|LoadStreamLevel(byName) _output false) ; you cant use it in loop
        (Utilities|FlowControl|Delay (Variables|Default|GetDelayEachLoop))
        (Math|Integer|IncrementInt (Variables|Default|GetHowManyChunksHaveLoaded)
          (:%20%20
            (Utilities|IsValid _loadingscreenwb
              (:Is%20Valid
                (Progress|SetPercent (Variables|/Game/TD2020/Widgets/Loading/WB_LoadingScreen.WB_LoadingScreen_C|GetLoadProgress _loadingscreenwb) (/ (Math|Conversions|ToFloat(Integer) (Variables|Default|GetHowManyChunksHaveLoaded)) (Math|Conversions|ToFloat(Integer) (Utilities|Array|Length (Variables|Default|GetSubLevelListInitial))))))
              (:Is%20Not%20Valid
                _))
            (CallFunction|LoopBack)))))
    (else
      ;[1 1 1] Camer a fade out with some slow mo on the particles (not necessary)
      (if (Variables|Default|GetUseTransitions)
        (bind (_direction _camera_fade _slow_particles) (Timeline|Timeline_0 Play)
          (:Update
            (Class|PlayerCameraManager|SetManualCameraFade :self (Game|GetPlayerCameraManager 0) :InFadeAmount (- 1.0 _camera_fade))
            (Variables|/Script/Engine.Actor|SetCustomTimeDilation self _slow_particles))
          (:Finished
            ;[1 1 1] When all is done, make the sublevels visible
            (for _array_element (Variables|Default|GetSubLevelListInitial) :!label _label
              (Variables|/Script/Engine.LevelStreaming|SetbShouldBeVisible (Class|GameplayStatics|GetStreamingLevel _array_element) true))
            ;[1 1 1] Remove loading widget
            (Default|LoadingScreenDestruction (Variables|Default|GetMyGameInstanceRef))
            ;[1 1 1] Transition the camera from black to white and unload the transition level
            (if (Variables|Default|GetUseTransitions)
              (bind _camera_fade_2 (Timeline|Timeline_1 Play)
                (:Update
                  (Class|PlayerCameraManager|SetManualCameraFade :self (Game|GetPlayerCameraManager 0) :InFadeAmount _camera_fade_2))
                (:Finished)))))
        (else
          (goto _label))))))

(event EventBeginPlay
  (bind _sublevellistinitial (Variables|Default|GetSubLevelListInitial))
  (bind _howmanychunkshaveloaded (Variables|Default|GetHowManyChunksHaveLoaded))
  (bind _output (Utilities|Array|Get(acopy) _sublevellistinitial _howmanychunkshaveloaded))
  ;[1 1 1] Set
  (Variables|Default|SetMyGameInstanceRef (.AsGI%20My%20GI (Utilities|Casting|CastToGI_MyGI (Game|GetGameInstance))))
  (Variables|Default|SetPlayerController (.AsPC%20Gameplay%20PC (Utilities|Casting|CastToPC_GameplayPC (Game|GetPlayerController 0))))
  ;[1 1 1] Posses new pawn
  (Pawn|Possess (Variables|Default|GetPlayerController) self)
  ;[1 1 1] Trigger loading screen widget
  (Default|ShowLoadingScreen (Variables|Default|GetMyGameInstanceRef))
  ;[1 1 1] Loading screen progress bar
  (if (>= (Variables|Default|GetHowManyChunksHaveLoaded) (Utilities|Array|Length (Variables|Default|GetSubLevelListInitial)))
    (Variables|Default|SetDoneWithLoadingLoop true)
    (CallFunction|LoopBack)
    (else
      (Default|SetDisplayText (Variables|Default|GetMyGameInstanceRef) _output)
      (Game|LoadStreamLevel(byName) _output false) ; you cant use it in loop
      (Utilities|FlowControl|Delay (Variables|Default|GetDelayEachLoop))
      (Math|Integer|IncrementInt (Variables|Default|GetHowManyChunksHaveLoaded)
        (:%20%20
          (Utilities|IsValid (Variables|/Game/TD2020/Blueprints/Logics/GI_MyGI.GI_MyGI_C|GetLoadingScreenWB (Variables|Default|GetMyGameInstanceRef))
            (:Is%20Valid
              (Progress|SetPercent (Variables|/Game/TD2020/Widgets/Loading/WB_LoadingScreen.WB_LoadingScreen_C|GetLoadProgress (Variables|/Game/TD2020/Blueprints/Logics/GI_MyGI.GI_MyGI_C|GetLoadingScreenWB (Variables|Default|GetMyGameInstanceRef))) (/ (Math|Conversions|ToFloat(Integer) (Variables|Default|GetHowManyChunksHaveLoaded)) (Math|Conversions|ToFloat(Integer) (Utilities|Array|Length (Variables|Default|GetSubLevelListInitial))))))
            (:Is%20Not%20Valid
              _))
          (CallFunction|LoopBack))))))

(event Input|AxisEvents|InputAxisCameraY
  (params (AxisValue :type Float%20%28single-precision%29))
  ;[1 1 1] Rotate X and Y
  (Utilities|FlowControl|Gate true
    (:Exit
      (CallFunction|Pan self -9e+01 9e+01 (Variables|Default|GetSensitivity) (stale Input|AxisEvents|InputAxisCameraX AxisValue) AxisValue))))

(event Input|AxisEvents|InputAxisCameraX
  (params (AxisValue :type Float%20%28single-precision%29))
  ;[1 1 1] Rotate X and Y
  (Utilities|FlowControl|Gate true
    (:Exit
      (CallFunction|Pan self -9e+01 9e+01 (Variables|Default|GetSensitivity) AxisValue (stale Input|AxisEvents|InputAxisCameraY AxisValue)))))

(event Input|MouseEvents|LeftMouseButton
  (params (Key :type Key%20Structure))
  ;[1 1 1] Rotate X and Y
  (:Pressed
    (Utilities|FlowControl|Gate true) ; enters at Open
  )
  (:Released
    (Utilities|FlowControl|Gate true) ; enters at Close
  ))

(fn ConstructionScript)