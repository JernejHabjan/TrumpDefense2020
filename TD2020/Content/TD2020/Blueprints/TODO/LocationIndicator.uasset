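; LocationIndicator is an actor that keeps itself resting on the surface below or above it, apparently as a location marker.
; On BeginPlay it starts a looping 0.1-second timer that calls FindGround, rather than using Tick.
; FindGround line-traces the Visibility channel along the actor's up axis, from far above to far below.
; It then sets only the actor's Z to the hit location, without checking whether the trace hit.
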(event EventBeginPlay
  (Utilities|Time|SetTimerbyFunctionName 0 "FindGround" 0.1 true))

(event EventActorBeginOverlap
  (params (OtherActor :type Actor%20Object%20Reference)))

(event EventTick
  (params (DeltaSeconds :type Float%20%28single-precision%29)))

(fn ConstructionScript)

(fn FindGround
  (bind _returnvalue (Transformation|GetActorLocation))
  (bind _returnvalue_2 (Transformation|GetActorUpVector))
  (bind _returnvalue_3 (Transformation|GetActorLocation))
  (bind _returnvalue_4 (* _returnvalue_2 1e+04))
  (bind _returnvalue_5 (+ _returnvalue _returnvalue_4))
  (bind _outhit (Collision|LineTraceByChannel _returnvalue_5 (+ _returnvalue_5 (* _returnvalue_2 -2e+04)) "TraceTypeQuery1" false 0 "None"))
  (Transformation|SetActorLocation (Math|Vector|MakeVector (.x _returnvalue_3) (.y _returnvalue_3) (.z (.Location (Collision|BreakHitResult _outhit)))) false false))