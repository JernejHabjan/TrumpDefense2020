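; Spline-driven medieval wall actor that builds its wall meshes in the construction script.
; Each point-to-point segment gets a spline mesh using the spline's tangents, with configurable mesh, forward axis and collision.
; Toggles select one of four start and end cap options, though EndMesh4On places EndMesh3.
; Optional split meshes repeat at a set distance along the spline; they and the start cap are re-added on every segment pass.
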(fn ConstructionScript
  (bind _spline (Variables|Default|GetSpline))
  (bind _splitdistance (Variables|Default|GetSplitDistance))
  (bind _spline_2 (Variables|Default|GetSpline))
  (bind _firstindex (Variables|Default|GetFirstIndex))
  (bind _returnvalue (Spline|GetLocationatSplinePoint _spline_2 _firstindex "Local"))
  (bind _returnvalue_2 (Math|Transform|MakeTransform _returnvalue))
  (for _index (range (Variables|Default|GetFirstIndex) (- (Spline|GetNumberOfSplinePoints (Variables|Default|GetSpline)) 2))
    (if (Variables|StartMesh|GetStartMeshOn?)
      ;[1 1 1] Start Mesh
      (if (Variables|StartMesh|GetStartMesh1%20On?)
        (bind _returnvalue_3 (AddComponent|AddStaticMeshComponent false _returnvalue_2))
        (Components|StaticMesh|SetStaticMesh _returnvalue_3 (Variables|StartMesh|GetStartMesh1))
        ;[1 1 1] Make Spline
        (bind _returnvalue_4 (AddComponent|AddSplineMeshComponent false :!label _label))
        (Components|StaticMesh|SetStaticMesh _returnvalue_4 (Variables|Components|GetStatic%20Mesh))
        (SplineMesh|SetForwardAxis _returnvalue_4 (Variables|Default|GetForward%20Axis) true)
        (Transformation|AttachComponentToComponent _returnvalue_4 (Variables|Default|GetSpline) "None" "KeepRelative" "KeepRelative" "KeepRelative" true)
        (SplineMesh|SetStartandEnd _returnvalue_4 (Spline|GetLocationatSplinePoint _spline _index "Local") (Spline|GetTangentatSplinePoint _spline _index "Local") (Spline|GetLocationatSplinePoint _spline (+ _index 1) "Local") (Spline|GetTangentatSplinePoint _spline (+ _index 1) "Local") true :!class /Script/Engine.SplineMeshComponent)
        ;[1 1 1] Place Split Mesh
        (Collision|SetCollisionEnabled _returnvalue_4 (Variables|Default|GetCollision))
        (for _index_2 (range 0 (.ReturnValue (Math|Float|Division(WholeandRemainder) (Spline|GetSplineLength (Variables|Default|GetSpline)) _splitdistance)))
          (if (Variables|Default|GetSplitDistanceON?)
            (bind _returnvalue_5 (AddComponent|AddStaticMeshComponent false (Math|Transform|MakeTransform (Spline|GetLocationatDistanceAlongSpline (Variables|Default|GetSpline) (* _index_2 _splitdistance) "Local"))))
            (Components|StaticMesh|SetStaticMesh _returnvalue_5 (Variables|Default|GetSplitPointMesh))))
        (elif (Variables|StartMesh|GetStartMesh2%20On?)
          (bind _returnvalue_6 (AddComponent|AddStaticMeshComponent false _returnvalue_2))
          (Components|StaticMesh|SetStaticMesh _returnvalue_6 (Variables|StartMesh|GetStartMesh2))
          (goto _label)
          (elif (Variables|StartMesh|GetStartMesh3%20On?)
            (bind _returnvalue_7 (AddComponent|AddStaticMeshComponent false _returnvalue_2))
            (Components|StaticMesh|SetStaticMesh _returnvalue_7 (Variables|StartMesh|GetStartMesh3))
            (goto _label)
            (elif (Variables|StartMesh|GetStartMesh4%20On?)
              (bind _returnvalue_8 (AddComponent|AddStaticMeshComponent false _returnvalue_2))
              (Components|StaticMesh|SetStaticMesh _returnvalue_8 (Variables|StartMesh|GetStartMesh4))
              (goto _label)))))
      (else
        (goto _label))))
  (if (Variables|EndMesh|GetEndMeshOn?)
    ;[1 1 1] End Mesh
    (if (Variables|EndMesh|GetEndMesh1%20On?)
      (bind _returnvalue_9 (AddComponent|AddStaticMeshComponent false (Math|Transform|MakeTransform (Spline|GetLocationatSplinePoint (Variables|Default|GetSpline) _index "Local"))))
      (Components|StaticMesh|SetStaticMesh _returnvalue_9 (Variables|EndMesh|GetEndMesh1))
      (elif (Variables|EndMesh|GetEndMesh2%20On?)
        (bind _returnvalue_10 (AddComponent|AddStaticMeshComponent false (Math|Transform|MakeTransform (Spline|GetLocationatSplinePoint (Variables|Default|GetSpline) _index "Local"))))
        (Components|StaticMesh|SetStaticMesh _returnvalue_10 (Variables|EndMesh|GetEndMesh2))
        (elif (Variables|EndMesh|GetEndMesh3%20On?)
          (bind _returnvalue_11 (AddComponent|AddStaticMeshComponent false (Math|Transform|MakeTransform (Spline|GetLocationatSplinePoint (Variables|Default|GetSpline) _index "Local"))))
          (Components|StaticMesh|SetStaticMesh _returnvalue_11 (Variables|EndMesh|GetEndMesh3))
          (elif (Variables|EndMesh|GetEndMesh4%20On?)
            (bind _returnvalue_12 (AddComponent|AddStaticMeshComponent false (Math|Transform|MakeTransform (Spline|GetLocationatSplinePoint (Variables|Default|GetSpline) _index "Local"))))
            (Components|StaticMesh|SetStaticMesh _returnvalue_12 (Variables|EndMesh|GetEndMesh3))))))
    (else
      (bind _returnvalue_13 (AddComponent|AddSplineMeshComponent false))
      (Components|StaticMesh|SetStaticMesh _returnvalue_13 (Variables|Components|GetStatic%20Mesh))
      (SplineMesh|SetForwardAxis _returnvalue_13 (Variables|Default|GetForward%20Axis) true)
      (Transformation|AttachComponentToComponent _returnvalue_13 (Variables|Default|GetSpline) "None" "KeepRelative" "KeepRelative" "KeepRelative" true)
      (SplineMesh|SetStartandEnd _returnvalue_13 (Spline|GetLocationatSplinePoint _spline _index "Local") (Spline|GetTangentatSplinePoint _spline _index "Local") (Spline|GetLocationatSplinePoint _spline (+ _index 1) "Local") (Spline|GetTangentatSplinePoint _spline (+ _index 1) "Local") true :!class /Script/Engine.SplineMeshComponent)
      (Collision|SetCollisionEnabled _returnvalue_13 (Variables|Default|GetCollision))
      (for _index_3 (range 0 (.ReturnValue (Math|Float|Division(WholeandRemainder) (Spline|GetSplineLength (Variables|Default|GetSpline)) _splitdistance)))
        (if (Variables|Default|GetSplitDistanceON?)
          (bind _returnvalue_14 (AddComponent|AddStaticMeshComponent false (Math|Transform|MakeTransform (Spline|GetLocationatDistanceAlongSpline (Variables|Default|GetSpline) (* _index_3 _splitdistance) "Local"))))
          (Components|StaticMesh|SetStaticMesh _returnvalue_14 (Variables|Default|GetSplitPointMesh)))))))