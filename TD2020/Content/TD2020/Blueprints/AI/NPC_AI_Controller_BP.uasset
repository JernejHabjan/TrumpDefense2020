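; AI controller for NPCs that runs their behavior tree and manages stamina, housing, movement and combat sight.
; Looping timers scaled to the GameState's time unit deplete or regain stamina, re-evaluated on sleep switches and game-speed changes.
; Perception updates report sighted actors to the MasterCombat pawn and blackboard, with a gate and retriggerable delay postponing disengagement after losing the enemy.
; Helper functions find and assign residences, leave buildings or construction shifts, and issue moves.
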(event OnPerceptionUpdated(AIPerception)
  (params (UpdatedActors :type Array%20of%20Actor%20Object%20References))
  (bind _returnvalue (Pawn|GetControlledPawn))
  (bind _asmaster_combat (Utilities|Casting|CastToMasterCombat (Pawn|GetControlledPawn)))
  (Utilities|IsValid (Variables|/Game/TD2020/Blueprints/AI/Characters/MasterCombat.MasterCombat_C|GetEnemyToFight _asmaster_combat)
    (:Is%20Valid
      (bind _info (Class|AIPerceptionComponent|GetActorsPerception (Variables|Default|GetAIPerception) (Variables|/Game/TD2020/Blueprints/AI/Characters/MasterCombat.MasterCombat_C|GetEnemyToFight _asmaster_combat))) ; is the enemy to fight still in my perceptions?
      (AI|Components|Blackboard|SetValueasBool (AI|GetBlackboard _asmaster_combat) (Variables|/Game/TD2020/Blueprints/AI/Characters/MasterCombat.MasterCombat_C|GetBBK_EnemyVisible _asmaster_combat) (.bSuccessfullySensed (Utilities|Struct|BreakAIStimulus (Utilities|Array|Get(acopy) (.LastSensedStimuli (Utilities|Struct|BreakActorPerceptionBlueprintInfo _info))))))
      (if (.bSuccessfullySensed (Utilities|Struct|BreakAIStimulus (Utilities|Array|Get(acopy) (.LastSensedStimuli (Utilities|Struct|BreakActorPerceptionBlueprintInfo _info)))))
        (Default|OnEnemySight _asmaster_combat (Variables|/Game/TD2020/Blueprints/AI/Characters/MasterCombat.MasterCombat_C|GetEnemyToFight _asmaster_combat))
        (goto _label Close)
        (else
          (Utilities|FlowControl|Sequence
            (:then_0
              (goto _label Open))
            (:then_1
              (Utilities|FlowControl|RetriggerableDelay 3.0) ; if we find enemy again this will retrigger back to 3 seconds
              (Utilities|FlowControl|Gate true :!label _label
                (:Exit
                  (Default|Disengage _asmaster_combat))))))))
    (:Is%20Not%20Valid
      (bind _array_element (Utilities|Array|ForEachLoopwithBreak UpdatedActors :!label _label_2) ; searching for first enemy in our sight if we dont have set enemy yet
        (:LoopBody
          (Utilities|Casting|CastToPawn_MasterCommander _array_element ; can check for building here if attacking buildings ?
            (:CastFailed
              (Utilities|IsValid _array_element
                (:Is%20Valid
                  (if (not (== _array_element _returnvalue))
                    (if (Utilities|Name|Equal(Name) (Utilities|Array|Get(acopy) (Variables|/Script/Engine.Actor|GetTags _returnvalue)) (Utilities|Array|Get(acopy) (Variables|/Script/Engine.Actor|GetTags _array_element))) ; if our teams are same
                      _
                      (else
                        _))
                    (bind _asmaster_combat_2 (Utilities|Casting|CastToMasterCombat (Pawn|GetControlledPawn)))
                    (Default|OnEnemySight _asmaster_combat_2 _array_element)
                    (goto _label_2 Break)))))))))))

(event Custom|UpdateTime
  (params (NewTime :type Float%20%28single-precision%29))
  ;[1 1 1] Begin Play
  (Variables|Default|SetTimeUnit NewTime)
  (if (Class|KismetSystemLibrary|IsTimerPausedHandle (Variables|Default|GetDepleteStaminaHandle_0)) ; if is paused deplete handle
    (bind _returnvalue (Utilities|Time|SetTimerbyFunctionName 0 "RegainStamina_0" (/ (Variables|Default|GetTimeUnit) 6e+01) true))
    (Variables|Default|SetRegainStaminaHandle_0 _returnvalue)
    (else
      (bind _returnvalue_2 (Utilities|Time|SetTimerbyFunctionName 0 "DepleteStamina_0" (/ (Variables|Default|GetTimeUnit) 6e+01) true))
      (Variables|Default|SetDepleteStaminaHandle_0 _returnvalue_2))))

(event Custom|SwitchSleep
  (bind _timeunit (Variables|Default|GetTimeUnit))
  (bind _returnvalue (/ _timeunit 6e+01))
  ;[1 1 1] Begin Play
  (if (Class|KismetSystemLibrary|IsTimerPausedHandle (Variables|Default|GetDepleteStaminaHandle_0)) ; if is paused deplete handle
    (bind _returnvalue_2 (Utilities|Time|SetTimerbyFunctionName 0 "RegainStamina_0" _returnvalue true))
    (Variables|Default|SetRegainStaminaHandle_0 _returnvalue_2)
    (else
      (bind _returnvalue_3 (Utilities|Time|SetTimerbyFunctionName 0 "DepleteStamina_0" _returnvalue true))
      (Variables|Default|SetDepleteStaminaHandle_0 _returnvalue_3))))

(event EventBeginPlay
  ;[1 1 1] Begin Play
  (Variables|References|SetCameraControllerRef (.AsPC%20Gameplay%20PC (Utilities|Casting|CastToPC_GameplayPC (Game|GetPlayerController 0))))
  (bind _output_get (Variables|References|SetGameState (.AsGS%20My%20GS (Utilities|Casting|CastToGS_MyGS (Game|GetGameState)))))
  (Variables|Default|SetTimeUnit (Class|MyGameState|GetCurrentTimeUnit _output_get)) ; default time unit
  (EventDispatchers|BindEventtoUpdateGameSpeed (Variables|References|GetGameState) (EventDispatchers|CreateEvent :!event Custom|UpdateTime))
  (if (Class|KismetSystemLibrary|IsTimerPausedHandle (Variables|Default|GetDepleteStaminaHandle_0)) ; if is paused deplete handle
    (bind _returnvalue (Utilities|Time|SetTimerbyFunctionName 0 "RegainStamina_0" (/ (Variables|Default|GetTimeUnit) 6e+01) true))
    (Variables|Default|SetRegainStaminaHandle_0 _returnvalue)
    (else
      (bind _returnvalue_2 (Utilities|Time|SetTimerbyFunctionName 0 "DepleteStamina_0" (/ (Variables|Default|GetTimeUnit) 6e+01) true))
      (Variables|Default|SetDepleteStaminaHandle_0 _returnvalue_2))))

(event EventSwitchBehaviorTree
  (params (InBehaviorTree :type Behavior%20Tree%20Object%20Reference))
  (AI|RunBehaviorTree InBehaviorTree))

(event EventOnPossess
  (params (PossessedPawn :type Pawn%20Object%20Reference))
  ;[1 1 1] On Posses
  (bind _as0_base (Utilities|Casting|CastTo0_Base PossessedPawn))
  (bind _output_get (Variables|References|SetNPCRef _as0_base))
  (if (== (Utilities|GetClass _output_get) "/Game/TD2020/Blueprints/AI/Characters/NPC_BP.NPC_BP_C")
    (AI|RunBehaviorTree "/Game/TD2020/Blueprints/AI/BTs/NPC_BT.NPC_BT") ; USE BEHAVIOR TREE
  ))

(event EventMoveto
  (params (InLocation :type Vector :default "0, 0, 0"))
  (CallFunction|MovetobyController InLocation))

(fn ConstructionScript)

(fn CheckforHousing0
  (bind _array_element (Utilities|Array|ForEachLoopwithBreak (Variables|/Game/TD2020/Blueprints/Logics/GS_MyGS.GS_MyGS_C|GetResidentialBuildings_0 (Variables|References|GetGameState)) :!label _label)
    (:LoopBody
      (bind _asresidential_master_bp (Utilities|Casting|CastToResidentialMaster_BP _array_element)) ; if it succeeds - its residential
      (bind _accepted (Default|ApplyforResidency _asresidential_master_bp))
      (if _accepted
        (LocalVariables|SetFoundHousing_LOCAL true)
        (LocalVariables|SetResidents_LOCAL _asresidential_master_bp) ; breaks at first found
        (goto _label Break)
        (else
          (LocalVariables|SetFoundHousing_LOCAL false)
          (LocalVariables|SetResidents_LOCAL 0))))
    (:Completed
      (return (LocalVariables|GetFoundHousing_LOCAL) (LocalVariables|GetResidents_LOCAL)))))

(fn SetNewHouse0
  (params (House :type Actor%20Object%20Reference))
  (Variables|/Game/TD2020/Blueprints/AI/Characters/0_Base.0_Base_C|SetProfile (Variables|References|GetNPCRef) (Utilities|Struct|MakeNPCProfile_Struct_02 (.Name (Utilities|Struct|BreakNPCProfile_Struct_02 (Variables|/Game/TD2020/Blueprints/AI/Characters/0_Base.0_Base_C|GetProfile (Variables|References|GetNPCRef)))) (.Sex (Utilities|Struct|BreakNPCProfile_Struct_02 (Variables|/Game/TD2020/Blueprints/AI/Characters/0_Base.0_Base_C|GetProfile (Variables|References|GetNPCRef)))) (.OccupationType (Utilities|Struct|BreakNPCProfile_Struct_02 (Variables|/Game/TD2020/Blueprints/AI/Characters/0_Base.0_Base_C|GetProfile (Variables|References|GetNPCRef)))) (.PlaceOfEmployment (Utilities|Struct|BreakNPCProfile_Struct_02 (Variables|/Game/TD2020/Blueprints/AI/Characters/0_Base.0_Base_C|GetProfile (Variables|References|GetNPCRef)))) (.AsResidential%20Master%20BP (Utilities|Casting|CastToResidentialMaster_BP House)) "/Game/TD2020/Textures/StaticMeshes/RTSBuildings/Apartments.Apartments"))
  (return))

(fn RegainStamina0
  (Variables|/Game/TD2020/Blueprints/AI/Characters/NPC_BP.NPC_BP_C|SetStamina (Variables|References|GetNPCRef) (Math|Float|Clamp(Float) (+ (Variables|/Game/TD2020/Blueprints/AI/Characters/NPC_BP.NPC_BP_C|GetStamina (Variables|References|GetNPCRef)) (/ (Variables|Default|GetStaminaHourlyRegeneration_0) 6e+01)) 0.0 1e+02))
  (return))

(fn DepleteStamina0
  (Variables|/Game/TD2020/Blueprints/AI/Characters/NPC_BP.NPC_BP_C|SetStamina (Variables|References|GetNPCRef) (Math|Float|Clamp(Float) (- (Variables|/Game/TD2020/Blueprints/AI/Characters/NPC_BP.NPC_BP_C|GetStamina (Variables|References|GetNPCRef)) (/ (Variables|Default|GetStaminaHourlyDeduction) 6e+01)) 0.0 1e+02))
  (return))

(fn LeaveLocation0
  (params (Location :type Object%20Object%20Reference))
  (bind _asconstruction_proxy_bp (Utilities|Casting|CastToConstructionProxy_BP Location)
    (:then
      (bind _exitedbuilding (Default|LeaveShift _asconstruction_proxy_bp (.AsNPC%20BP (Utilities|Casting|CastToNPC_BP (Variables|References|GetNPCRef)))))
      (return _exitedbuilding))
    (:CastFailed
      (bind _asbuilding_master_bp (Utilities|Casting|CastToBuildingMaster_BP Location) ; everything aside of constr. proxy should be in building master
        (:then
          (bind _exitedbuilding_2 (Default|ExitBuilding _asbuilding_master_bp (.AsNPC%20BP (Utilities|Casting|CastToNPC_BP (Variables|References|GetNPCRef)))))
          (return _exitedbuilding_2))
        (:CastFailed
          ;[1 1 1] Add Other Checks for different types of building / jobs
          (return false))))))

(fn MovetoManually
  (params (InLocation :type Vector))
  (AI|Navigation|MovetoLocation InLocation 1.5e+02 true true false))

(fn MovetobyController
  (params (InLocation :type Vector))
  (AI|Navigation|MovetoLocation InLocation 1e+01 true true false))

(fn ImNotSelected
  (params (InPawn :type Pawn%20Master%20Commander%20Object%20Reference))
  (return 0))

(fn ImSelected
  (params (InPawn :type Pawn%20Master%20Commander%20Object%20Reference))
  (return 0))