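; NPC character for the TD2020 game that can take building jobs, obey commander move orders and act as a follow target for the player.
; If unemployed, it applies to a random available job from GameState, becoming builder or miner from the building's construction and resource-drain components, weighted when both exist.
; A gate controls snapping the player pawn to the NPC's location.
; Helpers set the blackboard busy flag and fill mesh arrays.
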(event Custom|OpenFollowGate
  (bind _returnvalue (Transformation|GetActorLocation))
  ;[1 1 1] EventTick
  (Utilities|FlowControl|Gate true ; enters at Open
    (:Exit
      (Transformation|SetActorLocation (Game|Player|GetPlayerPawn 0) (Math|Vector|MakeVector (.x _returnvalue) (.y _returnvalue) (.z (Transformation|GetActorLocation))) false false))))

(event Custom|CloseFollowGate
  (bind _returnvalue (Transformation|GetActorLocation))
  ;[1 1 1] EventTick
  (Utilities|FlowControl|Gate true ; enters at Close
    (:Exit
      (Transformation|SetActorLocation (Game|Player|GetPlayerPawn 0) (Math|Vector|MakeVector (.x _returnvalue) (.y _returnvalue) (.z (Transformation|GetActorLocation))) false false))))

(event Custom|DisplayHUD
  (params (Actor :type Actor%20Object%20Reference) (Bypass :type Boolean)))

(event EventBeginPlay
  (|CallParentFunction)
  (Variables|Default|SetIsBusy "IsBusy"))

(event EventUpdateWalkSpeed
  (params (TimeUnit :type Float%20%28single-precision%29))
  (|CallParentFunction TimeUnit))

(event EventMovebyCommander
  (params (InLocation :type Vector :default "0, 0, 0"))
  (CallFunction|MovetoLocation InLocation))

(event EventTick
  (params (DeltaSeconds :type Float%20%28single-precision%29))
  ;[1 1 1] EventTick
  (|CallParentFunction DeltaSeconds))

(fn ConstructionScript
  (|CallParentFunction))

(fn SetIsBusy
  (params (IsBusy :type Boolean))
  (AI|Components|Blackboard|SetValueasBool (AI|GetBlackboard (Variables|Default|GetAIController)) (Variables|Default|GetIsBusy) IsBusy)
  (return))

(fn CheckforEmployment
  (if (Utilities|Enum|Equal(Enum) (.OccupationType (Utilities|Struct|BreakNPCProfile_Struct_02 (Variables|Default|GetProfile))) "NewEnumerator0")
    (bind (_isjobavaliable _jobsavaliable) (Default|GetAvaliableJobs (Variables|Default|GetGameState)))
    (LocalVariables|SetAvaliableJobs_LOCAL _jobsavaliable)
    (if _isjobavaliable ; if job is avaliable
      (bind _building (Default|HireEmployee (Utilities|Array|Get(acopy) (LocalVariables|GetAvaliableJobs_LOCAL) (Math|Random|RandomIntegerinRange 0 (- (Utilities|Array|Length (LocalVariables|GetAvaliableJobs_LOCAL)) 1))) self))
      (LocalVariables|SetBuilding_LOCAL _building)
      (if true ; if i was hired
        (bind (_rtsselectable _rtsowner _rtsattackable _rtshealth _rtsproductioncost _rtsproduction _rtsconstructionsite _rtsportrait _td2020construction _td2020vacancy _rtsresourcedrain) (Default|GetComponents (LocalVariables|GetBuilding_LOCAL)))
        (Utilities|IsValid _td2020construction
          (:Is%20Valid
            (Utilities|IsValid _rtsresourcedrain ; if both valid -choose with percentage, else set as builder
              (:Is%20Valid
                (if (Math|Random|RandomBoolwithWeight (Variables|Default|GetPercentageBuilders))
                  (Utilities|Struct|SetmembersinNPCProfile_Struct_02 (Variables|Default|GetProfile) "NewEnumerator1" (.BuildingReference (Utilities|Struct|BreakBuilding_STRUCT_02 (Variables|/Game/TD2020/Blueprints/Buildings/BuildingMaster_BP.BuildingMaster_BP_C|GetBuildingStruct_BP (LocalVariables|GetBuilding_LOCAL)))) :!label _label)
                  (else
                    (Utilities|IsValid _rtsresourcedrain :!label _label_2 ; if only this one valid - set as miner
                      (:Is%20Valid
                        (Utilities|Struct|SetmembersinNPCProfile_Struct_02 (Variables|Default|GetProfile) "NewEnumerator2" (.BuildingReference (Utilities|Struct|BreakBuilding_STRUCT_02 (Variables|/Game/TD2020/Blueprints/Buildings/BuildingMaster_BP.BuildingMaster_BP_C|GetBuildingStruct_BP (LocalVariables|GetBuilding_LOCAL))))))))))
              (:Is%20Not%20Valid
                (goto _label))))
          (:Is%20Not%20Valid
            (goto _label_2)))
        (Development|PrintString (Utilities|String|Append "Hired in >" (Utilities|GetClassDisplayName (Utilities|GetClass (LocalVariables|GetBuilding_LOCAL))) "< as >" (Utilities|String|EnumtoString (.OccupationType (Utilities|Struct|BreakNPCProfile_Struct_02 (Variables|Default|GetProfile)))) "<") true true "(R=0.030566,G=1.000000,B=0.000000,A=1.000000)")
        (return true)
        (else
          (return false)))
      (else
        (return false) ; false
      ))
    (else
      (return false) ; something wrong - return false
    )))

(fn SetMeshes
  (bind _malemesh_0_1 (Variables|Default|GetMaleMesh_0_1))
  (bind _femalemesh_0_1 (Variables|Default|GetFemaleMesh_0_1))
  (Utilities|FlowControl|Sequence
    (:then_0
      (Utilities|Array|Add _malemesh_0_1 "/Game/TD2020/Meshes/SkeletalMeshes/Male_01.Male_01"))
    (:then_1
      (Utilities|Array|Add _malemesh_0_1 "/Game/TD2020/Meshes/SkeletalMeshes/Female_02.Female_02"))
    (:then_2
      (Utilities|FlowControl|Sequence
        (:then_0
          (Utilities|Array|Add _femalemesh_0_1 "/Game/TD2020/Meshes/SkeletalMeshes/Female_01.Female_01"))
        (:then_1
          (Utilities|Array|Add _femalemesh_0_1 "/Game/TD2020/Meshes/SkeletalMeshes/Female_02.Female_02"))
        (:then_2
          (return 0))))))