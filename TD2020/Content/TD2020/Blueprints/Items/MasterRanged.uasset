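; Base ranged weapon that fires arcing projectiles at the enemy targeted by its owner's TD2020AttackInfantryComponent.
; ROS_FireWeapon calls Fire, which acts only while the DamageIssuer stands still with a valid enemy.
; Fire pitches the spawn box by ballistic formulas for level or uneven ground, adding slight random pitch and yaw spread.
; It then spawns the projectile and re-arms itself by timer at FireRate, so the loop ends once conditions fail.
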(event Custom|ROS_FireWeapon
  (CallFunction|Fire))

(event EventBeginPlay
  (|CallParentFunction) ; This node is disabled and will not be called.\nDrag off pins to build functionality.
)

(event Collision|EventActorBeginOverlap
  (params (OtherActor :type Actor%20Object%20Reference))
  (|CallParentFunction OtherActor) ; This node is disabled and will not be called.\nDrag off pins to build functionality.
)

(event EventTick
  (params (DeltaSeconds :type Float%20%28single-precision%29))
  (|CallParentFunction DeltaSeconds) ; This node is disabled and will not be called.\nDrag off pins to build functionality.
)

(fn ConstructionScript
  (|CallParentFunction))

(fn Fire
  (bind _damageissuer (Variables|Default|GetDamageIssuer))
  (bind _gravity (LocalVariables|GetGravity))
  (bind _projectilespeedtemp (Variables|Default|GetProjectileSpeedTemp))
  (bind _projectilespawnbox (Variables|Default|GetProjectileSpawnBox))
  (bind _damageissuer_2 (Variables|Default|GetDamageIssuer))
  (bind _damageissuer_3 (Variables|Default|GetDamageIssuer))
  (bind _damageissuer_4 (Variables|Default|GetDamageIssuer))
  (bind _damageissuer_5 (Variables|Default|GetDamageIssuer))
  (bind _returnvalue (Transformation|GetActorRotation _damageissuer_3))
  (bind _returnvalue_2 (Actor|GetComponentbyClass _damageissuer "/Game/TD2020/Blueprints/Components/TD2020AttackInfantryComponent.TD2020AttackInfantryComponent_C"))
  (bind _returnvalue_3 (Transformation|GetActorRotation _damageissuer_4))
  (bind _returnvalue_4 (Transformation|GetWorldTransform _projectilespawnbox))
  (bind _returnvalue_5 (Math|Float|Square _projectilespeedtemp))
  (bind _returnvalue_6 (Transformation|GetActorLocation _damageissuer_5))
  (bind (_roll _pitch _yaw) (Math|Rotator|BreakRotator _returnvalue))
  (bind (_roll_2 _pitch_2 _yaw_2) (Math|Rotator|BreakRotator _returnvalue_3))
  (bind (_x _y) (Math|Vector|BreakVector _returnvalue_6))
  (bind _enemytofight (Variables|/Game/TD2020/Blueprints/Components/TD2020AttackComponent.TD2020AttackComponent_C|GetEnemyToFight _returnvalue_2))
  (bind _returnvalue_7 (Transformation|GetActorLocation _enemytofight))
  (bind _returnvalue_8 (Math|Vector2D|MakeVector2D _x _y))
  (bind _returnvalue_9 (- _returnvalue_6 _returnvalue_7))
  (bind (_x_2 _y_2) (Math|Vector|BreakVector _returnvalue_7))
  (bind _z (Math|Vector|BreakVector _returnvalue_9))
  (bind _returnvalue_10 (Math|Vector2D|MakeVector2D _x_2 _y_2))
  (bind _returnvalue_11 (- _returnvalue_10 _returnvalue_8))
  (bind _returnvalue_12 (Math|Vector2D|Vector2DLength _returnvalue_11))
  (bind _returnvalue_13 (* _returnvalue_12 _gravity))
  (Utilities|IsValid _damageissuer_2
    (:Is%20Valid
      (if (== (Math|Vector|VectorLength (Transformation|GetVelocity _damageissuer_2)) 0.0)
        (Utilities|IsValid _returnvalue_2
          (:Is%20Valid
            (Utilities|IsValid _enemytofight
              (:Is%20Valid
                (if (Math|Float|NearlyEqual(Float) _z 0.0 1e+01)
                  (Transformation|SetWorldRotation (Variables|Default|GetProjectileSpawnBox) (Math|Rotator|MakeRotator _roll_2 (+ (Class|KismetMathLibrary|DegAsin (Math|Float|Absolute(Float) (/ _returnvalue_13 (* _returnvalue_5 2.0)))) (Math|Conversions|ToFloat(Integer) (Math|Random|RandomIntegerinRange -1 1))) (+ _yaw_2 (Math|Conversions|ToFloat(Integer) (Math|Random|RandomIntegerinRange -1 1)))) false false)
                  (else
                    (Transformation|SetWorldRotation (Variables|Default|GetProjectileSpawnBox) (Math|Rotator|MakeRotator _roll (+ (Class|KismetMathLibrary|DegAtan (/ (- _returnvalue_5 (Math|Float|Sqrt (- (Math|Float|Square _returnvalue_5) (* (* (LocalVariables|GetGravity) -1.0) (+ (* (Math|Float|Square _returnvalue_12) (LocalVariables|GetGravity)) (* (* 2.0 _z) _returnvalue_5)))))) _returnvalue_13)) (Math|Conversions|ToFloat(Integer) (Math|Random|RandomIntegerinRange -1 1))) (+ _yaw (Math|Conversions|ToFloat(Integer) (Math|Random|RandomIntegerinRange -1 1)))) false false)))
                (Game|SpawnActorfromClass (Variables|Default|GetProjectileClass) (Math|Transform|MakeTransform (.location _returnvalue_4) (.rotation _returnvalue_4) "1,1,1") "Undefined" 0 (Variables|Default|GetDamageIssuer) 0)
                (Development|PrintString "SPAWNED PROJECTILEEE")
                (Utilities|Time|SetTimerbyFunctionName 0 "Fire" (Variables|Default|GetFireRate))))))))))