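; MasterProjectiles is a projectile that damages what it hits, spawns an impact effect and destroys itself.
; Startup configures movement speed and gravity and ignores the damage issuer while moving.
; Hits on body-tagged boxes apply damage after team and self checks, which are skipped if the issuer is invalid.
; The headshot multiplier is nested inside the body-tag check on the same tag index, so it appears unreachable.
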(event EventBeginPlay
  ;[1 1 1] Begin play
  (|CallParentFunction)
  (CallFunction|StartUp))

(event Collision|EventHit
  (params (MyComp :type Primitive%20Component%20Object%20Reference) (Other :type Actor%20Object%20Reference) (OtherComp :type Primitive%20Component%20Object%20Reference) (bSelfMoved :type Boolean) (HitLocation :type Vector :default "0, 0, 0") (HitNormal :type Vector :default "0, 0, 0") (NormalImpulse :type Vector :default "0, 0, 0") (Hit :type Hit%20Result%20Structure%20%28by%20ref%29))
  ;[1 1 1] Hit
  (CallFunction|ApplyDamagetoHitActor OtherComp Other HitLocation))

(fn ConstructionScript)

(fn Startup
  (bind _projectilemovement (Variables|Components|GetProjectileMovement))
  (|CallParentFunction)
  (Collision|IgnoreActorwhenMoving (Variables|Default|GetItemColision) (Variables|Default|GetDamageIssuer) true)
  (Actor|SetLifeSpan 0.0)
  (bind _output_get (Variables|/Script/Engine.ProjectileMovementComponent|SetInitialSpeed _projectilemovement (Variables|Default|GetInitialSpeed)))
  (Variables|/Script/Engine.ProjectileMovementComponent|SetMaxSpeed _projectilemovement _output_get)
  (Variables|/Script/Engine.ProjectileMovementComponent|SetProjectileGravityScale _projectilemovement (Variables|Default|GetGravityScale))
  (return 0))

(fn ApplyDamagetoHitActor
  (params (InHitBox :type Primitive%20Component%20Object%20Reference) (InHitActor :type Actor%20Object%20Reference) (InHitLocation :type Vector :default "0, 0, 0"))
  (|CallParentFunction InHitBox InHitActor InHitLocation)
  (bind _asbox_collision (Utilities|Casting|CastToBoxComponent InHitBox)
    (:then
      (if (Utilities|Name|Equal(Name) (Utilities|Array|Get(acopy) (Variables|/Script/Engine.ActorComponent|GetComponentTags _asbox_collision) 1) "BodyHitBox") ; didnt hit body hitbox
        (if (Utilities|Name|Equal(Name) (Utilities|Array|Get(acopy) (Variables|/Script/Engine.ActorComponent|GetComponentTags _asbox_collision) 1) "HeadHitBox") ; check for crit
          (Variables|Default|SetImpactDamage (* (Variables|Default|GetImpactDamage) (Variables|Default|GetCriticalValue))) ; critical hit
        )
        (Utilities|IsValid (Variables|Default|GetDamageIssuer)
          (:Is%20Valid
            (Utilities|IsValid InHitActor
              (:Is%20Valid
                (if (and (not (CallFunction|CheckTeams (Variables|Default|GetDamageIssuer) InHitActor)) (!= (Variables|Default|GetDamageIssuer) InHitActor))
                  (Game|Damage|ApplyDamage InHitActor (Variables|Default|GetImpactDamage) 0 (Variables|Default|GetDamageIssuer))))
              (:Is%20Not%20Valid
                _)))
          (:Is%20Not%20Valid
            (Game|Damage|ApplyDamage InHitActor (Variables|Default|GetImpactDamage) 0 0) ; fired from is invalid - we are dead when fired bulled - TODO - WHAT ABOUT TEAMMATES ????
          ))))
    (:CastFailed
      _))
  (Effects|SpawnEmitteratLocation (Variables|Default|GetImpactParticleEffect) InHitLocation)
  (Actor|DestroyActor) ; because this is projectile, it gets destroyed at the end
  (return 0))