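; Game State for TD2020 that runs the in-game clock and calendar and tracks buildings and resources.
; Outside the main menu, Tick advances Clockwork by a speed-scaled TimeUnit, derives time and date, and pushes both to the commander pawn's HUD.
; Buildings register as residential or occupational by component, feeding open-job queries, while resources toggle placement decals by proximity type.
; It also broadcasts speed changes and toggles settings and pause widgets.
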(event EventBeginPlay
  ;[1 1 1] Begin Play
  (if (.bSuccess (Utilities|Casting|CastToGM_MainMenu (Game|GetGameMode))) ; if we have main menu mode - we are in menu
    (Variables|Default|SetInMenu true)
    (else
      (Variables|Default|SetInMenu false)
      (Variables|References|SetControllerRef_0 (.AsPC%20Gameplay%20PC (Utilities|Casting|CastToPC_GameplayPC (Game|GetPlayerController 0))))
      (Variables|Default|SetClockwork (+ (Math|Conversions|ToFloat(Integer) (Variables|Default|GetHours)) (Math|Conversions|ToFloat(Integer) (Variables|Default|GetMinutes)) (Math|Conversions|ToFloat(Integer) (Variables|Default|GetSeconds))))
      (Variables|Default|SetGameDate (Utilities|Array|MakeArray (Variables|Default|GetDay) (Variables|Default|GetMonth) (Variables|Default|GetYear)))
      (bind _aspawn_master_commander (Utilities|Casting|CastToPawn_MasterCommander (Game|Player|GetPlayerPawn 0) :!label _label)
        (:then
          (Variables|Components|SetMainUIRef_0 (Variables|/Game/TD2020/Blueprints/Units/Commanders/Pawn_MasterCommander.Pawn_MasterCommander_C|GetWB_MainUI _aspawn_master_commander))
          (Variables|Default|SetTimeUnit (Variables|Default|GetDefaultGameSpeed)))
        (:CastFailed
          (Utilities|FlowControl|Delay 0.01)
          (goto _label))))))

(event EventTick
  (params (DeltaSeconds :type Float%20%28single-precision%29))
  ;[1 1 1] Tick
  (if (and (not (Variables|Default|GetInMenu)) (Utilities|IsValid (Variables|References|GetControllerRef_0)))
    (Variables|Default|SetClockwork (.ClockworkOut (Class|FunctionLibrary|SetClockwork DeltaSeconds (Variables|Default|GetTimeUnit) (Variables|Default|GetClockwork)))) ; remainder of 24
    (Variables|Default|SetDayTick (.DayTick (Class|FunctionLibrary|SetClockwork DeltaSeconds (Variables|Default|GetTimeUnit) (Variables|Default|GetClockwork))))
    (CallFunction|Clock)
    (CallFunction|Calendar)))

(event EventUpdateGameStateSpeed
  (params (Multiplier :type Float%20%28single-precision%29))
  ;[1 1 1] Update Game Speed
  (bind _output_get (Variables|Default|SetSpeedMultiplier Multiplier))
  (bind _output_get_2 (Variables|Default|SetTimeUnit (* _output_get (Variables|Default|GetDefaultGameSpeed))))
  (Default|CallUpdateGameSpeed _output_get_2))

(fn ConstructionScript)

(fn AddBuildingtoGame
  (params (Building :type Building%20Master%20BP%20Object%20Reference))
  (bind _output_get (LocalVariables|SetBuildingRef_LOCAL Building))
  (bind (_rtsselectable _rtsowner _rtsattackable _rtshealth _rtsproductioncost _rtsproduction _rtsconstructionsite _rtsportrait _td2020construction _td2020vacancy _rtsresourcedrain) (Default|GetComponents _output_get))
  (Utilities|IsValid _td2020vacancy
    (:Is%20Valid
      (Utilities|Array|AddUnique (Variables|Buildings|GetResidentialBuildings_0) (LocalVariables|GetBuildingRef_LOCAL)))
    (:Is%20Not%20Valid
      _))
  (if (or (Utilities|IsValid _td2020construction) (Utilities|IsValid _rtsresourcedrain))
    (Utilities|Array|AddUnique (Variables|Buildings|GetOccupationalBuildings_0) (LocalVariables|GetBuildingRef_LOCAL))))

(fn GetAvaliableJobs
  (bind _avaliablejoblocations_local (LocalVariables|GetAvaliableJobLocations_LOCAL))
  (bind _returnvalue (Utilities|Array|Length _avaliablejoblocations_local))
  (if (> (Utilities|Array|Length (Variables|Buildings|GetOccupationalBuildings_0)) 0)
    (for _array_element (Variables|Buildings|GetOccupationalBuildings_0)
      (Utilities|IsValid _array_element
        (:Is%20Valid
          (bind _output_get (LocalVariables|SetCurrentBuilding_LOCAL _array_element))
          (if (not (>= (.NumberOfOccupants (Default|GetOccupants _output_get)) (.MaxEmployees (Utilities|Struct|BreakBuilding_STRUCT_02 (Variables|/Game/TD2020/Blueprints/Buildings/BuildingMaster_BP.BuildingMaster_BP_C|GetBuildingStruct_BP (LocalVariables|GetCurrentBuilding_LOCAL)))))) ; if lesser than max
            (Utilities|Array|AddUnique (LocalVariables|GetAvaliableJobLocations_LOCAL) (LocalVariables|GetCurrentBuilding_LOCAL))))
        (:Is%20Not%20Valid
          (Utilities|Array|RemoveItem (Variables|Buildings|GetOccupationalBuildings_0) _array_element))))
    (Development|PrintString (Utilities|String|ToString(Integer) _returnvalue))
    (if (> _returnvalue 0) ; if its false - no avaliable buildings with jobs
      (return true (LocalVariables|GetAvaliableJobLocations_LOCAL))
      (else
        _)))
  (Development|PrintString "No Avaliable Jbs")
  (return false (LocalVariables|GetAvaliableJobLocations_LOCAL)))

(fn ShowProximity
  (params (ProximityType :type EProximityType_Enum%20Enum :default "None"))
  (LocalVariables|SetProximityType_LOCAL ProximityType)
  (if (> (Utilities|Array|Length (Variables|Default|GetResources_0)) 0)
    (for _array_element (Variables|Default|GetResources_0)
      (if (Utilities|Enum|Equal(Enum) (.ProximityType (Utilities|Struct|BreakResources_Struct (Variables|/Game/TD2020/Blueprints/Resources/Resource_ResourcesMaster.Resource_ResourcesMaster_C|GetResourceStruct _array_element))) (LocalVariables|GetProximityType_LOCAL))
        (Rendering|ToggleVisibility (Variables|/Game/TD2020/Blueprints/Resources/Resource_ResourcesMaster.Resource_ResourcesMaster_C|GetGoodPlacementDecal _array_element) false)
        (Utilities|Array|AddUnique (Variables|Default|GetVisibleResourceProximity_0) _array_element)))
    (return)
    (else
      (return))))

(fn AddResource
  (params (Resource :type Resource%20Resources%20Master%20Object%20Reference))
  (Utilities|Array|AddUnique (Variables|Default|GetResources_0) Resource)
  (return))

(fn GetCurrentTimeUnit
  (return (Variables|Default|GetTimeUnit)))

(fn HideProximity
  (for _array_element (Variables|Default|GetVisibleResourceProximity_0)
    (Rendering|ToggleVisibility (Variables|/Game/TD2020/Blueprints/Resources/Resource_ResourcesMaster.Resource_ResourcesMaster_C|GetGoodPlacementDecal _array_element) false))
  (Utilities|Array|Clear (Variables|Default|GetVisibleResourceProximity_0))
  (return true))

(fn Clock
  (bind _returnvalue (Game|Player|GetPlayerPawn 0))
  (bind _clockwork (Variables|Default|GetClockwork))
  (bind _returnvalue_2 (* _clockwork 3.6e+03))
  (bind _aspawn_master_commander (Utilities|Casting|CastToPawn_MasterCommander _returnvalue))
  (bind (_remainder _returnvalue_3) (Math|Float|Division(WholeandRemainder) _returnvalue_2 6e+01))
  (bind _returnvalue_4 (Math|Conversions|ToFloat(Integer) _returnvalue_3))
  (bind (_remainder_2 _returnvalue_5) (Math|Float|Division(WholeandRemainder) _returnvalue_4 6e+01))
  (Variables|Default|SetSeconds (Math|Float|Floor _remainder))
  (Variables|Default|SetMinutes (Math|Float|Floor _remainder_2))
  (Variables|Default|SetHours (Math|Float|Floor (.Remainder (Math|Float|Division(WholeandRemainder) (Math|Conversions|ToFloat(Integer) _returnvalue_5) 24.0))))
  (bind _output_get (Variables|Default|SetGameTime (Utilities|Array|MakeArray (Variables|Default|GetSeconds) (Variables|Default|GetMinutes) (Variables|Default|GetHours))))
  (Utilities|IsValid _aspawn_master_commander
    (:Is%20Valid
      (bind _success (Class|IHUD|SetClock(Message) (Variables|/Game/TD2020/Blueprints/Units/Commanders/Pawn_MasterCommander.Pawn_MasterCommander_C|GetWB_MainUI _aspawn_master_commander) _output_get)))
    (:Is%20Not%20Valid
      _))
  (return _success))

(fn Calendar
  (bind _returnvalue (Game|Player|GetPlayerPawn 0))
  (bind _aspawn_master_commander (Utilities|Casting|CastToPawn_MasterCommander _returnvalue))
  (bind _output_get (Variables|Default|SetDay (+ (Variables|Default|GetDayTick) (Variables|Default|GetDay))))
  (if (> _output_get (Class|KismetMathLibrary|DaysinMonth (Variables|Default|GetYear) (Variables|Default|GetMonth)))
    (Variables|Default|SetDay 1) ; we reached the end of the month
    (Math|Integer|IncrementInt (Variables|Default|GetMonth) ; increment month
      (:%20%20
        _)))
  (if (> (Variables|Default|GetMonth) 12)
    (Variables|Default|SetMonth 1)
    (Math|Integer|IncrementInt (Variables|Default|GetYear)
      (:%20%20
        _)))
  (bind _output_get_2 (Variables|Default|SetGameDate (Utilities|Array|MakeArray (Variables|Default|GetDay) (Variables|Default|GetMonth) (Variables|Default|GetYear))))
  (Utilities|IsValid _aspawn_master_commander
    (:Is%20Valid
      (bind _success (Class|IHUD|SetCalendar(Message) (Variables|/Game/TD2020/Blueprints/Units/Commanders/Pawn_MasterCommander.Pawn_MasterCommander_C|GetWB_MainUI _aspawn_master_commander) _output_get_2)) ; set HUD calendar
    )
    (:Is%20Not%20Valid
      _))
  (return _success))

(fn ToggleMenu
  (bind _returnvalue (Game|Player|GetPlayerPawn 0))
  (bind _mainmenu_widget (Variables|Default|GetMainMenu_Widget))
  (bind _aspawn_master_commander (Utilities|Casting|CastToPawn_MasterCommander _returnvalue))
  (bind _wb_pause (Variables|/Game/TD2020/Blueprints/Units/Commanders/Pawn_MasterCommander.Pawn_MasterCommander_C|GetWB_Pause _aspawn_master_commander))
  (Utilities|FlowControl|Sequence
    (:then_0
      (if (Variables|Menu|GetIsMenuShown) ; if is shown settings menu
        (Utilities|FlowControl|Sequence
          (:then_0
            ;[1 1 1] Remove main menu VBOX
            (Utilities|IsValid _mainmenu_widget
              (:Is%20Valid
                (Default|ToggleComponentVisibility _mainmenu_widget (Variables|/Game/TD2020/Widgets/MainMenu/WB_Main_MainMenu.WB_Main_MainMenu_C|GetMain_VBox _mainmenu_widget)))))
          (:then_1
            ;[1 1 1] Remove settings widget
            (Widget|RemovefromParent (Variables|Default|GetMenu))
            (Variables|Menu|SetIsMenuShown false)))
        (else
          ;[1 1 1] Create settings widget
          (bind _returnvalue_2 (UserInterface|CreateWidget "/Game/TD2020/Widgets/MainMenu/Settings/WTF-Settings-CompleteExample.WTF-Settings-CompleteExample_C" (Game|GetPlayerController 0)))
          (bind _output_get (Variables|Default|SetMenu _returnvalue_2))
          (UserInterface|Viewport|AddtoViewport _output_get 0)
          (Variables|Menu|SetIsMenuShown true))))
    (:then_1
      ;[1 1 1] Toggle visiblility of pause widget
      (Default|ToggleComponentVisibility _wb_pause (Variables|/Game/TD2020/Widgets/PauseMenu/WB_Pause.WB_Pause_C|GetPause_VBox _wb_pause)))))

(fn SetCalendar
  (params (Date :type Array%20of%20Integers))
  (return false))

(fn SetClock
  (params (Time :type Array%20of%20Integers))
  (return false))

(fn SetResources
  (params (InGold :type Float%20%28single-precision%29))
  (return false))