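; AI commander pawn for the computer side, standing in for a player when constructing buildings and producing units.
; On BeginPlay it spawns its own gameplay PlayerController and makes it its owner before running parent logic.
; Construct spawns actual buildings with itself as commander, while Spawn delegates unit production to the given building.
; Selection and command overrides are empty stubs, and the NPC spawn-and-move test in the event graph is disconnected.
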(event EventTick
  (params (DeltaSeconds :type Float%20%28single-precision%29))
  ;[1 1 1] Tick
)

(event EventBeginPlay
  ;[1 1 1] Begin play
  (bind _returnvalue (Game|SpawnActorfromClass "/Game/TD2020/Blueprints/Logics/PC_GameplayPC.PC_GameplayPC_C" (Math|Transform|MakeTransform "0, 0, 0") "AlwaysSpawn" 0 0))
  (bind _output_get (Variables|Default|SetPlayerController _returnvalue))
  (Actor|SetOwner _output_get)
  (|CallParentFunction))

(fn ConstructionScript
  (|CallParentFunction))

(fn SelectOur
  (return 0))

(fn SelectEnemy
  (return 0))

(fn SelectNeutral
  (return 0))

(fn IssueCommandOnto
  (return))

(fn Construct
  (params (ConstructionStruct :type Construction%20Struct%2002%20Structure))
  ;[1 1 1] For now ACTUAL
  (CallFunction|SpawnActualBuilding ConstructionStruct self))

(fn Spawn
  (params (Building :type Building%20Master%20BP%20Object%20Reference) (Class :type 0%20Base%20Class%20Reference))
  ;[1 1 1] TODO - AI spawns unit automatically - any unit from any building
  (Default|ToCommanderSpawnUnit Building Class))