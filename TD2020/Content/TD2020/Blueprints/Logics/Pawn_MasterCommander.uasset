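; Player commander pawn for an RTS, holding gold, team info and the current selection, and issuing build, spawn and unit orders.
; BeginPlay spawns the construction manager and ghost building, then requests initial buildings.
; ROS server events handle movement and rally queues directly, but route building and unit spawns through MC events gated to authority.
; Other functions drive selection, action-list UI, shortcuts and pausing, alongside leftover networking tests and stubs.
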(event Custom|ROS_AddRally
  (params (Condition :type Boolean) (Location :type Vector) (Action :type String) (Actor :type Actor%20Object%20Reference) (SelectedActors :type Array%20of%20Actor%20Object%20References))
  ;[1 0.1899 0] Add Rally - TODOOOOO
  (Commands|AddRallyCommand Condition Location Action Actor SelectedActors))

(event Custom|MC_SpawnActualBuilding
  (params (ConstructionStruct :type Construction%20Struct%2002%20Structure) (LocalCommander :type Pawn%20Master%20Commander%20Object%20Reference))
  ;[1 1 1] Spawn Actual Building
  (Networking|SwitchHasAuthority
    (:Authority
      (BuildingPlacement|SpawnActualBuilding ConstructionStruct LocalCommander))))

(event Custom|ROS_MoveSelectedUnitsTo
  (params (InUnits :type Array%20of%20Actor%20Object%20References) (InLocation :type Vector))
  ;[1 1 1] Move Units to
  (CallFunction|MoveSelectedUnitsto InUnits InLocation))

(event Custom|ROS_ActionQueue
  (params (Character :type 0%20Base%20Object%20Reference))
  (bind _returnvalue (AI|GetAIController Character))
  ;[1 1 1] ROS Action Queue
  (Utilities|IsValid _returnvalue
    (:Is%20Valid
      (bind _ascharacter_aicontroller (Utilities|Casting|CastToCharacterAIController _returnvalue))
      (Default|ActionQueue _ascharacter_aicontroller))))

(event Custom|ROS_SpawnProxyBuilding
  (params (ConstructionStruct :type Construction%20Struct%2002%20Structure) (Commander :type Pawn%20Master%20Commander%20Object%20Reference) (EntityStruct :type Entity%20Struct%20Structure))
  ;[1 1 1] Spawn Proxy Building
  (CallFunction|MCSpawnProxyBuilding ConstructionStruct Commander EntityStruct))

(event Custom|ROS_RemoveRallies
  (params (Target :type Actor%20Object%20Reference))
  ;[1 0.1899 0] Add Rally - TODOOOOO
  (Class|ITD2020|RemoveRallies(Message) Target))

(event Custom|ROS_SpawnActualBuilding
  (params (ConstructionStruct :type Construction%20Struct%2002%20Structure) (LocalCommander :type Pawn%20Master%20Commander%20Object%20Reference))
  ;[1 1 1] Spawn Actual Building
  (CallFunction|MCSpawnActualBuilding ConstructionStruct LocalCommander))

(event Custom|MC_SpawnProxyBuilding
  (params (ConstructionStruct :type Construction%20Struct%2002%20Structure) (Commander :type Pawn%20Master%20Commander%20Object%20Reference) (EntityStruct :type Entity%20Struct%20Structure))
  ;[1 1 1] Spawn Proxy Building
  (Networking|SwitchHasAuthority
    (:Authority
      (BuildingPlacement|SpawnProxyBuilding ConstructionStruct Commander EntityStruct))))

(event Custom|ROS_MoveUnitTo
  (params (Actor :type Actor%20Object%20Reference) (InLocation :type Vector))
  ;[1 1 1] Move Units to
  (CallFunction|MoveUnitto Actor InLocation))

(event Custom|ROS_SpawnUnit
  (params (InUnit :type 0%20Base%20Class%20Reference) (InSpawnPoint :type Transform) (InCommander :type Pawn%20Object%20Reference) (InSpawnFlagLocation :type Vector))
  ;[1 1 1] Spawn unit - spawn them on server - because player controller is only on server - dont multicast
  (CallFunction|MCSpawnUnit InUnit InSpawnPoint InCommander InSpawnFlagLocation))

(event Custom|EOS_CreateWidgets
  ;[1 0.214 0] TODO TRANSFET THIS IN PLAYER CONTROLELR
  ;;[1 1 1] Create widgets
  (CallFunction|CreateWidgets))

(event Custom|MC_SpawnUnit
  (params (InUnit :type 0%20Base%20Class%20Reference) (InSpawnPoint :type Transform) (InCommander :type Pawn%20Object%20Reference) (InSpawnFlagLocation :type Vector))
  ;[1 1 1] Spawn unit - spawn them on server - because player controller is only on server - dont multicast
  (Networking|SwitchHasAuthority
    (:Authority
      (UnitSpawning|SpawnUnit InUnit InSpawnPoint InCommander InSpawnFlagLocation))))

(event EventBeginPlay
  ;[1 1 1] Begin Play
  (CallFunction|CreateReferences)
  (Class|RTSOwnerComponent|SetPlayerOwner (Variables|Default|GetRTSOwner) (.AsController (Utilities|Casting|CastToController (Components|GetOwner))))
  (Default|SpawnInitialBuildings (Variables|References|GetConstructionManagerRef)) ; If you want something to spawn for both players on start - spawn from construction manager for example
)

(event Custom|pr
  (params (InString :type String))
  ;[1 1 1] EXAMPLES
  (Development|PrintString InString true true "(R=1.000000,G=0.736534,B=0.115012,A=1.000000)" 222.0))

(event Custom|mcast
  (params (SpawnTransform :type Transform) (ControllerRef_BP :type PC%20Gameplay%20PC%20Object%20Reference))
  ;[1 1 1] EXAMPLES
  ;;[0.1153 0.8196 1] Spawn example
  (Game|SpawnActorfromClass "/Game/TD2020/tempCube.tempCube_C" SpawnTransform "Undefined" 0 0)
  (Game|SpawnActorfromClass "/Game/TD2020/Blueprints/Buildings/AllBuildings/HumanBarracks.HumanBarracks_C" SpawnTransform "Undefined" 0 0 5e+01 (.AsPawn%20Master%20Commander (Utilities|Casting|CastToPawn_MasterCommander (Pawn|GetControlledPawn ControllerRef_BP))) 0))

(event Custom|srver
  (params (SpawnTransform :type Transform) (ControllerRef_BP :type PC%20Gameplay%20PC%20Object%20Reference))
  ;[1 1 1] EXAMPLES
  ;;[0.1153 0.8196 1] Spawn example
  (CallFunction|Mcast SpawnTransform ControllerRef_BP))

(event Input|KeyboardEvents|X
  (params (Key :type Key%20Structure))
  ;[1 1 1] EXAMPLES
  ;;[0.1153 0.8196 1] Spawn example
  (:Pressed
    (CallFunction|Srver (Transformation|GetActorTransform) (.AsPC%20Gameplay%20PC (Utilities|Casting|CastToPC_GameplayPC (Game|GetPlayerController 0))))))

(fn ConstructionScript
  (Variables|Gold|SetGold 2e+04) ; to avoid crashes
)

(fn IsMoving
  (params (AxisX :type Float%20%28single-precision%29) (AxisY :type Float%20%28single-precision%29))
  (return (or (> (Math|Float|Absolute(Float) AxisX) 0.0) (> (Math|Float|Absolute(Float) AxisY) 0.0))))

(fn SetNPCSpawnPoint
  (bind _returnvalue (Game|GetPlayerController 0))
  (bind _aspc_gameplay_pc (Utilities|Casting|CastToPC_GameplayPC _returnvalue))
  (bind _location (CallFunction|SetCursorWorldPosition _aspc_gameplay_pc 1e+04))
  (Variables|Camera|SetCursorWorldPosition (Math|Vector|MakeVector (.x _location) (.y _location) (+ (.z _location) 1e+02)))
  (return (Math|Transform|MakeTransform (Variables|Camera|GetCursorWorldPosition) "0, 0, 0" (Variables|Construction|GetActorScaleFactor))))

(fn SaveGame
  (bind _returnvalue (SaveGame|DoesSaveGameExist "PlayerSave"))
  (if _returnvalue
    (bind _returnvalue_2 (SaveGame|LoadGamefromSlot "PlayerSave"))
    (bind _output_get (Variables|SaveGame|SetSaverSubClass _returnvalue_2)) ; Puts all info from load game into saver subclass
    (bind _assg_player_save_game (Utilities|Casting|CastToSG_PlayerSaveGame _output_get))
    (bind _result (Math|Integer|IncrementInt (Variables|/Game/TD2020/Blueprints/Logics/SG_PlayerSaveGame.SG_PlayerSaveGame_C|GetNumberOfClicks _assg_player_save_game))
      (:%20%20
        (SaveGame|SaveGametoSlot (Variables|SaveGame|GetSaverSubClass) "PlayerSave")
        (Development|PrintString (Utilities|String|ToString(Integer) _result))))
    (else
      (bind _returnvalue_3 (SaveGame|CreateSaveGameObject "/Game/TD2020/Blueprints/Logics/SG_PlayerSaveGame.SG_PlayerSaveGame_C"))
      (bind _output_get_2 (Variables|SaveGame|SetSaverSubClass _returnvalue_3)) ; creates save game and puts it into saver subclass
      (bind _assg_player_save_game_2 (Utilities|Casting|CastToSG_PlayerSaveGame _output_get_2))
      (Math|Integer|IncrementInt (Variables|/Game/TD2020/Blueprints/Logics/SG_PlayerSaveGame.SG_PlayerSaveGame_C|GetNumberOfClicks _assg_player_save_game_2)
        (:%20%20
          (SaveGame|SaveGametoSlot (Variables|SaveGame|GetSaverSubClass) "PlayerSave")
          (Development|PrintString (Utilities|String|ToString(Integer) (Variables|/Game/TD2020/Blueprints/Logics/SG_PlayerSaveGame.SG_PlayerSaveGame_C|GetNumberOfClicks _assg_player_save_game_2))))))))

(fn SpawnUnit
  (params (InUnit :type 0%20Base%20Class%20Reference) (InSpawnPoint :type Transform) (InCommander :type Pawn%20Object%20Reference) (InSpawnFlagLocation :type Vector))
  (bind _randomlocation (Class|NavigationSystem|GetRandomPointinNavigableRadius InSpawnFlagLocation 3e+02))
  (bind _aspawn_master_commander (Utilities|Casting|CastToPawn_MasterCommander InCommander))
  (bind (_x _y _z) (Math|Vector|BreakVector _randomlocation))
  (bind _returnvalue (Game|SpawnActorfromClass InUnit InSpawnPoint "AdjustIfPossibleButAlwaysSpawn" 0 (.AsGS%20My%20GS (Utilities|Casting|CastToGS_MyGS (Game|GetGameState))) _aspawn_master_commander (Utilities|Struct|MakeEntity_Struct (Utilities|String|ToString(Name) (.TeamName (Utilities|Struct|BreakPlayerInfo (Variables|Pawn_MasterCommander_C|GetPlayerInfo _aspawn_master_commander)))) "EntityName" 50 50 "/Game/TD2020/Textures/StaticMeshes/RTSBuildings/Apartments.Apartments") 0))
  (Pawn|SpawnDefaultController _returnvalue)
  (Class|ITD2020|MovebyCommander(Message) _returnvalue (Math|Vector|MakeVector _x _y (+ _z 1e+02))))

(fn MoveSelectedUnitsto
  (params (InUnits :type Array%20of%20Actor%20Object%20References) (InLocation :type Vector))
  (for _array_element InUnits
    (Class|ITD2020|MovebyCommander(Message) _array_element (.RandomLocation (Class|NavigationSystem|GetRandomPointinNavigableRadius InLocation (* (Utilities|Array|Length InUnits) 2e+01))))))

(fn ManageGold
  (params (InGold :type Float%20%28single-precision%29))
  (Variables|/Game/TD2020/Widgets/HUDs/WB_MainUI.WB_MainUI_C|SetGoldText (.AsWB%20Main%20UI (Utilities|Casting|CastToWB_MainUI (Variables|Widgets|GetWB_MainUI))) (Utilities|Text|ToText(Float) (+ InGold (Variables|Gold|GetGold)) "HalfToEven"))
  (bind _output_get (Variables|Gold|SetGold (+ InGold (Variables|Gold|GetGold))))
  (return _output_get))

(fn SpawnActualBuilding
  (params (ConstructionStruct :type Construction%20Struct%2002%20Structure) (LocalCommander :type Pawn%20Master%20Commander%20Object%20Reference))
  (bind (_buildingclass _proxyclass _transform _displaymesh _goldcost) (Utilities|Struct|BreakConstruction_Struct_02 ConstructionStruct))
  (Game|SpawnActorfromClass _buildingclass _transform "Undefined" 0 0 _goldcost LocalCommander 0))

(fn SpawnProxyBuilding
  (params (ConstructionStruct :type Construction%20Struct%2002%20Structure) (Commander :type Pawn%20Master%20Commander%20Object%20Reference) (EntityStruct :type Entity%20Struct%20Structure))
  (bind (_buildingclass _proxyclass _transform _displaymesh _goldcost) (Utilities|Struct|BreakConstruction_Struct_02 ConstructionStruct))
  (bind _returnvalue (Game|SpawnActorfromClass _proxyclass _transform "Undefined" 0 _displaymesh _goldcost Commander EntityStruct 0))
  (Default|ProxyStart (Variables|References|GetConstructionManagerRef) _returnvalue ConstructionStruct))

(fn CreateWidgets
  (return 0))

(fn MoveUnitto
  (params (Actor :type Actor%20Object%20Reference) (InLocation :type Vector))
  (Class|ITD2020|MovebyCommander(Message) Actor (.RandomLocation (Class|NavigationSystem|GetRandomPointinNavigableRadius InLocation 5e+01))))

(fn SelectActor
  (params (Actor :type Actor%20Object%20Reference))
  (bind _rtsselectable (Class|ITD2020|GetComponents(Message) Actor))
  (Utilities|IsValid _rtsselectable
    (:Is%20Valid
      (Class|RTSSelectableComponent|SelectActor _rtsselectable)
      (Utilities|Casting|CastTo0_Base Actor
        (:then
          (Variables|Selection|SetSelectedAnyNPCS? true))
        (:CastFailed
          _))
      (if (not (Utilities|Array|ContainsItem (Variables|Selection|GetCurrentSelectedActors) Actor))
        (Utilities|Array|Add (Variables|Selection|GetCurrentSelectedActors) Actor)
        (Class|ITD2020|ImSelected(Message) Actor self)))))

(fn DeselectActor
  (params (Actor :type Actor%20Object%20Reference) (MultipleDeselect? :type Boolean))
  (bind _wb_mainui (Variables|Widgets|GetWB_MainUI))
  (bind _aswb_main_ui (Utilities|Casting|CastToWB_MainUI _wb_mainui))
  (if (Utilities|Array|ContainsItem (Variables|Selection|GetCurrentSelectedActors) Actor) ; if false it, we may be deselecting enemy units
    (Utilities|Array|RemoveItem (Variables|Selection|GetCurrentSelectedActors) Actor))
  (Utilities|IsValid Actor
    (:Is%20Valid
      (Class|ITD2020|ImNotSelected(Message) Actor self))
    (:Is%20Not%20Valid
      _))
  (Default|SwapSelectedActorWidget _aswb_main_ui) ; clear profile pic and data
  (Default|RemovefromSelection (Variables|/Game/TD2020/Widgets/HUDs/WB_MainUI.WB_MainUI_C|GetWB_Selection _aswb_main_ui) Actor)
  ;[1 1 1] RTS
  (Utilities|IsValid Actor
    (:Is%20Valid
      (Class|RTSSelectableComponent|DeselectActor (Actor|GetComponentbyClass Actor "/Script/RTSPlugin.RTSSelectableComponent"))
      (if (not MultipleDeselect?) ; if running deselect all actors - call clear selections instead of running for loops in WB Selection widget for each actor
        ;[1 1 1] Selection tab - little icons
        (Default|RemovefromSelection (Variables|/Game/TD2020/Widgets/HUDs/WB_MainUI.WB_MainUI_C|GetWB_Selection (.AsWB%20Main%20UI (Utilities|Casting|CastToWB_MainUI (Variables|Widgets|GetWB_MainUI)))) Actor)))))

(fn AddRallyCommand
  (params (MultipleSelection? :type Boolean) (Location :type Vector) (Action :type String) (Actor :type Actor%20Object%20Reference) (SelectedActors :type Array%20of%20Actor%20Object%20References))
  (LocalVariables|SetLocation_LOCAL Location)
  (LocalVariables|SetAction_LOCAL Action)
  (LocalVariables|SetActor_LOCAL Actor)
  (if MultipleSelection? ; if holding shift while
    (for _array_element SelectedActors
      (bind _as0_base (Utilities|Casting|CastTo0_Base _array_element)
        (:then
          (Class|ITD2020|AddRally(Message) (Variables|/Game/TD2020/Blueprints/AI/Characters/0_Base.0_Base_C|GetAIController _as0_base) (LocalVariables|GetLocation_LOCAL) (LocalVariables|GetAction_LOCAL) (LocalVariables|GetActor_LOCAL)))
        (:CastFailed
          (Class|ITD2020|AddRally(Message) _array_element (LocalVariables|GetLocation_LOCAL) (LocalVariables|GetAction_LOCAL) (LocalVariables|GetActor_LOCAL)))))
    (else
      (for _array_element_2 SelectedActors
        (bind _as0_base_2 (Utilities|Casting|CastTo0_Base _array_element_2)
          (:then
            (Default|RemoveRallies (Variables|/Game/TD2020/Blueprints/AI/Characters/0_Base.0_Base_C|GetAIController _as0_base_2))
            (Class|ITD2020|AddRally(Message) (Variables|/Game/TD2020/Blueprints/AI/Characters/0_Base.0_Base_C|GetAIController _as0_base_2) (LocalVariables|GetLocation_LOCAL) (LocalVariables|GetAction_LOCAL) (LocalVariables|GetActor_LOCAL)))
          (:CastFailed
            (Class|ITD2020|RemoveRallies(Message) _array_element_2)
            (Class|ITD2020|AddRally(Message) _array_element_2 (LocalVariables|GetLocation_LOCAL) (LocalVariables|GetAction_LOCAL) (LocalVariables|GetActor_LOCAL))))))))

(fn StopCommand
  (for _array_element (Variables|Selection|GetCurrentSelectedActors)
    (bind _rallylocations (Class|ITD2020|GetRallies(Message) _array_element))
    (LocalVariables|SetTempRallyLocations _rallylocations)
    (if (Variables|Selection|GetMultipleSelection)
      (if (> (Utilities|Array|Length (LocalVariables|GetTempRallyLocations)) 1)
        (CallFunction|ROSAddRally (Variables|Selection|GetMultipleSelection) (Utilities|Array|Get(acopy) (LocalVariables|GetTempRallyLocations) (- (Utilities|Array|Length (LocalVariables|GetTempRallyLocations)) 1)) "Stop" 0 (Variables|Selection|GetCurrentSelectedActors))
        (else
          (CallFunction|ROSAddRally (Variables|Selection|GetMultipleSelection) (Transformation|GetActorLocation _array_element) "Stop" 0 (Variables|Selection|GetCurrentSelectedActors) :!label _label)))
      (else
        (goto _label)))))

(fn DeselectActors
  (params (Array :type Array%20of%20Actor%20Object%20References))
  (for _array_element Array
    (Selection|DeselectActor _array_element true))
  (Utilities|Array|Clear Array)
  ;[1 1 1] Selection tab - little icons
  (Default|ClearSelections (Variables|/Game/TD2020/Widgets/HUDs/WB_MainUI.WB_MainUI_C|GetWB_Selection (.AsWB%20Main%20UI (Utilities|Casting|CastToWB_MainUI (Variables|Widgets|GetWB_MainUI))))))

(fn SetCurrentActionList
  (params (Issuer :type Actor%20Object%20Reference) (Action :type Action%20Struct%20Structure) (ParentListName :type Name))
  (bind _wb_mainui (Variables|Widgets|GetWB_MainUI))
  (bind _aswb_main_ui (Utilities|Casting|CastToWB_MainUI _wb_mainui))
  (Variables|Default|SetCurrentExecutingAction (.ActionName (Utilities|Struct|BreakAction_Struct Action)))
  (bind _returnvalue (UserInterface|CreateWidget "/Game/TD2020/Widgets/HUDs/HumanWidgets/WB_CurrentActionList.WB_CurrentActionList_C" 0 self Issuer Action ParentListName))
  (bind _output_get (Variables|Default|SetWB_CurrentAction _returnvalue))
  (Variables|/Game/TD2020/Widgets/HUDs/WB_MainUI.WB_MainUI_C|SetCurrentActionList _aswb_main_ui _output_get)
  (Default|ShowDesiredList _aswb_main_ui "CurrentActionList"))

(fn PromptingAction
  (params (KeyPressed :type String))
  (bind _wb_mainui (Variables|Widgets|GetWB_MainUI))
  (bind _aswb_main_ui (Utilities|Casting|CastToWB_MainUI _wb_mainui))
  (LocalVariables|SetKey KeyPressed)
  (switch name (Default|GetListShown _aswb_main_ui)
    (:BuildingList
      (Default|CheckShortcuts (.AsWB%20Human%20Building%20List (Utilities|Casting|CastToWB_Human_BuildingList (Variables|/Game/TD2020/Widgets/HUDs/WB_MainUI.WB_MainUI_C|GetBuildingList _aswb_main_ui))) (LocalVariables|GetKey)))
    (:InfantryList
      (Default|CheckShortcuts (.AsWB%20Human%20Infantry%20List (Utilities|Casting|CastToWB_Human_InfantryList (Variables|/Game/TD2020/Widgets/HUDs/WB_MainUI.WB_MainUI_C|GetInfantryList _aswb_main_ui))) (LocalVariables|GetKey)))
    (:ActionList
      (Default|CheckShortcuts (.AsWB%20Action%20List (Utilities|Casting|CastToWB_ActionList (Variables|/Game/TD2020/Widgets/HUDs/WB_MainUI.WB_MainUI_C|GetActionList _aswb_main_ui))) (LocalVariables|GetKey)))))

(fn SelectActors
  (params (Actors :type Array%20of%20Actor%20Object%20References))
  (Default|SelectActors (.AsWB%20Main%20UI (Utilities|Casting|CastToWB_MainUI (Variables|Widgets|GetWB_MainUI))) Actors)
  (for _array_element Actors
    (Selection|SelectActor _array_element)))

(fn ExitPressedF
  (if (not (Variables|Camera|GetPauseScreenShown?))
    (UserInterface|Viewport|AddtoViewport (Variables|Widgets|GetWB_Pause) 0)
    (Input|SetInputModeUIOnly (Game|GetPlayerController 0) (Variables|Widgets|GetWB_Pause) "LockAlways") ; disables our keyboard functions
    (Variables|Camera|SetDisableCamNav true)
    (Widget|SetIsEnabled (Variables|Widgets|GetWB_MainUI) false) ; disable creating buildings
    (Variables|Camera|SetPauseScreenShown? true)
    (Game|SetGamePaused true)))

(fn CreateReferences
  (Variables|References|SetGS_MyGS (.AsGS%20My%20GS (Utilities|Casting|CastToGS_MyGS (Game|GetGameState))))
  (Variables|References|SetPlayerController (.AsPC%20Gameplay%20PC (Utilities|Casting|CastToPC_GameplayPC (Game|GetPlayerController 0))))
  (bind _returnvalue (Game|SpawnActorfromClass "/Game/TD2020/Blueprints/Buildings/Special/ConstructionManager_BP.ConstructionManager_BP_C" (Math|Transform|MakeTransform "0, 0, 0" "0, 0, 0" (Variables|Construction|GetActorScaleFactor)) "AlwaysSpawn" (Variables|References|GetPlayerController) (Variables|References|GetGS_MyGS) (Variables|References|GetPlayerController) self 0))
  (Variables|References|SetConstructionManagerRef _returnvalue)
  (bind _returnvalue_2 (Game|SpawnActorfromClass "/Game/TD2020/Blueprints/Buildings/Special/GhostBuilding_BP.GhostBuilding_BP_C" (Math|Transform|MakeTransform "0, 0, 0" "0, 0, 0" (Variables|Construction|GetActorScaleFactor)) "AlwaysSpawn" (Variables|References|GetPlayerController) (Variables|References|GetPlayerController) 0))
  (Variables|References|SetGhostBuildingRef _returnvalue_2))

(fn AddRally
  (params (Location :type Vector :default "0, 0, 0") (Action :type String) (Actor :type Actor%20Object%20Reference))
  (return 0))

(fn GetComponents
  (return 0 0 0 0 0 0 0 0 0 0 0 0))

(fn GetListName
  (return "None"))

(fn GetRallies
  (return "0, 0, 0" 0 0))

(fn GetTeamName
  (return (Utilities|String|ToString(Name) (.TeamName (Utilities|Struct|BreakPlayerInfo (Variables|Default|GetPlayerInfo))))))

(fn ImNotSelected
  (params (InPawn :type Pawn%20Master%20Commander%20Object%20Reference))
  (return 0))

(fn ImSelected
  (params (InPawn :type Pawn%20Master%20Commander%20Object%20Reference))
  (return 0))

(fn RemoveRallies
  (return 0))

(fn RMBHit
  (params (InCommander :type Actor%20Object%20Reference))
  (return 0))

(fn SetCalendar
  (params (Date :type Array%20of%20Integers))
  (return false))

(fn SetClock
  (params (Time :type Array%20of%20Integers))
  (return false))

(fn SetResources
  (params (InGold :type Float%20%28single-precision%29))
  (bind _output_get (Variables|Gold|SetGold InGold))
  (bind _success (Class|IHUD|SetResources(Message) (Variables|Widgets|GetWB_MainUI) _output_get))
  (return _success))

(fn SetTeamName
  (params (TeamName :type String))
  (Utilities|Struct|SetmembersinPlayerInfo (Variables|Default|GetPlayerInfo) (Utilities|String|StringToName TeamName))
  (return 0))