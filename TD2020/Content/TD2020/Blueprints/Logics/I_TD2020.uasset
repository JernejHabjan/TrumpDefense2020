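; I_TD2020 is a Blueprint interface that declares the shared messages of the TD2020 game logic for commander-driven selection, movement and building.
; Unit-facing calls cover selection notifications, move orders, behavior tree switching and right-click hits.
; Building calls cover completion, rally point management and linking builder lists to a commander and start-build buttons.
; Further functions expose components, team names and list names, with no gameplay logic in the interface itself.
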(fn MovebyCommander
  (params (InLocation :type Vector)))

(fn BuildingBuilt)

(fn SetCommander
  (params (InCommander :type Pawn%20Object%20Reference)))

(fn ImSelected
  (params (InPawn :type Pawn%20Master%20Commander%20Object%20Reference))
  (return 0))

(fn ImNotSelected
  (params (InPawn :type Pawn%20Master%20Commander%20Object%20Reference))
  (return 0))

(fn ListtoButtonStartBuild)

(fn SetCommanderBuilderList
  (params (InCommander :type Pawn%20Object%20Reference) (InBuilder :type Actor%20Object%20Reference) (InParentList :type User%20Widget%20Object%20Reference)))

(fn Moveto
  (params (InLocation :type Vector)))

(fn SwitchBehaviorTree
  (params (InBehaviorTree :type Behavior%20Tree%20Object%20Reference)))

(fn RMBHit
  (params (InCommander :type Actor%20Object%20Reference))
  (return 0))

(fn AddRally
  (params (Location :type Vector) (Action :type String) (Actor :type Actor%20Object%20Reference))
  (return 0))

(fn RemoveRallies
  (return 0))

(fn GetRallies
  (return "0, 0, 0" 0 0))

(fn GetComponents
  (return 0 0 0 0 0 0 0 0 0 0 0))

(fn SetTeamName
  (params (TeamName :type String))
  (return 0))

(fn GetTeamName
  (return ""))

(fn GetListName
  (return "None"))