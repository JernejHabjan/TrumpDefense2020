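; Gameplay player controller for a networked RTS that links the commander pawn, minimap, chat, resources and victory screen.
; On init it loads saved player settings, has the game mode respawn the player, then hooks up chat and team vision.
; Minimap clicks move the camera or issue move and attack rallies to selected units, while a timer refreshes scene captures.
; Chat fans out to every controller, and resource changes are relayed through server and client events.
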(event OnResourcesChanged(PlayerResourcesComponent)
  (params (ResourceType :type TD2020%20Resource%20Type%20Class%20Reference) (OldResourceAmount :type Float%20%28single-precision%29) (NewResourceAmount :type Float%20%28single-precision%29) (bSyncedFromServer :type Boolean))
  ;[1 1 1] On resources changed - sned message to all recievers
  (CallFunction|ROSResourcesChanged ResourceType OldResourceAmount NewResourceAmount))

(event Custom|ROC_Victory
  (params (WiningStatement :type Text))
  ;[1 1 1] Victory
  (bind _returnvalue (UserInterface|CreateWidget "/Game/TD2020/Widgets/PauseMenu/WB_GameFinish.WB_GameFinish_C" 0 WiningStatement))
  (UserInterface|Viewport|AddtoViewport _returnvalue 0)
  (Development|PrintString (Utilities|String|Append "victory shown on controller ->" (Utilities|GetObjectName self)) true true "(R=1.000000,G=0.901284,B=0.000000,A=1.000000)" 1e+01))

(event Custom|ROS_Move
  (params (Commander :type Pawn%20Master%20Commander%20Object%20Reference) (NewLocation :type Vector))
  (bind _returnvalue (Transformation|GetActorTransform Commander))
  ;[1 1 1] Ros move
  (if (Variables|/Game/TD2020/Blueprints/Pawns/Pawn_MasterCommander.Pawn_MasterCommander_C|GetAttackPressed? Commander)
    (Default|ROSAddRally Commander (Variables|/Game/TD2020/Blueprints/Pawns/Pawn_MasterCommander.Pawn_MasterCommander_C|GetMultipleSelection Commander) NewLocation "AttackMove" 0 (Variables|/Game/TD2020/Blueprints/Pawns/Pawn_MasterCommander.Pawn_MasterCommander_C|GetCurrentSelectedActors Commander))
    (else
      (bind _aspawn_master_player (Utilities|Casting|CastToPawn_MasterPlayer (Variables|Default|GetCommander)))
      (bind _outtransform (Default|CameraFollowSlope _aspawn_master_player (Math|Transform|MakeTransform NewLocation (.rotation _returnvalue) (.scale _returnvalue))))
      (Transformation|SetActorLocation Commander (.location _outtransform) false false))))

(event Custom|PassCharacterInfo
  (params (PlayerSettingsInfo :type Player%20Info%20Struct%20Structure))
  (bind _returnvalue (Game|GetGameInstance))
  (bind _asgi_my_gi (Utilities|Casting|CastToGI_MyGI _returnvalue))
  ;[1 1 1] Pass Character Info - Passes character info / calls setup chat window
  (Variables|Default|SetPlayerSettings PlayerSettingsInfo)
  (if (Variables|/Game/TD2020/Blueprints/Logics/GI_MyGI.GI_MyGI_C|GetStartedFromLobby? _asgi_my_gi)
    (Variables|Default|SetMaxPlayers (Variables|/Game/TD2020/Blueprints/Logics/GI_MyGI.GI_MyGI_C|GetMaxPlayers _asgi_my_gi))
    (else
      (Variables|Default|SetMaxPlayers 3)))
  (bind _asgm_gameplay_gm (Utilities|Casting|CastToGM_GameplayGM (Game|GetGameMode)))
  (Default|RespawnPlayer _asgm_gameplay_gm self (Variables|Default|GetPlayerSettings))
  (CallFunction|SetupChatWindow))

(event Custom|InitPC
  ;[1 1 1] Init PC - Loads player info and pass to serverside player controller
  (if (Pawn|IsLocalController)
    (Viewport|RemoveAllWidgets)
    (bind _playerinfo (CallFunction|LoadGame))
    (CallFunction|PassCharacterInfo _playerinfo)))

(event Custom|GetChatMessage
  (params (TextToSend :type Text))
  ;[1 1 1] Get Chat Message - Process and handle incoming chat / calls Update chat on the client
  (Variables|Default|SetSenderText TextToSend)
  (Variables|Default|SetSenderName (.MyPlayerName (Utilities|Struct|BreakPlayerInfo_Struct (Variables|Default|GetPlayerSettings))))
  (bind _asgm_gameplay_gm (Utilities|Casting|CastToGM_GameplayGM (Game|GetGameMode)))
  (if (== (Utilities|Array|Length (Variables|/Game/TD2020/Blueprints/Logics/GM_GameplayGM.GM_GameplayGM_C|GetAllPlayerControllers _asgm_gameplay_gm)) 0)
    (bind _outactors (Actor|GetAllActorsOfClass "PC_GameplayPC_C")) ; started from editor and didn't swap controllers so GM doesn't fill controlles on its own
    (Variables|/Game/TD2020/Blueprints/Logics/GM_GameplayGM.GM_GameplayGM_C|SetAllPlayerControllers _asgm_gameplay_gm _outactors))
  (for _array_element (Variables|/Game/TD2020/Blueprints/Logics/GM_GameplayGM.GM_GameplayGM_C|GetAllPlayerControllers _asgm_gameplay_gm)
    (bind _aspc_gameplay_pc (Utilities|Casting|CastToPC_GameplayPC _array_element))
    (CallFunction|UpdateChat _aspc_gameplay_pc (Variables|Default|GetSenderName) (Variables|Default|GetSenderText))))

(event Custom|PlayerResourcesActivated
  (bind _playerresourcescomponent (Variables|Default|GetPlayerResourcesComponent))
  ;[1 1 1] Resources component activated
  (for (_array_element _array_index) (Variables|/Script/TD2020.TD2020PlayerResourcesComponent|GetResourceTypes _playerresourcescomponent)
    (CallFunction|ROSResourcesChanged _array_element (Utilities|Array|Get(acopy) (Variables|/Script/TD2020.TD2020PlayerResourcesComponent|GetResourceAmounts _playerresourcescomponent) _array_index) (Utilities|Array|Get(acopy) (Variables|/Script/TD2020.TD2020PlayerResourcesComponent|GetResourceAmounts _playerresourcescomponent) _array_index))))

(event Custom|ROC_ResourcesChanged
  (params (ResourceType :type TD2020%20Resource%20Type%20Class%20Reference) (OldResourceAmount :type Float%20%28single-precision%29) (NewResourceAmount :type Float%20%28single-precision%29))
  ;[1 1 1] ROC Resources changed
  (Default|CallResourcesChanged ResourceType OldResourceAmount NewResourceAmount))

(event Custom|UpdateChat
  (params (SenderName :type Text) (SenderText :type Text))
  ;[1 1 1] Update Chat - Updates the client chat window
  (Default|UpdateChatWindow (Variables|/Game/TD2020/Widgets/HUDs/Chat/GameplayChat.GameplayChat_C|GetGameplayChat (Variables|Default|GetGameplayChatWB)) SenderName SenderText))

(event Custom|SetupChatWindow
  (bind _returnvalue (Class|TD2020PlayerController|GetTeamInfo))
  ;[1 1 1] Setup Chat window -Creates gameplay chat and adds it to the viewport
  (bind _aspawn_master_commander (Utilities|Casting|CastToPawn_MasterCommander (Game|Player|GetPlayerPawn 0)))
  (Utilities|IsValid (Variables|/Game/TD2020/Blueprints/Pawns/Pawn_MasterCommander.Pawn_MasterCommander_C|GetWB_MainUI _aspawn_master_commander)
    (:Is%20Valid
      (Variables|Default|SetGameplayChatWB (Variables|/Game/TD2020/Widgets/HUDs/WB_MainUI.WB_MainUI_C|GetGameplayChat (Variables|/Game/TD2020/Blueprints/Pawns/Pawn_MasterCommander.Pawn_MasterCommander_C|GetWB_MainUI _aspawn_master_commander)))
      ;[1 1 1] Initialize HUD.
      (Utilities|IsValid _returnvalue ; i guess dela čeprov client nima team infota
        (:Is%20Valid
          (bind _returnvalue_2 (Class|TD2020VisionInfo|GetVisionInfoforTeam (Variables|/Script/TD2020.TD2020TeamInfo|GetTeamIndex _returnvalue)))
          (Class|TD2020MinimapWidget|SetupVisionInfo (Variables|/Game/TD2020/Widgets/HUDs/WB_MainUI.WB_MainUI_C|GetTD2020SampleMinimapWidget (Variables|/Game/TD2020/Blueprints/Pawns/Pawn_MasterCommander.Pawn_MasterCommander_C|GetWB_MainUI (Variables|Default|GetCommander))) _returnvalue_2))))))

(event Custom|ROS_ResourcesChanged
  (params (ResourceType :type TD2020%20Resource%20Type%20Class%20Reference) (OldResourceAmount :type Float%20%28single-precision%29) (NewResourceAmount :type Float%20%28single-precision%29))
  ;[1 1 1] ROS resources changed
  (CallFunction|ROCResourcesChanged ResourceType OldResourceAmount NewResourceAmount))

(event EventOnVisionInfoAvailable
  (params (VisionInfo :type TD2020%20Vision%20Info%20Object%20Reference))
  (bind _commander (Variables|Default|GetCommander))
  ;[1 1 1] vision
  (Utilities|IsValid _commander
    (:Is%20Valid
      (Class|TD2020MinimapWidget|SetupVisionInfo (Variables|/Game/TD2020/Widgets/HUDs/WB_MainUI.WB_MainUI_C|GetTD2020SampleMinimapWidget (Variables|/Game/TD2020/Blueprints/Pawns/Pawn_MasterCommander.Pawn_MasterCommander_C|GetWB_MainUI _commander)) VisionInfo))))

(event EventMinimapLeftClick
  (params (InMouseEvent :type Pointer%20Event%20Structure%20%28by%20ref%29) (MinimapPosition :type Vector%202D%20Structure%20%28by%20ref%29) (WorldPosition :type Vector%20%28by%20ref%29 :default "0, 0, 0"))
  ;[1 1 1] Minimap Left Click
  (CallFunction|ROSMove (Variables|Default|GetCommander) WorldPosition))

(event EventOnMinimapClicked
  (params (InMouseEvent :type Pointer%20Event%20Structure%20%28by%20ref%29) (MinimapPosition :type Vector%202D%20Structure%20%28by%20ref%29) (WorldPosition :type Vector%20%28by%20ref%29 :default "0, 0, 0"))
  (bind _commander (Variables|Default|GetCommander))
  (bind _currentselectedactors (Variables|/Game/TD2020/Blueprints/Pawns/Pawn_MasterCommander.Pawn_MasterCommander_C|GetCurrentSelectedActors _commander))
  ;[1 1 1] On Minimap clicked - right mouse button - move selected units
  (if (== (Class|KismetInputLibrary|PointerEventGetEffectingButton InMouseEvent) "RightMouseButton")
    (if (Variables|/Game/TD2020/Blueprints/Pawns/Pawn_MasterCommander.Pawn_MasterCommander_C|GetAttackPressed? (Variables|Default|GetCommander))
      (Default|ROSAddRally _commander false WorldPosition "Attack" 0 _currentselectedactors)
      (Development|PrintString "Minimap Attack" true true "(R=0.000000,G=0.660000,B=1.000000,A=1.000000)" 5.0)
      (else
        (Default|ROSAddRally _commander false WorldPosition "Move" 0 _currentselectedactors)
        (Development|PrintString "Minimap Move" true true "(R=0.000000,G=0.660000,B=1.000000,A=1.000000)" 5.0)))))

(event EventBeginPlay
  ;[1 1 1] Begin play- set timer to update minimap every .2 seconds
  (Utilities|Time|SetTimerbyFunctionName 0 "UpdateMinimap" 0.2 true))

(fn ConstructionScript)

(fn LoadGame
  (bind _returnvalue (SaveGame|DoesSaveGameExist (Variables|Default|GetPlayerSettingsSave)))
  (if _returnvalue
    (bind _returnvalue_2 (SaveGame|LoadGamefromSlot (Variables|Default|GetPlayerSettingsSave)))
    (bind _assg_player_info (Utilities|Casting|CastToSG_PlayerInfo _returnvalue_2))
    (Variables|Default|SetPlayerSettings (Variables|/Game/TD2020/Blueprints/SaveGame/SG_PlayerInfo.SG_PlayerInfo_C|GetPlayerInfoStruct _assg_player_info))
    (else
      (Variables|Default|SetPlayerSettings (Utilities|Struct|MakePlayerInfo_Struct "DefaultName" "/Game/TD2020/Textures/SkeletalMeshes/UE4_LOGO_CARD.UE4_LOGO_CARD" "/Game/TD2020/Blueprints/Pawns/Pawn_HumanCommander.Pawn_HumanCommander_C" "/Game/TD2020/Textures/SkeletalMeshes/UE4Man_Logo_N.UE4Man_Logo_N" "DefaultState"))))
  (return (Variables|Default|GetPlayerSettings)))

(fn OnRepNumTravelingPlayers)

(fn ShowGameEndWidget
  (params (WiningStatement :type Text))
  (CallFunction|ROCVictory WiningStatement))

(fn UpdateMinimap
  (bind _commander (Variables|Default|GetCommander))
  (if (LocalVariables|GetKeepUpdating?)
    (bind _outactors (Actor|GetAllActorsOfClass "/Script/Engine.SceneCapture2D"))
    (for _array_element _outactors
      (Rendering|SceneCapture|CaptureScene (Variables|/Script/Engine.SceneCapture2D|GetCaptureComponent2D _array_element) :!class /Script/Engine.SceneCaptureComponent2D))
    (if (== (Utilities|Array|Length _outactors) 0)
      (LocalVariables|SetKeepUpdating? false)
      (Utilities|IsValid _commander
        (:Is%20Valid
          (Widget|SetVisibility (Variables|/Game/TD2020/Widgets/HUDs/WB_MainUI.WB_MainUI_C|GetTD2020SampleMinimapWidget (Variables|/Game/TD2020/Blueprints/Pawns/Pawn_MasterCommander.Pawn_MasterCommander_C|GetWB_MainUI _commander)) "Hidden"))))))