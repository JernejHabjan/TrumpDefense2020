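; Blueprint function library of shared helpers for a team-based strategy game with commanders, buildings and infantry.
; Mouse and touch helpers deproject screen positions and trace the landscape channel, while pan helpers rotate a pawn or spring arm with clamped pitch.
; Team-name comparison drives friendly-actor filtering, and actor data comes from DT_MyActor rows keyed by trimmed class names.
; Other helpers fit building collision boxes to mesh bounds and refresh tech requirements in the commander's UI.
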(fn SetCursorWorldPosition
  (params (Controller :type PC%20Gameplay%20PC%20Object%20Reference) (SightDistance :type Float%20%28single-precision%29))
  (bind (_worldlocation _worlddirection) (Game|Player|ConvertMouseLocationToWorldSpace Controller))
  (Utilities|IsValid Controller
    (:Is%20Valid
      (bind _outhit (Collision|LineTraceByChannel 0 _worldlocation (+ _worldlocation (* _worlddirection SightDistance)) "TraceTypeQuery3" false 0 "None")) ; Landscape is setup in project settings -> collision
      (return (.Location (Collision|BreakHitResult _outhit)) (.HitActor (Collision|BreakHitResult _outhit))))
    (:Is%20Not%20Valid
      (Development|PrintString 0 "Controller in function library is not valid" true true "(R=1.000000,G=0.034090,B=0.000000,A=1.000000)" 0.1))))

(fn SetTouchWorldPosition
  (params (CameraPawnControllerRef :type PC%20Gameplay%20PC%20Object%20Reference) (InLocation :type Vector) (SightDistance :type Float%20%28single-precision%29))
  (bind (_x _y) (Math|Vector|BreakVector InLocation))
  (bind (_worldlocation _worlddirection) (Class|PlayerController|DeprojectScreenPositiontoWorld CameraPawnControllerRef _x _y))
  (bind _outhit (Collision|LineTraceByChannel 0 _worldlocation (+ _worldlocation (* _worlddirection SightDistance)) "TraceTypeQuery3" false 0 "None")) ; Landscape is setup in project settings -> collision
  (if (!= (.HitActor (Collision|BreakHitResult _outhit)) 0)
    (return (.Location (Collision|BreakHitResult _outhit)))))

(fn Pan
  (params (PawnRef :type Pawn%20Object%20Reference) (MinPanY :type Float%20%28single-precision%29) (MaxPanY :type Float%20%28single-precision%29) (Sensitivity :type Float%20%28single-precision%29) (CameraX :type Float%20%28single-precision%29) (CameraY :type Float%20%28single-precision%29))
  (bind _returnvalue (Transformation|GetActorRotation PawnRef))
  (bind (_roll _pitch _yaw) (Math|Rotator|BreakRotator _returnvalue))
  (Transformation|SetActorRotation PawnRef (Math|Rotator|MakeRotator _roll (Math|Float|Clamp(Float) (+ _pitch (* Sensitivity CameraY)) MinPanY MaxPanY) (+ _yaw (* Sensitivity CameraX))))
  (return))

(fn PanMasterCommander
  (params (SpringArm :type Spring%20Arm%20Component%20Object%20Reference) (CamX :type Float%20%28single-precision%29) (CamY :type Float%20%28single-precision%29))
  (bind _returnvalue (Transformation|GetWorldRotation SpringArm))
  (bind _sensitivity_local (LocalVariables|GetSensitivity_LOCAL))
  (bind (_roll _pitch _yaw) (Math|Rotator|BreakRotator _returnvalue))
  (Transformation|SetWorldRotation SpringArm (Math|Rotator|MakeRotator _roll (Math|Float|Clamp(Float) (+ _pitch (* CamY _sensitivity_local)) (LocalVariables|GetMaxPanY_LOCAL) (LocalVariables|GetMinPanY_LOCAL)) (+ _yaw (* _sensitivity_local CamX))) false false))

(fn CheckTeams
  (params (Actor1 :type Actor%20Object%20Reference) (Actor2 :type Actor%20Object%20Reference))
  (Utilities|IsValid Actor1 ; if not dead
    (:Is%20Valid
      (bind _teamname (Class|ITD2020|GetTeamName(Message) Actor1))
      (Utilities|IsValid Actor2
        (:Is%20Valid
          (bind _teamname_2 (Class|ITD2020|GetTeamName(Message) Actor2))
          (return (Utilities|Enum|Equal(Enum) _teamname_2 _teamname)))
        (:Is%20Not%20Valid
          _)))
    (:Is%20Not%20Valid
      _))
  (return false))

(fn SetBuildingCollisionBox
  (params (Collision :type Box%20Component%20Object%20Reference) (Mesh :type Static%20Mesh%20Component%20Object%20Reference))
  (bind _min (Components|StaticMesh|GetLocalBounds Mesh))
  (bind (_x _y) (Math|Vector|BreakVector _min))
  (Components|Box|SetBoxExtent Collision (Math|Vector|MakeVector (- (Math|Float|Absolute(Float) _x) (LocalVariables|GetDisplaceX)) (LocalVariables|GetDisplaceY) (LocalVariables|GetDisplaceZ)) false)
  (Transformation|SetRelativeLocation Collision (Math|Vector|MakeVector 0.0 (+ (Math|Float|Absolute(Float) _y) (LocalVariables|GetDisplaceY)) (LocalVariables|GetDisplaceZ)) false false))

(fn RetrieveActorData
  (params (ActorClass :type My%20Actor%20Class%20Reference))
  (bind _returnvalue (Utilities|GetClassDisplayName ActorClass))
  (bind _returnvalue_2 (Utilities|String|LeftChop _returnvalue 2))
  (bind _returnvalue_3 (Utilities|GetDataTableRow "/Game/TD2020/DatatableStructs/DT_MyActor.DT_MyActor" (Utilities|String|StringToName _returnvalue_2))
    (:then
      (return _returnvalue_3))
    (:RowNotFound
      (Development|PrintString 0 (Utilities|String|Append "Row not found for actor " _returnvalue_2)))))

(fn GetFriendlyActorsOfClass
  (params (WorldContextObject :type Object%20Object%20Reference) (ActorClass :type Actor%20Class%20Reference) (Pawn :type Pawn%20Master%20Commander%20Object%20Reference))
  (bind _outactors (Actor|GetAllActorsOfClass WorldContextObject ActorClass))
  (for _array_element _outactors
    (if (CallFunction|CheckTeams _array_element Pawn WorldContextObject)
      (Utilities|Array|Add (LocalVariables|GetActors) _array_element)))
  (return (LocalVariables|GetActors)))

(fn UpdateRequirements
  (params (Commander :type Pawn%20Master%20Commander%20Object%20Reference))
  (bind _wb_mainui (Variables|/Game/TD2020/Blueprints/Pawns/Pawn_MasterCommander.Pawn_MasterCommander_C|GetWB_MainUI Commander))
  (bind _infantrylist (Variables|/Game/TD2020/Widgets/HUDs/WB_MainUI.WB_MainUI_C|GetInfantryList _wb_mainui))
  (Utilities|IsValid _wb_mainui
    (:Is%20Valid
      (Default|UpdateTechRequirements (Variables|/Game/TD2020/Widgets/HUDs/WB_MainUI.WB_MainUI_C|GetBuildingList _wb_mainui))
      (Utilities|IsValid _infantrylist
        (:Is%20Valid
          (Default|UpdateTechRequirements _infantrylist))))))