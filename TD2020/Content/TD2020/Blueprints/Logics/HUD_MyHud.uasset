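; RTS-style HUD that draws drag selection, rally paths, build grid, health and progress bars, and hovered actors' owner names.
; While dragging, DrawHUD draws the box and screen-projects locally controlled 0_Base actors to select them through Pawn_MasterCommander.
; Otherwise it draws action-colored rally lines for same-team selections and, in build mode, placement-colored tiles around the ghost building.
; Unit rallies come from AI controllers, so they may not show on clients.
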(event Custom|EventDrawRally
  (params (StartLocation :type Vector%20%28by%20ref%29) (RallyLocations :type Array%20of%20Vectors) (RallyActions :type Array%20of%20Strings))
  ;[1 1 1] Rally
  (Variables|Default|SetPrevLocation (.ScreenPosition (Class|GameplayStatics|ProjectWorldtoScreen (Variables|Default|GetPlayerOwner) StartLocation false)))
  (for (_array_element _array_index) RallyLocations
    (switch string (Utilities|Array|Get(acopy) RallyActions _array_index) ; get line color according to action
      (:Default
        (Variables|Default|SetRallyLineColor (Math|Color|MakeColor 1.0 1.0 0.0)))
      (:Move
        (Variables|Default|SetRallyLineColor (Math|Color|MakeColor 0.0 1.0 0.0)))
      (:Attack
        (Variables|Default|SetRallyLineColor (Math|Color|MakeColor 1.0 0.0 0.0))))
    (Class|HUD|DrawLine (.x (Variables|Default|GetPrevLocation)) (.y (Variables|Default|GetPrevLocation)) (.X (Math|Vector2D|BreakVector2D (.ScreenPosition (Class|GameplayStatics|ProjectWorldtoScreen (Variables|Default|GetPlayerOwner) _array_element false)))) (.Y (Math|Vector2D|BreakVector2D (.ScreenPosition (Class|GameplayStatics|ProjectWorldtoScreen (Variables|Default|GetPlayerOwner) _array_element false)))) (Variables|Default|GetRallyLineColor) 1.0)
    (Variables|Default|SetPrevLocation (.ScreenPosition (Class|GameplayStatics|ProjectWorldtoScreen (Variables|Default|GetPlayerOwner) _array_element false)))))

(event Custom|DrawGridTile
  (params (GridLocation :type Vector) (PlacementType :type PlacementType%20Enum :default "NewEnumerator0"))
  (bind (_x _y _z) (Math|Vector|BreakVector GridLocation))
  (bind _playerowner (Variables|Default|GetPlayerOwner))
  (bind _playerowner_2 (Variables|Default|GetPlayerOwner))
  (bind _screenposition (Class|GameplayStatics|ProjectWorldtoScreen _playerowner_2 GridLocation false))
  (bind _returnvalue (+ _y 128.0))
  (bind _returnvalue_2 (+ _x 128.0))
  (bind _returnvalue_3 (Math|Vector|MakeVector _returnvalue_2 _returnvalue _z))
  (bind (_x_2 _y_2) (Math|Vector2D|BreakVector2D _screenposition))
  (bind _screenposition_2 (Class|GameplayStatics|ProjectWorldtoScreen _playerowner _returnvalue_3 false))
  (bind (_x_3 _y_3) (Math|Vector2D|BreakVector2D _screenposition_2))
  (bind _returnvalue_4 (- _x_2 _x_3))
  (bind _returnvalue_5 (- _y_2 _y_3))
  (bind _returnvalue_6 (Math|Float|Absolute(Float) _returnvalue_4))
  (bind _returnvalue_7 (Math|Float|Absolute(Float) _returnvalue_5))
  (bind _returnvalue_8 (+ _x_2 _returnvalue_6))
  (bind _returnvalue_9 (+ _y_2 _returnvalue_7))
  ;[1 1 1] DrawGridTile
  (switch Utilities|FlowControl|Switch|SwitchonPlacementType PlacementType
    (:NewEnumerator0
      (Variables|Default|SetPlacementGridColor "(R=1.000000,G=1.000000,B=0.000000,A=0.300000)"))
    (:NewEnumerator1
      (Variables|Default|SetPlacementGridColor "(R=0.000000,G=1.000000,B=0.000000,A=0.300000)"))
    (:NewEnumerator2
      (Variables|Default|SetPlacementGridColor "(R=1.000000,G=0.000000,B=0.000000,A=0.300000)")))
  (HUD|DrawRect (Math|Color|MakeColor (.R (Math|Color|BreakColor (Variables|Default|GetPlacementGridColor))) (.G (Math|Color|BreakColor (Variables|Default|GetPlacementGridColor))) (.B (Math|Color|BreakColor (Variables|Default|GetPlacementGridColor))) 0.1) _x_2 _y_2 _returnvalue_6 _returnvalue_7)
  (Class|HUD|DrawLine _x_2 _y_2 _returnvalue_8 _y_2 (Variables|Default|GetPlacementGridColor) 0.0)
  (Class|HUD|DrawLine _returnvalue_8 _y_2 _returnvalue_8 _returnvalue_9 (Variables|Default|GetPlacementGridColor) 0.0)
  (Class|HUD|DrawLine _returnvalue_8 _returnvalue_9 _x_2 _returnvalue_9 (Variables|Default|GetPlacementGridColor) 0.0)
  (Class|HUD|DrawLine _x_2 _returnvalue_9 _x_2 _y_2 (Variables|Default|GetPlacementGridColor) 0.0))

(event Custom|DrawSelectionFrameFunction
  (params (ScreenX :type Float%20%28single-precision%29) (ScreenY :type Float%20%28single-precision%29) (Width :type Float%20%28single-precision%29) (Height :type Float%20%28single-precision%29))
  (bind _returnvalue (Math|Color|MakeColor 0.0 1.0 0.165606))
  (bind _returnvalue_2 (+ ScreenX Width))
  (bind _returnvalue_3 (+ ScreenY Height))
  ;[1 1 1] DrawSelectionFrame
  (HUD|DrawRect "(R=0.000000,G=1.000000,B=0.165606,A=0.136000)" ScreenX ScreenY Width Height)
  (Class|HUD|DrawLine ScreenX ScreenY _returnvalue_2 ScreenY _returnvalue 0.0)
  (Class|HUD|DrawLine _returnvalue_2 ScreenY _returnvalue_2 _returnvalue_3 _returnvalue 0.0)
  (Class|HUD|DrawLine _returnvalue_2 _returnvalue_3 ScreenX _returnvalue_3 _returnvalue 0.0)
  (Class|HUD|DrawLine ScreenX _returnvalue_3 ScreenX ScreenY _returnvalue 0.0))

(event EventDrawHoveredActorEffect
  (params (HoveredActor :type Actor%20Object%20Reference))
  (bind _returnvalue (Actor|GetComponentbyClass HoveredActor "/Script/RTSPlugin.RTSOwnerComponent"))
  (bind _returnvalue_2 (Class|RTSHUD|GetActorCenteronScreen HoveredActor))
  (bind (_x _y) (Math|Vector2D|BreakVector2D _returnvalue_2))
  ;[1 1 1] OnHoveredActorEffect
  (Utilities|IsValid HoveredActor
    (:Is%20Valid
      (Utilities|IsValid _returnvalue
        (:Is%20Valid
          (bind _returnvalue_3 (Class|RTSOwnerComponent|GetPlayerOwner _returnvalue))
          (Utilities|IsValid _returnvalue_3
            (:Is%20Valid
              (HUD|DrawText (Variables|/Script/Engine.PlayerState|GetPlayerName _returnvalue_3) "(R=0,G=0,B=0,A=1)" (- _x (/ (.OutWidth (Class|HUD|GetTextSize (Variables|/Script/Engine.PlayerState|GetPlayerName _returnvalue_3) 0 1.0)) 2.0)) (+ (- _y (.Y (Math|Vector2D|BreakVector2D (Class|RTSHUD|GetActorSizeonScreen HoveredActor)))) 1e+01) 0 1.0 false))))))))

(event EventDrawHealthBar
  (params (Actor :type Actor%20Object%20Reference) (CurrentHealth :type Float%20%28single-precision%29) (MaximumHealth :type Float%20%28single-precision%29) (HealthPercentage :type Float%20%28single-precision%29) (SuggestedHealthBarLeft :type Float%20%28single-precision%29) (SuggestedHealthBarTop :type Float%20%28single-precision%29) (SuggestedHealthBarWidth :type Float%20%28single-precision%29) (SuggestedHealthBarHeight :type Float%20%28single-precision%29))
  (bind _returnvalue (Math|Float|MakeLiteralFloat 2.0))
  (bind _returnvalue_2 (+ SuggestedHealthBarLeft _returnvalue))
  (bind _returnvalue_3 (+ SuggestedHealthBarTop _returnvalue))
  (bind _returnvalue_4 (* _returnvalue 2.0))
  (bind _returnvalue_5 (- SuggestedHealthBarWidth _returnvalue_4))
  (bind _returnvalue_6 (- SuggestedHealthBarHeight _returnvalue_4))
  ;[1 1 1] DrawHealthBar
  (HUD|DrawRect "(R=1.000000,G=1.000000,B=1.000000,A=1.000000)" SuggestedHealthBarLeft SuggestedHealthBarTop SuggestedHealthBarWidth SuggestedHealthBarHeight) ; Draw Health Bar Border
  (HUD|DrawRect "(R=0.000000,G=0.000000,B=0.000000,A=1.000000)" _returnvalue_2 _returnvalue_3 _returnvalue_5 _returnvalue_6) ; Draw Health Bar Background
  (HUD|DrawRect "(R=0.023822,G=1.000000,B=0.000000,A=1.000000)" _returnvalue_2 _returnvalue_3 (* _returnvalue_5 HealthPercentage) _returnvalue_6) ; Draw Health Bar
)

(event EventDrawProductionProgressBar
  (params (Actor :type Actor%20Object%20Reference) (ProductionTime :type Float%20%28single-precision%29) (RemainingProductionTime :type Float%20%28single-precision%29) (ProgressPercentage :type Float%20%28single-precision%29) (SuggestedProgressBarLeft :type Float%20%28single-precision%29) (SuggestedProgressBarTop :type Float%20%28single-precision%29) (SuggestedProgressBarWidth :type Float%20%28single-precision%29) (SuggestedProgressBarHeight :type Float%20%28single-precision%29))
  (bind _returnvalue (Math|Float|MakeLiteralFloat 2.0))
  (bind _returnvalue_2 (+ SuggestedProgressBarLeft _returnvalue))
  (bind _returnvalue_3 (+ SuggestedProgressBarTop _returnvalue))
  (bind _returnvalue_4 (* _returnvalue 2.0))
  (bind _returnvalue_5 (- SuggestedProgressBarWidth _returnvalue_4))
  (bind _returnvalue_6 (- SuggestedProgressBarHeight _returnvalue_4))
  ;[1 1 1] DrawProductionProgressBar
  (HUD|DrawRect "(R=1.000000,G=1.000000,B=1.000000,A=1.000000)" SuggestedProgressBarLeft SuggestedProgressBarTop SuggestedProgressBarWidth SuggestedProgressBarHeight) ; Draw Health Bar Border
  (HUD|DrawRect "(R=0.000000,G=0.000000,B=0.000000,A=1.000000)" _returnvalue_2 _returnvalue_3 _returnvalue_5 _returnvalue_6) ; Draw Health Bar Background
  (HUD|DrawRect "(R=0.337222,G=0.000000,B=1.000000,A=1.000000)" _returnvalue_2 _returnvalue_3 (* _returnvalue_5 ProgressPercentage) _returnvalue_6) ; Draw Health Bar
)

(event EventDrawHUD
  (params (SizeX :type Integer) (SizeY :type Integer))
  (bind _returnvalue (Game|GetPlayerController 0))
  (bind _clickedlocation (Variables|Default|GetClickedLocation))
  (bind (_x _y) (Math|Vector2D|BreakVector2D _clickedlocation))
  (bind (_locationx _locationy) (Game|Player|GetMousePosition _returnvalue))
  ;[1 1 1] Draw HUD
  (Variables|Default|SetScreenResolution (Math|Vector2D|MakeVector2D (Math|Conversions|ToFloat(Integer) SizeX) (Math|Conversions|ToFloat(Integer) SizeY)))
  (if (Variables|Default|GetIsDrawing)
    (Variables|Default|SetCurrentMouseLocation (Math|Vector2D|MakeVector2D _locationx _locationy))
    (CallFunction|DrawSelectionFrameFunction _x _y (.X (Math|Vector2D|BreakVector2D (- (Variables|Default|GetCurrentMouseLocation) (Variables|Default|GetClickedLocation)))) (.Y (Math|Vector2D|BreakVector2D (- (Variables|Default|GetCurrentMouseLocation) (Variables|Default|GetClickedLocation)))))
    (CallFunction|CheckActorsinDragBox)
    (else
      (CallFunction|Rally)
      (CallFunction|Grid))))

(event EventDrawSelectionFrame
  (params (ScreenX :type Float%20%28single-precision%29) (ScreenY :type Float%20%28single-precision%29) (Width :type Float%20%28single-precision%29) (Height :type Float%20%28single-precision%29))
  ;[1 1 1] Event selectionFrame
  (CallFunction|DrawSelectionFrameFunction ScreenX ScreenY Width Height)
  (CallFunction|CheckActorsinDragBox))

(event EventDrawConstructionProgressBar
  (params (Actor :type Actor%20Object%20Reference) (ConstructionTime :type Float%20%28single-precision%29) (RemainingConstructionTime :type Float%20%28single-precision%29) (ProgressPercentage :type Float%20%28single-precision%29) (SuggestedProgressBarLeft :type Float%20%28single-precision%29) (SuggestedProgressBarTop :type Float%20%28single-precision%29) (SuggestedProgressBarWidth :type Float%20%28single-precision%29) (SuggestedProgressBarHeight :type Float%20%28single-precision%29))
  (bind _returnvalue (Math|Float|MakeLiteralFloat 2.0))
  (bind _returnvalue_2 (+ SuggestedProgressBarLeft _returnvalue))
  (bind _returnvalue_3 (+ SuggestedProgressBarTop _returnvalue))
  (bind _returnvalue_4 (* _returnvalue 2.0))
  (bind _returnvalue_5 (- SuggestedProgressBarWidth _returnvalue_4))
  (bind _returnvalue_6 (- SuggestedProgressBarHeight _returnvalue_4))
  ;[1 1 1] DrawConstructionProgressBar
  (HUD|DrawRect "(R=1.000000,G=1.000000,B=1.000000,A=1.000000)" SuggestedProgressBarLeft SuggestedProgressBarTop SuggestedProgressBarWidth SuggestedProgressBarHeight) ; Draw Health Bar Border
  (HUD|DrawRect "(R=0.000000,G=0.000000,B=0.000000,A=1.000000)" _returnvalue_2 _returnvalue_3 _returnvalue_5 _returnvalue_6) ; Draw Health Bar Background
  (HUD|DrawRect "(R=0.000000,G=0.243758,B=1.000000,A=1.000000)" _returnvalue_2 _returnvalue_3 (* _returnvalue_5 ProgressPercentage) _returnvalue_6) ; Draw Health Bar
)

(fn ConstructionScript)

(fn CheckDragBoxDimension
  (bind _currentmouselocation (Variables|Default|GetCurrentMouseLocation))
  (bind _clickedlocation (Variables|Default|GetClickedLocation))
  (bind (_x _y) (Math|Vector2D|BreakVector2D _currentmouselocation))
  (bind (_x_2 _y_2) (Math|Vector2D|BreakVector2D _clickedlocation))
  (Utilities|FlowControl|Sequence
    (:then_0
      (if (>= (- _x _x_2) 0.0)
        (Variables|Default|SetXmin _x_2)
        (Variables|Default|SetXmax _x)
        (else
          (Variables|Default|SetXmin _x)
          (Variables|Default|SetXmax _x_2))))
    (:then_1
      (if (>= (- _y _y_2) 0.0)
        (Variables|Default|SetYmin _y_2)
        (Variables|Default|SetYmax _y)
        (else
          (Variables|Default|SetYmin _y)
          (Variables|Default|SetYmax _y_2))))))

(fn IsActorinDragBox
  (params (InActor2DVector :type Vector%202D%20Structure))
  (bind (_x _y) (Math|Vector2D|BreakVector2D InActor2DVector))
  (return (Math|Boolean|ANDBoolean (>= _x (Variables|Default|GetXmin)) (<= _x (Variables|Default|GetXmax)) (>= _y (Variables|Default|GetYmin)) (<= _y (Variables|Default|GetYmax)))))

(fn ActorIsinDragBox
  (params (InActor :type Actor%20Object%20Reference))
  (Default|SelectActor (.AsPawn%20Master%20Commander (Utilities|Casting|CastToPawn_MasterCommander (Game|Player|GetPlayerPawn 0))) InActor))

(fn ActorIsNotinDragBox
  (params (InActor :type Actor%20Object%20Reference))
  (if (Utilities|Array|ContainsItem (Variables|Default|GetSelectedActors) InActor)
    (Class|ITD2020|ImNotSelected(Message) InActor (.AsPawn%20Master%20Commander (Utilities|Casting|CastToPawn_MasterCommander (Game|Player|GetPlayerPawn 0))))
    (Utilities|Array|RemoveItem (Variables|Default|GetSelectedActors) InActor)))

(fn CheckActorsinDragBox
  (CallFunction|CheckDragBoxDimension)
  (bind _outactors (Actor|GetAllActorsOfClass "/Game/TD2020/Blueprints/AI/Characters/0_Base.0_Base_C")) ; Now only for units
  (for _array_element _outactors
    (if (Pawn|IsLocallyControlled (Variables|/Game/TD2020/Blueprints/AI/Characters/0_Base.0_Base_C|GetLocalCommander _array_element)) ; Checking only our units
      (bind _isindragbox (CallFunction|IsActorinDragBox (.ScreenLocation (Class|PlayerController|ProjectWorldLocationtoScreen (Game|GetPlayerController 0) (Transformation|GetActorLocation _array_element) false))))
      (if _isindragbox
        (CallFunction|ActorIsinDragBox _array_element)
        (elif (Variables|Default|GetMultipleSelection)
          (Development|PrintString "Multiple selection")
          (else
            (CallFunction|ActorIsNotinDragBox _array_element)))))))

(fn Rally
  (bind _aspawn_master_commander (Utilities|Casting|CastToPawn_MasterCommander (Pawn|GetControlledPawn (.AsPC%20Gameplay%20PC (Utilities|Casting|CastToPC_GameplayPC (Variables|Default|GetPlayerOwner))))))
  (for _array_element (Variables|/Game/TD2020/Blueprints/Logics/Pawn_MasterCommander.Pawn_MasterCommander_C|GetCurrentSelectedActors _aspawn_master_commander)
    (Utilities|IsValid _array_element
      (:Is%20Valid
        (if (CallFunction|CheckTeams _array_element _aspawn_master_commander) ; draw rally only if teams are same
          (bind _as0_base (Utilities|Casting|CastTo0_Base _array_element)
            (:then
              ;[1 1 1] TODO - rallies are stored in ai controller - may not be valid on client - so rallies are not displayed
              (Utilities|IsValid (Variables|/Game/TD2020/Blueprints/AI/Characters/0_Base.0_Base_C|GetAIController _as0_base)
                (:Is%20Valid
                  (bind (_startlocation _rallylocations _rallyactions) (Default|GetRallies (Variables|/Game/TD2020/Blueprints/AI/Characters/0_Base.0_Base_C|GetAIController _as0_base))) ; fallies are in AI controller for characters
                  (CallFunction|EventDrawRally _startlocation _rallylocations _rallyactions))))
            (:CastFailed
              (bind (_startlocation_2 _rallylocations_2 _rallyactions_2) (Class|ITD2020|GetRallies(Message) _array_element))
              (CallFunction|EventDrawRally _startlocation_2 _rallylocations_2 _rallyactions_2))))))))

(fn Grid
  (bind _aspawn_master_commander (Utilities|Casting|CastToPawn_MasterCommander (Pawn|GetControlledPawn (.AsPC%20Gameplay%20PC (Utilities|Casting|CastToPC_GameplayPC (Variables|Default|GetPlayerOwner))))))
  (if (Variables|/Game/TD2020/Blueprints/Logics/Pawn_MasterCommander.Pawn_MasterCommander_C|GetBuildModeActive _aspawn_master_commander)
    (bind (_gridlocations _placementtypes) (Default|GetSurroundingGrid (Variables|/Game/TD2020/Blueprints/Logics/Pawn_MasterCommander.Pawn_MasterCommander_C|GetGhostBuildingRef _aspawn_master_commander)))
    (for (_array_element _array_index) _gridlocations
      (CallFunction|DrawGridTile _array_element (Utilities|Array|Get(acopy) _placementtypes _array_index)))))